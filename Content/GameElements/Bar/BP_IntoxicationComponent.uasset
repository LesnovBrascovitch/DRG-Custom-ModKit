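; Intoxication component for the bar game element, exposing drunk begin, tick, end and pass-out hooks.
; The four drunk lifecycle events only forward to the parent class, so any actual behavior comes from there.
; Effect push/pop, movement and post-process lerp events are empty stubs, as are the helper functions, which return blank or zero values where a result is expected.
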(event `Lerp Movement Stength`
  (params (DeltaTime :type "Float (double-precision)")))

(event `Push Effects`)

(event `Pop Effects`
  (params (DebugReason :type String)))

(event `self.ReceiveDrunkTick`
  (params (DeltaTime :type "Float (single-precision)") (DrunkTime :type "Float (single-precision)"))
  (`parent.ReceiveDrunkTick` DeltaTime DrunkTime))

(event `self.ReceivePassOutDrunk`
  (`parent.ReceivePassOutDrunk`))

(event `Lerp Post Process Strength`
  (params (DeltaTime :type "Float (double-precision)")))

(event `self.ReceiveDrunkEnd`
  (`parent.ReceiveDrunkEnd`))

(event `self.ReceiveDrunkBegin`
  (`parent.ReceiveDrunkBegin`))

(fn `MyLerp`
  (params (`Current Value` :type "Float (double-precision)") (`Target Value` :type "Float (double-precision)") (`Delta Time` :type "Float (double-precision)"))
  (returns (Result :type "Float (double-precision)"))
  (return 0.0))

(fn `SetPostProcessStrength`
  (params (NewStrength :type "Float (double-precision)")))

(fn `ToPercentStr`
  (params (Progress :type "Float (double-precision)"))
  (returns (PercentString :type String))
  (return ""))