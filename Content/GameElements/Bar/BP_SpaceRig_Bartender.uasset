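; BP_SpaceRig_Bartender is a stub of the Space Rig bartender, declaring its interface for serving drinks to players.
; Only BeginPlay and PlayBartenderTip do anything, forwarding to the parent; all other events and functions are empty or return false or zero.
; The declared members outline customer tracking with replicated state, server and client drink spawning, pouring with lerp timelines, animations, a mixer, lights, fireworks and payment.
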(event `self.ReceiveBeginPlay`
  (`parent.ReceiveBeginPlay`))

(event `LerpTimeline__FinishedFunc`)

(event `LerpTimeline__UpdateFunc`)

(event `FinishedTimeline__FinishedFunc`)

(event `FinishedTimeline__UpdateFunc`)

(event `LookAtCustomer`
  (params (Customer :type "PlayerCharacter Object Reference")))

(event `OnPlayerLeave_Event`
  (params (PlayerState :type "FSDPlayerState Object Reference")))

(event `Update Bartender Lights`)

(event `SpawnDrinks`
  (params (Drinable :type "DrinkableDataAsset Object Reference")))

(event `Lerp To`
  (params (PourTransform :type "Transform Structure") (Duration :type "Float (double-precision)")))

(event `Server Spawn Next Drink`)

(event `OnAvailableForNewDrink_Event`
  (params (DrinkBox :type "/Game/LevelElements/Spacerig/Bar/DrinksDispenser/Assets/BP_DrinksBox Object Reference")))

(event `OnDrinkReady_Event`
  (params (DrinkBox :type "/Game/LevelElements/Spacerig/Bar/DrinksDispenser/Assets/BP_DrinksBox Object Reference")))

(event `Return To Idle`)

(event `All_BeginSpawnDrinks`
  (params (PlayFireworks :type Boolean)))

(event `Client Spawn Next Drink`
  (params (DrinkBox :type "/Game/LevelElements/Spacerig/Bar/DrinksDispenser/Assets/BP_DrinksBox Object Reference")))

(event `Look Towards`
  (params (Actor :type "Actor Object Reference") (Duration :type "Float (double-precision)")))

(event `Init Background Menu`)

(event `Toggle Fireworks`
  (params (Enabled :type Boolean)))

(event `InitializeMixer`)

(event `OnUsableChanged_Mixer`
  (params (canUse :type Boolean)))

(event `self.PlayBartenderTip`
  (params (User :type "PlayerCharacter Object Reference"))
  (`parent.PlayBartenderTip` User))

(fn `CanOrderNewRound`
  (returns (CanOrder :type Boolean))
  (return false))

(fn `OnRep_CurrentCustomerState`)

(fn `PayCredits`
  (params (User :type "PlayerCharacter Object Reference") (Amount :type Integer))
  (returns (Purchased :type Boolean))
  (return false))

(fn `PlayAffirmative`
  (returns (Duration :type "Float (double-precision)"))
  (return 0.0))

(fn `PlayAnim`
  (params (MontageToPlay :type "AnimMontage Object Reference"))
  (returns (Duration :type "Float (double-precision)"))
  (return 0.0))

(fn `PlayGreeting`
  (returns (Duration :type "Float (double-precision)"))
  (return 0.0))

(fn `PlayNegative`
  (returns (Duration :type "Float (double-precision)"))
  (return 0.0))

(fn `Pour`
  (params (DrinkBox :type "/Game/LevelElements/Spacerig/Bar/DrinksDispenser/Assets/BP_DrinksBox Object Reference"))
  (returns (PourDuration :type "Float (double-precision)"))
  (return 0.0))

(fn `PourFinished`)

(fn `SetBartenderLightMaterial`
  (params (SourceMaterial :type "MaterialInterface Object Reference")))

(fn `SetCableAnchors`)

(fn `SetCustomer`
  (params (Customer :type "PlayerCharacter Object Reference")))

(fn `Spawn Mixer Beer`
  (params (ControlEventID :type String) (MixerCooldownToSet :type Integer) (OrderedDrink :type "DrinkableDataAsset Object Reference") (`Ordering Player` :type String) (`Announcement Text` :type Text)))

(fn `UpdateHolidayDecoration`)

(fn `UserConstructionScript`)