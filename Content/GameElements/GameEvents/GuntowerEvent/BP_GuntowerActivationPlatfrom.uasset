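; BP_GuntowerActivationPlatfrom is an activation platform in the Guntower game event that players step on and off.
; Its event handlers for begin play, disabled changes, shutdown, finish and player step counts only forward to the parent class, which supplies the behavior.
; SetLightColor and DisableLight are empty, so this Blueprint adds no light logic of its own.
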(event `self.ReceiveBeginPlay`
  (`parent.ReceiveBeginPlay`))

(event `self.OnDisabledChanged`
  (params (IsDisabled :type Boolean))
  (`parent.OnDisabledChanged` IsDisabled))

(event `self.OnShutDown`
  (`parent.OnShutDown`))

(event `self.OnFinished`
  (`parent.OnFinished`))

(event `self.PlayerSteppedOn`
  (params (CurrentCount :type Integer))
  (`parent.PlayerSteppedOn` CurrentCount))

(event `self.PlayerSteppedOff`
  (params (CurrentCount :type Integer))
  (`parent.PlayerSteppedOff` CurrentCount))

(fn `DisableLight`)

(fn `SetLightColor`
  (params (LightColor :type "Color Structure")))

(fn `UserConstructionScript`)