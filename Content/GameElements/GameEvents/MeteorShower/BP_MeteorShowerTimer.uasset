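; BP_MeteorShowerTimer is a meteor shower game event Blueprint that is almost entirely a stub.
; BeginPlay, PreEventSpawn, construction and GetSpawnTransform defer to the parent class.
; The meteor spawn, completion, failure, plague heart and warning sound events have empty bodies, and GetValidMeteor returns without logic.
; No timer logic appears in its graphs, and Tick and overlap are disabled.
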(event `self.ReceiveBeginPlay`
  (`parent.ReceiveBeginPlay`))

(event `SpawnedMeteor`
  (params (Spawned :type "Actor Object Reference")))

(event `SpawnSequenceComplete`)

(event `MetorSpawned`
  (params (Actor :type "Actor Object Reference")))

(event `SpawnFailed`)

(event `AssignPlagueHeart`)

(event `self.PreEventSpawn`
  (`parent.PreEventSpawn`))

(event `All_PlayWarningSound`)

(fn `GetSpawnTransform`
  (returns (ReturnValue :type "Transform Structure"))
  (return (`parent.GetSpawnTransform`)))

(fn `GetValidMeteor`
  (return))

(fn `UserConstructionScript`
  (`parent.UserConstructionScript`))