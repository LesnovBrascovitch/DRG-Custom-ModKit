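; Plague meteor game event Blueprint that appears to be a thin child of a shared meteor event class.
; Drop, near-impact, impact, late-join impact, visuals, stage and heart fail-safe events only forward to the parent.
; Event flow, pod, piston, crevasse, roof-break and heart-spawn hooks are empty, as are the replication callbacks.
; The file adds no logic of its own, and its finished check always returns false.
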(event `self.ReceiveBeginPlay`
  (`parent.ReceiveBeginPlay`))

(event `self.DropStarted`
  (`parent.DropStarted`))

(event `self.Impacted`
  (`parent.Impacted`))

(event `self.EnableVisuals`
  (`parent.EnableVisuals`))

(event `PowerLineConnected`
  (params (EndPoint :type "/Game/WeaponsNTools/RockCrackerBuilder/BP_RockCracker_EndPoint Object Reference")))

(event `Failed`)

(event `Success`)

(event `OnPistonRepaired`
  (params (user :type "PlayerCharacter Object Reference") (key :type "EInputKeys Enum" :default "Use")))

(event `EndExplosion`)

(event `EventFinished`)

(event `self.OnStageAdvanced`
  (params (Stage :type Integer))
  (`parent.OnStageAdvanced` Stage))

(event `OnHeartDeposited`)

(event `self.NearImpact`
  (`parent.NearImpact`))

(event `CarveCrevasse`
  (params (StaticMesh :type "StaticMesh Object Reference") (transform :type "Transform Structure (by ref)")))

(event `StartRepairPistons`)

(event `OnPodsLanded`
  (params (InPod :type "RessuplyPod Object Reference") (InState :type "ERessuplyPodState Enum" :default "ReadyToDrop")))

(event `StartEvent`)

(event `PushEventWidget_WhenHudIsReady`)

(event `TestIfRoofBreak`)

(event `SpawnBreakThroughParticle`
  (params (Location :type "Vector Structure")))

(event `StartBreakThroughTimer`)

(event `StateChanged`
  (params (currentState :type "ERockCrackerstate Enum" :default "Init") (previousState :type "ERockCrackerstate Enum" :default "Init")))

(event `WorkingPodCountChanged`
  (params (OldCount :type Integer) (NewCount :type Integer)))

(event `self.LastaudioSignal`
  (`parent.LastaudioSignal`))

(event `OpenMeteor`)

(event `SpawnHearts`)

(event `TestDestroy`)

(event `self.Impacted_Latejoin`
  (`parent.Impacted_Latejoin`))

(event `self.DestroyAndSpawnHearts_FailSafe`
  (`parent.DestroyAndSpawnHearts_FailSafe`))

(fn `ConvertToImpactPos`
  (params (InTransform :type "Transform Structure"))
  (returns (OutTransform :type "Transform Structure"))
  (return))

(fn `IsEventFinished`
  (returns (IsFinished :type Boolean))
  (return false))

(fn `OnRep_Event_MeteorDefence`)

(fn `OnRep_EventUIActive`)

(fn `OnRep_IsEventDone`)

(fn `OnRep_ShowOnScanner`)

(fn `SetWorkingPodCount`
  (params (Count :type Integer)))

(fn `UserConstructionScript`)