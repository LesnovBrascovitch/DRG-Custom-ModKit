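; Rock cracker pod Blueprint for the Plague Meteor game event, built as a child of a parent pod class.
; Start and end, droppod impact, pod state changes and yellow light switching all forward to the parent's implementations.
; Carver resizing, end point, fuel line and light material hooks are empty, so this graph adds no logic of its own.
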(event `self.ReceiveBeginPlay`
  (`parent.ReceiveBeginPlay`))

(event `self.OnEventStarted`
  (`parent.OnEventStarted`))

(event `self.OnEventEnded`
  (params (wasSuccess :type Boolean))
  (`parent.OnEventEnded` wasSuccess))

(event `self.OnDroppodImpact`
  (`parent.OnDroppodImpact`))

(event `ResizeCarver`)

(event `SetEndPoint`
  (params (EndPoint :type "/Game/WeaponsNTools/RockCrackerBuilder/BP_RockCracker_EndPoint Object Reference")))

(event `OnFirstFuelLineSegment`
  (params (InFirstSegment :type "FuelLineSegment Object Reference")))

(event `self.OnEnterState`
  (params (NewPodState :type "ERockCrackerstate Enum" :default "Init"))
  (`parent.OnEnterState` NewPodState))

(event `self.OnExitState`
  (params (NewPodState :type "ERockCrackerstate Enum" :default "Init"))
  (`parent.OnExitState` NewPodState))

(event `self.SwitchYellowLights`
  (params (isGreen :type Boolean))
  (`parent.SwitchYellowLights` isGreen))

(fn `OnRep_FuelLineStartLocation`)

(fn `UpdateLights`
  (params (NewMaterial :type "MaterialInterface Object Reference")))

(fn `UserConstructionScript`)