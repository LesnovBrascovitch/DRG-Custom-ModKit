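; Explosive barrel dispenser platform for the explosive barrels game event, built as a child Blueprint with drop pod behavior inherited from its parent.
; BeginPlay, drop start, close-to-impact and impact events only forward to the parent.
; Other event hooks, such as opening, progress, triggering, deploy animations, outlines and carver resizing, are empty.
; Event setup, progress and objective functions are stubs returning false, so this Blueprint adds no logic of its own.
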(event `self.ReceiveBeginPlay`
  (`parent.ReceiveBeginPlay`))

(event `self.OnEventOpened`)

(event `self.OnEventProgress`
  (params (Progress :type "Float (single-precision)")))

(event `self.OnEventTriggered`)

(event `self.OnDropStarted`
  (`parent.OnDropStarted`))

(event `self.OnDroppodImpact`
  (`parent.OnDroppodImpact`))

(event `DeployAnimations`)

(event `self.OnEventFinished`
  (params (eventSuccess :type Boolean)))

(event `ManageOutLines`)

(event `self.OnDroppodCloseToImpact`
  (`parent.OnDroppodCloseToImpact`))

(event `ResizeCarver`)

(fn `AddEventProgress`
  (params (Progress :type "Float (double-precision)"))
  (returns (ReturnValue :type Boolean))
  (return false))

(fn `AdvanceOneObjective`
  (returns (ReturnValue :type Boolean))
  (return false))

(fn `OnRep_ChildrenActive`)

(fn `SetChildrenReady`
  (params (IsReady :type Boolean)))

(fn `SetupEvent`
  (params (GameEvent :type "GameEvent Object Reference"))
  (returns (ReturnValue :type Boolean))
  (return false))

(fn `UserConstructionScript`)