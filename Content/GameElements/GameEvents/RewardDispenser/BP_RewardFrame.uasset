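; BP_RewardFrame is a game-event actor that, judging by its function names, frames a group of reward dispensers.
; It declares hooks for event lifecycle and progress, dispenser setup and alignment, an attention-light timeline, key recall, gravity and a finish-event cheat.
; Nearly every body is an empty stub returning nothing or false; only BeginPlay does work, by calling its parent.
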(event `self.ReceiveBeginPlay`
  (`parent.ReceiveBeginPlay`))

(event `AttentionLightTimeLine__FinishedFunc`)

(event `AttentionLightTimeLine__UpdateFunc`)

(event `self.OnEventOpened`)

(event `self.OnEventProgress`
  (params (Progress :type "Float (single-precision)")))

(event `self.OnEventFinished`
  (params (eventSuccess :type Boolean)))

(event `self.OnEventTriggered`)

(event `Toggle Attention Light`
  (params (InVisible :type Boolean)))

(event `Recall Key`)

(event `EnableGravity`)

(event `Cheat_FinishEvent`)

(fn `AddEventProgress`
  (params (Progress :type "Float (double-precision)"))
  (returns (ReturnValue :type Boolean))
  (return false))

(fn `AdvanceOneObjective`
  (returns (ReturnValue :type Boolean))
  (return false))

(fn `AlignDispensers`)

(fn `AllDispensersFinished`
  (returns (IsFinished :type Boolean))
  (return false))

(fn `GetLocalPlayerDispenser`
  (returns (OutDispenser :type "EventRewardDispenser Object Reference"))
  (return null))

(fn `GetRandomPlayer`
  (returns (Output :type "PlayerCharacter Object Reference"))
  (return null))

(fn `SetupDispenser`
  (params (dispenser :type "EventRewardDispenser Object Reference")))

(fn `SetupEvent`
  (params (GameEvent :type "GameEvent Object Reference"))
  (returns (ReturnValue :type Boolean))
  (return false))

(fn `StartEventUI`)

(fn `UpdateLights`)

(fn `UserConstructionScript`)