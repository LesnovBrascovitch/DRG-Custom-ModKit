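; Reward dispenser actor Blueprint for game events, with hooks for owner assignment, power-up, opening, schematic selection and reward selection.
; Owner, power-up, open and reward-selected events only call the parent implementation.
; Initialize, selector-finished, button and selector-toggle hooks are empty.
; State and local-control checks return false and the selector getter returns nothing, so this graph adds no behavior of its own.
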(event `self.OnOwnerAssigned`
  (`parent.OnOwnerAssigned`))

(event `self.OnPoweredUp`
  (`parent.OnPoweredUp`))

(event `Initialize`)

(event `self.OnOpenDispenser`
  (`parent.OnOpenDispenser`))

(event `On Selector Finished`
  (params (SchematicReward :type "Schematic Object Reference")))

(event `self.OnRewardSelected`
  (`parent.OnRewardSelected`))

(event `Turn On Buttons`)

(fn `GetRewardSelector`
  (return))

(fn `IsPlayerLocallyControlled`
  (returns (LocallyControlled :type Boolean))
  (return false))

(fn `IsStateValid`
  (returns (ReturnValue :type Boolean))
  (return false))

(fn `ToggleRewardSelector`
  (params (InVisible :type Boolean)))

(fn `UserConstructionScript`)