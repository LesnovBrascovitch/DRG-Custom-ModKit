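; BP_Donkey is a Blueprint for the Donkey, an entity that can be called to positions and sent to the drop ship.
; It is nearly a shell: BeginPlay, button enabling, down-state replication, drop ship handlers and the calling-shout getter forward to the parent.
; Its other events and functions, including destination, breadcrumb, tray, player-leave and photosensitivity hooks, have empty bodies, so the file adds no logic of its own.
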(event `self.ReceiveBeginPlay`
  (`parent.ReceiveBeginPlay`))

(event `OnDonkeyCalled`
  (params (position :type "Vector Structure") (requester :type "PlayerCharacter Object Reference")))

(event `SetDonkeyPos`
  (params (Pos :type "Vector Structure")))

(event `On Goto Dropship`)

(event `SpawnBreadCrumb`)

(event `Update Button State`)

(event `self.EnableButton`
  (`parent.EnableButton`))

(event `self.OnRep_IsDown`
  (`parent.OnRep_IsDown`))

(event `self.SetControlledByDropShip`
  (params (Control :type Boolean))
  (`parent.SetControlledByDropShip` Control))

(event `OnPlayerLeft`
  (params (PlayerState :type "FSDPlayerState Object Reference")))

(event `self.SetGotoDropShip`
  (params (Location :type "Vector Structure (by ref)"))
  (`parent.SetGotoDropShip` Location))

(fn `GetCallingShout`
  (returns (ReturnValue :type "DialogDataAsset Object Reference"))
  (return (`parent.GetCallingShout`)))

(fn `GotoDropShip`
  (params (Pos :type "Vector Structure")))

(fn `HandlePhotosensitivity`)

(fn `OnRep_IsTrayOpen`)

(fn `Set Controlled by Drop Ship`
  (params (control :type Boolean)))

(fn `SetDestination`
  (params (Destination :type "Vector Structure") (InCalledBy :type "PlayerCharacter Object Reference")))

(fn `UpdateStopCallRequests`)

(fn `UserConstructionScript`)