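; BP_Bosco is the Blueprint for the Bosco drone, a thin child class that leaves its behavior to its parent.
; BeginPlay, AI messages and triggers, self-destruct, state changes and possession all forward straight to the parent implementations.
; The construction script, ScareEffect, gear stat entry and projectile diff functions are empty stubs, so the graphs add no logic of their own.
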(event `self.ReceiveBeginPlay`
  (`parent.ReceiveBeginPlay`))

(event `self.OnMessageAI`
  (params (TriggerName :type Name))
  (`parent.OnMessageAI` TriggerName))

(event `self.SelfDestruct`
  (`parent.SelfDestruct`))

(event `self.StateChanged`
  (params (aCurrentState :type "EDroneAIState Enum" :default "Follow"))
  (`parent.StateChanged` aCurrentState))

(event `self.ReceivePossessed`
  (params (NewController :type "Controller Object Reference"))
  (`parent.ReceivePossessed` NewController))

(fn `GetGearStatEntry`
  (params (PlayerState :type "FSDPlayerState Object Reference") (Stats :type "Array of GearStatEntry Structure (by ref)"))
  (return))

(fn `Handle Projectile diffs`
  (params (`Gear stat` :type "GearStatEntry Structure") (`Cryo upgrade preview status` :type "EItemPreviewStatus Enum" :default "Normal") (`damage upgrade type` :type "EDamageUpgrade Enum" :default "Damage") (`FSD player state` :type "FSDPlayerState Object Reference"))
  (returns (`gear stat out` :type "GearStatEntry Structure"))
  (return))

(fn `OnTriggerAI`
  (params (TriggerName :type Name))
  (returns (ReturnValue :type Boolean))
  (bind _returnvalue (`parent.OnTriggerAI` TriggerName))
  (return _returnvalue))

(fn `ScareEffect`)

(fn `UserConstructionScript`)