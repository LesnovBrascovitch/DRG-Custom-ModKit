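; BP_JetBootsMovement is a Blueprint for jet boots movement, with hooks for activation, take-off, fuel and overheat.
; Its event graph adds no behavior of its own: character-set, destroy, overheat, local take-off and active-change events (local, non-local, server) only forward to the parent implementation.
; The fuel events, BeginPlay and Tick are empty stubs, so any logic in these events comes from the parent class.
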(event `FuelUpdated_Event_0`
  (params (jetFuel :type "Float (double-precision)") (overHeated :type Boolean)))

(event `self.Receive_OnCharacterSet`
  (params (Player :type "PlayerCharacter Object Reference"))
  (`parent.Receive_OnCharacterSet` Player))

(event `self.Receive_OnActiveChangedLocal`
  (params (IsActive :type Boolean) (fromTakeOff :type Boolean))
  (`parent.Receive_OnActiveChangedLocal` IsActive fromTakeOff))

(event `BindToFuelUsed`)

(event `OnFuelUsed`
  (params (jetFuel :type "Float (double-precision)") (overHeated :type Boolean)))

(event `self.Receive_OnDestroy`
  (`parent.Receive_OnDestroy`))

(event `self.Receive_OnOverheatedChanged`
  (params (NewOverHeated :type Boolean))
  (`parent.Receive_OnOverheatedChanged` NewOverHeated))

(event `self.Receive_OnActiveChangedNonLocal`
  (params (IsActive :type Boolean) (fromTakeOff :type Boolean))
  (`parent.Receive_OnActiveChangedNonLocal` IsActive fromTakeOff))

(event `self.Receive_OnTakeOffLocal`
  (`parent.Receive_OnTakeOffLocal`))

(event `self.Receive_OnActiveChangedServer`
  (params (IsActive :type Boolean) (fromTakeOff :type Boolean))
  (`parent.Receive_OnActiveChangedServer` IsActive fromTakeOff))