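; Shield generator variant of a facility power station objective, built as a thin child Blueprint that adds no logic of its own.
; BeginPlay, construction, hacking completion, widget class and connector point all pass straight through to the parent.
; LaunchPlates and the Rep_IsCharged function are left empty, with no parent calls.
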(event `self.ReceiveBeginPlay`
  (`parent.ReceiveBeginPlay`))

(event `LaunchPlates`)

(event `self.OnHackingComplete`
  (`parent.OnHackingComplete`))

(fn `GetConnectorPoint`
  (returns (OutTransform :type "Array of Transform Structure"))
  (return (`parent.GetConnectorPoint`)))

(fn `GetWidgetClass`
  (returns (ReturnValue :type "BossFightWidget Class Reference"))
  (bind _returnvalue (`parent.GetWidgetClass`))
  (return _returnvalue))

(fn `Rep_IsCharged`
  (params (IsCharged :type Boolean)))

(fn `UserConstructionScript`
  (`parent.UserConstructionScript`))