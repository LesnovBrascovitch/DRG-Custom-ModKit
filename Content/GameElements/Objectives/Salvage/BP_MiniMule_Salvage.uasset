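; BP_MiniMule_Salvage is the Mini Mule actor for the Salvage objective, built almost entirely from stubbed functions and events.
; It reports that it needs no legs, always returns the same state and ignores state changes.
; Drop pod travel, beacon, ping FX, distress audio and lost-leg detection are empty.
; BeginPlay, AI messages, leg visibility, dropship control, down-state replication and CheatRepair only forward to the parent.
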(event `self.ReceiveBeginPlay`
  (`parent.ReceiveBeginPlay`))

(event `Sphere Timeline__FinishedFunc`)

(event `Sphere Timeline__UpdateFunc`)

(event `Intensity__FinishedFunc`)

(event `Intensity__UpdateFunc`)

(event `GotoDropPod`
  (params (Droppod :type "/Game/LevelElements/Droppod/BP_DropPod_Base Object Reference")))

(event `Cheat_TeleportPlayer`)

(event `Stop Beacon`)

(event `Cheat_Repair`
  (params (user :type "PlayerCharacter Object Reference")))

(event `self.OnMessageAI`
  (params (TriggerName :type Name))
  (`parent.OnMessageAI` TriggerName))

(event `OnFallToTerrainStateChanged`
  (params (IsFalling :type Boolean)))

(event `self.OnLegsSetVisible`
  (`parent.OnLegsSetVisible`))

(event `PingFX`)

(event `self.SetControlledByDropShip`
  (params (Control :type Boolean))
  (`parent.SetControlledByDropShip` Control))

(event `self.OnRep_IsDown`
  (`parent.OnRep_IsDown`))

(event `self.CheatRepair`
  (`parent.CheatRepair`))

(fn `GetNeedsLegs`
  (returns (OutNeedsLegs :type Boolean))
  (return false))

(fn `GetState`
  (returns (NewParam :type "/Game/GameElements/Objectives/Salvage/MiniMule_State Enum"))
  (return "NewEnumerator0"))

(fn `PlayDistressAudio`)

(fn `Set Detect Lost Legs`
  (params (InDetect :type Boolean)))

(fn `SetState`
  (params (EnumValue :type "/Game/GameElements/Objectives/Salvage/MiniMule_State Enum" :default "NewEnumerator0")))

(fn `TryDestroyComponent`
  (params (Component :type "ActorComponent Object Reference")))

(fn `UserConstructionScript`)