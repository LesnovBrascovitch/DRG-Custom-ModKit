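; BP_EscortMule is the Blueprint for the escort objective's drilling vehicle, with hooks for engine, refueling, tunnel carving, drilling at the destination, repair and damage effects.
; In this file nearly every event and function is an empty stub, including the timeline and montage callbacks.
; The few implemented overrides only forward to the parent class, covering objective state, extractor slots, path readiness, carving replication, damage effects and targeting queries.
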(event `self.ReceiveBeginPlay`
  (`parent.ReceiveBeginPlay`))

(event `self.ReceiveTick`
  (params (DeltaSeconds :type "Float (single-precision)"))
  (`parent.ReceiveTick` DeltaSeconds))

(event `HammerDrillTest__FinishedFunc`)

(event `HammerDrillTest__UpdateFunc`)

(event `HammerDrillTest__HitEvents__EventFunc`)

(event `MoveCloser__FinishedFunc`)

(event `MoveCloser__UpdateFunc`)

(event `Timeline_MoveDrillOut__FinishedFunc`)

(event `Timeline_MoveDrillOut__UpdateFunc`)

(event `OnNotifyEnd_654993624EF7011EBE481AB20B9D51EC`
  (params (NotifyName :type Name)))

(event `OnNotifyBegin_654993624EF7011EBE481AB20B9D51EC`
  (params (NotifyName :type Name)))

(event `OnInterrupted_654993624EF7011EBE481AB20B9D51EC`
  (params (NotifyName :type Name)))

(event `OnBlendOut_654993624EF7011EBE481AB20B9D51EC`
  (params (NotifyName :type Name)))

(event `OnCompleted_654993624EF7011EBE481AB20B9D51EC`
  (params (NotifyName :type Name)))

(event `self.OnObjectiveStateChanged`
  (params (oldState :type "EEscortMissionState Enum" :default "Stationary"))
  (`parent.OnObjectiveStateChanged` oldState))

(event `StateChanged`
  (params (OldState :type "EEscortMissionState Enum" :default "Stationary")))

(event `EngineStartFX`)

(event `EngineStopFX`)

(event `RefuelCompleteFx`)

(event `DrillingAtDestinationFx`)

(event `ShellCrackedFx`)

(event `RefreshPathfindingCollision`)

(event `VehicleDestroyedFx`)

(event `self.OnExtractorSlotChanged`
  (params (Slot :type "EscortMuleExtractorSlot Structure (by ref)") (Index :type Integer))
  (`parent.OnExtractorSlotChanged` Slot Index))

(event `ChechHover`)

(event `SetActiveRepair`
  (params (Collider :type "PrimitiveComponent Object Reference") (ActiveRepairMest :type "SkeletalMeshComponent Object Reference")))

(event `ExplodeRepair`
  (params (Collider :type "SkeletalMeshComponent Object Reference")))

(event `ShellCracked`
  (params (numberOfShellsCracked :type Integer)))

(event `self.OnRep_IsCarvingTunnel`
  (`parent.OnRep_IsCarvingTunnel`))

(event `UpdateCarvingState`)

(event `SetDrillAtTargetActive`
  (params (IsActive :type Boolean)))

(event `SetDrillCooldown`
  (params (Seconds :type "Float (double-precision)")))

(event `TryDamageSound`
  (params (Attacker :type "Actor Object Reference")))

(event `self.ShowDamageEffects`
  (params (Particles :type "ParticleSystem Object Reference") (Location :type "Vector Structure") (Orientation :type "Rotator Structure"))
  (`parent.ShowDamageEffects` Particles Location Orientation))

(event `All_PlayDamageSound`
  (params (Location :type "Vector_NetQuantize Structure")))

(event `SpawnDamageEffects`
  (params (EmitterTemplate :type "ParticleSystem Object Reference") (Location :type "Vector_NetQuantize Structure") (Rotation :type "Rotator Structure")))

(event `CheckRepair`)

(event `On Damage Enemy While Riding`
  (params (EnemyHealth :type "Health Interface (by ref)") (Damage :type "Float (double-precision)") (DamageModifier :type "Float (double-precision)") (HealthRemaining :type "Float (double-precision)") (IsWeakpoint :type Boolean) (IsRadial :type Boolean)))

(event `All_PlayPetAnimation`)

(event `TestDorettaHead`)

(event `self.PathIsReady`
  (`parent.PathIsReady`))

(event `SetButtonUsable`
  (params (canUse :type Boolean)))

(event `OnCheat_SetMuleSpeed`
  (params (floatValue :type "Float (double-precision)")))

(fn `AllCanistersFull`
  (returns (areFull :type Boolean))
  (return false))

(fn `CreateCanister`
  (params (NewItem_Usable :type "InstantUsable Object Reference") (MeshComponent :type "SkinnedMeshComponent Object Reference") (Widget :type "WidgetComponent Object Reference")))

(fn `GetIsTargetable`
  (returns (ReturnValue :type Boolean))
  (return (`parent.GetIsTargetable`)))

(fn `GetTargetCenterMass`
  (returns (ReturnValue :type "Vector Structure"))
  (return (`parent.GetTargetCenterMass`)))

(fn `GetTargetHealthComponent`
  (returns (ReturnValue :type "HealthComponentBase Object Reference"))
  (return (`parent.GetTargetHealthComponent`)))

(fn `HandleCannisterUsed`
  (params (User :type "PlayerCharacter Object Reference") (Usable :type "InstantUsable Object Reference")))

(fn `IsFriendlyFire`
  (params (Object :type "Actor Object Reference"))
  (returns (bSuccess :type Boolean))
  (return false))

(fn `OnRep_DrillPaused`)

(fn `RepComponentDamage`)

(fn `SetBothCannistersVisibility`
  (params (IsVisible :type Boolean)))

(fn `SetupParticleMaterials`)

(fn `TryPlayDamageSound`
  (params (Location :type "Vector Structure")))

(fn `Update Moving FX`
  (params (InState :type "EEscortMissionState Enum" :default "Stationary")))

(fn `UpdateBoxDamageEmitter`
  (params (ParticlesLow :type "NiagaraComponent Object Reference") (ParticlesMedium :type "NiagaraComponent Object Reference") (ParticlesHigh :type "NiagaraComponent Object Reference") (HealthPercent :type "Float (double-precision)")))

(fn `UpdateRepairBoxLook`)

(fn `UserConstructionScript`)