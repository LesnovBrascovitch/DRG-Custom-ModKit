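; BP_Refinery is the refinery level-element Blueprint, a skeleton that adds no behavior of its own.
; BeginPlay, drop pod impact, refinery and pipeline state changes, and drilling start only forward to the parent class.
; Events for audio, GFX, camera shake, enemies, mission shouts and use UI are empty, as are landing zone, pipeline shout and pathfinder blocker functions.
; HasRequiredSecondary always returns false.
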(event `self.ReceiveBeginPlay`
  (`parent.ReceiveBeginPlay`))

(event `self.OnDroppodImpact`
  (`parent.OnDroppodImpact`))

(event `self.ReceiveRefineryStateChanged`
  (params (InState :type "ERefineryState Enum" :default "Landing"))
  (`parent.ReceiveRefineryStateChanged` InState))

(event `EnemiesOnStateChanged`)

(event `Mission Shouts on State Changed`)

(event `self.ReceivePipelineStateChanged`
  (params (InPipeline :type "PipelineStart Object Reference") (InState :type "EPipelineBuildState Enum" :default "NotStarted"))
  (`parent.ReceivePipelineStateChanged` InPipeline InState))

(event `self.OnDrillingStarted`
  (`parent.OnDrillingStarted`))

(event `AudioOnStateChanged`)

(event `OnDropStartedGFX`)

(event `OnDropImpactGFX`)

(event `SetupUseButtonUI`)

(event `CameraShakeOnStateChange`)

(event `UpdateUseIcon`)

(fn `ActivatePathfinderBlockers`)

(fn `CheckPipelineMissionShout`
  (params (InPipelineStart :type "PipelineStart Object Reference") (InPipelineState :type "EPipelineBuildState Enum" :default "NotStarted")))

(fn `HasRequiredSecondary`
  (returns (ReturnValue :type Boolean))
  (return false))

(fn `Spawn Landing Zone`)

(fn `UserConstructionScript`)