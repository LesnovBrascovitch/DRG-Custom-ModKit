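; Refinery pipeline segment Blueprint, with hooks for placement, build progress, breakage and repair of a segment.
; Placement, activation progress, broken-state and repair events only forward to the parent implementation.
; The GFX, audio, carving, numbering and timeline handlers are empty stubs, as are the construction script and visual update functions.
; IsPhotosensitiveMode always returns false and HandlePhotosensitivity does nothing, so this graph adds no behavior of its own.
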(event `self.ReceiveBeginPlay`
  (`parent.ReceiveBeginPlay`))

(event `BuildTimeline__FinishedFunc`)

(event `BuildTimeline__UpdateFunc`)

(event `Timeline_0__FinishedFunc`)

(event `Timeline_0__UpdateFunc`)

(event `self.ReceivPlacementValidChanged`
  (params (InIsValid :type Boolean))
  (`parent.ReceivPlacementValidChanged` InIsValid))

(event `self.ReceivePlacementStateChanged`
  (params (NewState :type "ETrackBuildPlacementState Enum" :default "NotBeingPlaced"))
  (`parent.ReceivePlacementStateChanged` NewState))

(event `ReversePipelineAnim`)

(event `Update Can Undo`)

(event `self.ReceiveSegmentBrokenChanged`
  (params (InSegmentBroken :type Boolean))
  (`parent.ReceiveSegmentBrokenChanged` InSegmentBroken))

(event `self.ReceivePlacementFinished`
  (`parent.ReceivePlacementFinished`))

(event `UpdateCanActivateSegmentGFX`)

(event `ScheduleUpdatePlacementState`)

(event `CarveAroundSegment`)

(event `self.ReceiveSegmentActivatedProgress`
  (params (InProgress :type "Float (single-precision)"))
  (`parent.ReceiveSegmentActivatedProgress` InProgress))

(event `self.OnRepaired`
  (params (InUser :type "PlayerCharacter Object Reference"))
  (`parent.OnRepaired` InUser))

(event `Hide Endpost Items`)

(event `SetupPipelineNumber`)

(event `SegmentBrokenGFX`)

(event `SegmentBrokenLocalWave`)

(event `SegmentBrokenLaserpointerInfo`)

(event `SegmentBrokenAudio`)

(event `self.ReceivePlacementBegin`
  (`parent.ReceivePlacementBegin`))

(event `ParticlesOnPlaced`)

(fn `HandlePhotosensitivity`)

(fn `IsPhotosensitiveMode`
  (returns (ReturnValue :type Boolean))
  (return false))

(fn `OverrideEndPostMaterial`
  (params (Material :type "MaterialInterface Object Reference")))

(fn `UpdateConnectableGFX`)

(fn `UpdatePipelineNumber`)

(fn `UpdatePlacementState`
  (params (InState :type "ETrackBuildPlacementState Enum" :default "NotBeingPlaced")))

(fn `UserConstructionScript`)