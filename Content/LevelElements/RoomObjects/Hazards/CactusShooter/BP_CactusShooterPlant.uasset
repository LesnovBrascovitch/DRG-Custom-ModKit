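; BP_CactusShooterPlant is a cactus hazard that fires volleys of PRJ_CactusSpike projectiles in random directions.
; ShootTheSpikes re-arms itself on a ResetTime timer, then spawns NumSpikes spikes at random heights above the actor origin, each ignoring the plant when moving.
; Nothing live here starts that cycle: the trigger overlap and PlayerNearby events are empty, and the CanTrigger cooldown logic is disconnected.
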(event `self.ReceiveBeginPlay`
  (`parent.ReceiveBeginPlay`))

(event `OnTerrainPointRemoved`)

(event `PlayerNearby`
  (params (player :type "PlayerCharacter Object Reference") (enteredTrigger :type Boolean)))

(event `ShootTheSpikes`
  (bind (_spikeoriginheightminmax_x _spikeoriginheightminmax_y) (`KismetMathLibrary.BreakVector2D` (`self.SpikeOriginHeightMinMax`)))
  (`KismetSystemLibrary.K2_SetTimerDelegate` (delegate `ShootTheSpikes`) (`self.ResetTime`))
  (for _ (range 1 (+ (`self.NumSpikes`) 1))
    (bind _returnvalue (`|SpawnActorFromClass` "/Game/LevelElements/RoomObjects/Hazards/CactusShooter/PRJ_CactusSpike.PRJ_CactusSpike_C" (`KismetMathLibrary.MakeTransform` (+ (`self.K2_GetActorLocation`) (`KismetMathLibrary.MakeVector` 0.0 0.0 (`KismetMathLibrary.RandomFloatInRange` _spikeoriginheightminmax_x _spikeoriginheightminmax_y))) (`KismetMathLibrary.RandomRotator` false)) "AdjustIfPossibleButAlwaysSpawn" "OverrideRootScale" self null))
    (`PrimitiveComponent.IgnoreActorWhenMoving` (`ProjectileBase.CollisionComponent` _returnvalue) self true)))

(event `self.ShootSpinesTrigger.OnComponentBeginOverlap`
  (params (OverlappedComponent :type "PrimitiveComponent Object Reference") (OtherActor :type "Actor Object Reference") (OtherComp :type "PrimitiveComponent Object Reference") (OtherBodyIndex :type Integer) (bFromSweep :type Boolean) (SweepResult :type "HitResult Structure (by ref)")))

(fn `UserConstructionScript`)