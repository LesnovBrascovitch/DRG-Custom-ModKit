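; Hoops minigame for the Space Rig bar, with a hoop that slides back and forth between a left and a right destination.
; Tick moves the hoop at constant speed with VInterpToConstant, flipping IsMovingRightServer when it nears either end.
; Events for scoring, hoop entries, restart and combo-loss audio, plus the OnRep functions, are empty stubs, and GetBarrelScoreData returns zero points.
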(event `self.ReceiveBeginPlay`
  (`parent.ReceiveBeginPlay`))

(event `self.ReceiveTick`
  (params (DeltaSeconds :type "Float (single-precision)"))
  (bind _hoop (`self.Hoop`))
  (`parent.ReceiveTick` DeltaSeconds)
  (`SceneComponent.K2_SetRelativeLocation` _hoop (`KismetMathLibrary.VInterpTo_Constant` (`SceneComponent.RelativeLocation` _hoop) (`KismetMathLibrary.SelectVector` (`SceneComponent.RelativeLocation` (`self.DestinationRight`)) (`SceneComponent.RelativeLocation` (`self.DestinationLeft`)) (`self.IsMovingRightServer`)) DeltaSeconds 333.0) false false)
  (if (== (`SceneComponent.RelativeLocation` (`self.Hoop`)) (`SceneComponent.RelativeLocation` (`self.DestinationRight`)) :`ErrorTolerance` 5.0)
    (set `self.IsMovingRightServer` false)
    (elif (== (`SceneComponent.RelativeLocation` (`self.Hoop`)) (`SceneComponent.RelativeLocation` (`self.DestinationLeft`)) :`ErrorTolerance` 5.0)
      (set `self.IsMovingRightServer` true))))

(event `Restart`)

(event `StoreScore`
  (params (NewScore :type Integer)))

(event `Cheat_ToggleHoopGameMovement`)

(event `Set Latest Barrel kicker`
  (params (`Kicked by` :type "PlayerCharacter Object Reference")))

(event `On Barrel In Hoop`
  (params (Barrel :type "/Game/Art/Environments/SpaceRig/BP_Phys_Barrel01 Object Reference")))

(event `On Barglass In Hoop`
  (params (Glass :type "/Game/GameElements/Bar/Bar_Glass_Physics Object Reference")))

(event `On Player In Hoop`
  (params (Player :type "PlayerCharacter Object Reference")))

(event `OnSpaceballInHoop`
  (params (ScoreToAdd :type Integer)))

(event `All_PlayComboLostSFX`)

(fn `GetBarrelScoreData`
  (params (Barrel :type "/Game/Art/Environments/SpaceRig/BP_Phys_Barrel01 Object Reference"))
  (returns (Audio :type "SoundCue Object Reference") (OutBarrel :type "/Game/Art/Environments/SpaceRig/BP_Phys_Barrel01 Object Reference") (Points :type Integer))
  (return null null 0))

(fn `OnRep_ComboMultiplier`)

(fn `OnRep_CurrentScore`)

(fn `OnRep_IsMovingRightServer`)

(fn `OnRep_Scores`)

(fn `UserConstructionScript`)