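; BP_DropPod_Escape_Damaged is a child Blueprint for a damaged variant of the escape drop pod.
; Begin play, construction, mule-loaded and powering-up events only forward to the parent.
; A DistressLightIntensity timeline, a match-started event and a photosensitivity handler for the damaged pod are present but have empty bodies.
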(event `self.ReceiveBeginPlay`
  (`parent.ReceiveBeginPlay`))

(event `DistressLightIntensity__FinishedFunc`)

(event `DistressLightIntensity__UpdateFunc`)

(event `/Game/LevelElements/Droppod/BP_DropPod_Base.OnMuleLoaded`
  (`parent.OnMuleLoaded`))

(event `OnMatchStarted_Event_0`)

(event `self.OnPoweringUp`
  (`parent.OnPoweringUp`))

(event `self.OnPoweredUp`
  (`parent.OnPoweredUp`))

(fn `Handle PhotosenitivityDamagedPod`)

(fn `UserConstructionScript`
  (`parent.UserConstructionScript`))