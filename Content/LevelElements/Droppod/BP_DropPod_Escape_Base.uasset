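; BP_DropPod_Escape_Base is a base Blueprint for the escape drop pod, exposing hooks for impact, drilling, departure, mule loading, characters boarding and return timers.
; It adds no behavior of its own: most events simply forward to the parent implementation, and a few are empty.
; Functions such as GetFrontLocation, IsAnyCharacterInEscapePod and LockCharactersInPod are placeholder stubs that do nothing or return default values.
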(event `self.ReceiveBeginPlay`
  (`parent.ReceiveBeginPlay`))

(event `self.OnDroppodImpact`
  (`parent.OnDroppodImpact`))

(event `self.OnDrillingStarted`
  (`parent.OnDrillingStarted`))

(event `OnDonkeyReachedDropShip`)

(event `self.OnDeparting`
  (`parent.OnDeparting`))

(event `self.OnPrepForTakeOff`
  (`parent.OnPrepForTakeOff`))

(event `self.OnMuleLoaded`
  (`parent.OnMuleLoaded`))

(event `self.OnCharacterEnter`
  (params (Character :type "PlayerCharacter Object Reference"))
  (`parent.OnCharacterEnter` Character))

(event `self.OnCharacterExit`
  (params (Character :type "PlayerCharacter Object Reference"))
  (`parent.OnCharacterExit` Character))

(event `HandleHurryShouts`)

(event `self.OnRepDoorState`
  (`parent.OnRepDoorState`))

(event `OnMuleBayOpenedDispatch_Event_1`)

(event `self.ForceTakeoff`
  (`parent.ForceTakeoff`))

(event `self.RecieveReturnTimerFifteenSecondWarning`
  (`parent.RecieveReturnTimerFifteenSecondWarning`))

(event `self.RecieveReturnTimerExpired`
  (`parent.RecieveReturnTimerExpired`))

(event `self.OnAllDwavesInsidePod`
  (params (AllInside :type Boolean))
  (`parent.OnAllDwavesInsidePod` AllInside))

(fn `DisableDynamicElements`
  (params (Enabled :type Boolean)))

(fn `GetFrontLocation`
  (returns (DoorLocation :type "Vector Structure"))
  (return (0.0 0.0 0.0)))

(fn `HandlePhotosentitivity`)

(fn `IsAnyCharacterInEscapePod`
  (returns (EscapePodPopulated :type Boolean))
  (return false))

(fn `LockCharactersInPod`)

(fn `UserConstructionScript`
  (`parent.UserConstructionScript`))