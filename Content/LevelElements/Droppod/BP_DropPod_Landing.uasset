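; Landing variant of the drop pod, layered on a parent pod class that is notified of impact, drilling, departure and characters entering or leaving.
; Most events simply forward to the parent.
; The only added behavior is on impact, where it calls the parent and then deactivates an audio component and the door rocks particle system.
; The spawn point, attach, fade and audio helper functions have no logic here.
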(event `self.ReceiveBeginPlay`
  (`parent.ReceiveBeginPlay`))

(event `self.OnAllPlayersLeftPod`
  (`parent.OnAllPlayersLeftPod`))

(event `self.OnDroppodImpact`
  (`parent.OnDroppodImpact`)
  (`ActorComponent.Deactivate` (`self.Audio_0`))
  (`ActorComponent.Deactivate` (`self.ParticleSystem_DroppodDoorRocks`)))

(event `self.OnDrillingStarted`
  (`parent.OnDrillingStarted`))

(event `self.OnDeparting`
  (`parent.OnDeparting`))

(event `self.OnCharacterEnter`
  (params (Character :type "PlayerCharacter Object Reference"))
  (`parent.OnCharacterEnter` Character))

(event `self.OnCharacterExit`
  (params (Character :type "PlayerCharacter Object Reference"))
  (`parent.OnCharacterExit` Character))

(event `OnPlayerCharacterRegistered`
  (params (PlayerCharacter :type "PlayerCharacter Object Reference")))

(event `StopListeningToNewPlayers`)

(event `self.OnFirstPlayerLeftPod`
  (`parent.OnFirstPlayerLeftPod`))

(fn `AttachCharacter`
  (params (PlayerCharacter :type "PlayerCharacter Object Reference")))

(fn `DetachAll`)

(fn `FadeToBlack`)

(fn `FindSpawnPoint`
  (params (Controller :type "PlayerController Object Reference"))
  (returns (Start :type "ChildActorComponent Object Reference"))
  (return null))

(fn `IsOwnedPlayerStart`
  (params (Controller :type "PlayerController Object Reference") (Component :type "ChildActorComponent Object Reference"))
  (returns (ReturnValue :type Boolean))
  (return false))

(fn `SpawnAndStoreAudio`
  (params (Sound :type "SoundBase Object Reference") (AttachToComponent :type "SceneComponent Object Reference"))
  (returns (AudioComponent :type "AudioComponent Object Reference"))
  (return null))

(fn `UserConstructionScript`
  (`parent.UserConstructionScript`))