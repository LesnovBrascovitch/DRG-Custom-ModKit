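; Drop pod variant for the rig that switches off much of the behavior of its parent drop pod Blueprint.
; BeginPlay, mission selection, countdown, host timer and team achievement events are overridden empty, so the parent's BeginPlay never runs.
; Character enter/exit, host-inside and all-dwarves-inside events still forward to the parent, as does the construction script.
; ActivePlayerCount always returns zero.
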(event `self.ReceiveBeginPlay`)

(event `OnMissionSelected`
  (params (Mission :type "GeneratedMission Object Reference")))

(event `self.OnAllDwavesInsidePod`
  (params (AllInside :type Boolean))
  (`parent.OnAllDwavesInsidePod` AllInside))

(event `self.OnHostInsidePod`
  (params (isInside :type Boolean))
  (`parent.OnHostInsidePod` isInside))

(event `OnCountdownCompleted`)

(event `OnHostTimerChanged`
  (params (NewTime :type "Float (double-precision)")))

(event `Check for ATeamAchievement`)

(event `self.OnCharacterEnter`
  (params (Character :type "PlayerCharacter Object Reference"))
  (`parent.OnCharacterEnter` Character))

(event `self.OnCharacterExit`
  (params (Character :type "PlayerCharacter Object Reference"))
  (`parent.OnCharacterExit` Character))

(fn `ActivePlayerCount`
  (returns (ReturnValue :type Integer))
  (return 0))

(fn `UserConstructionScript`
  (`parent.UserConstructionScript`))