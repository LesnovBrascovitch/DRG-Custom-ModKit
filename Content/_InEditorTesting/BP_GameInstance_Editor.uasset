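; Editor-testing game instance that stores weapon and vanity settings and makes sure an EDTS_MainSettings actor is active once loading completes.
; On load complete it triggers ExecuteLogicsMessage on an existing settings actor, or spawns one with the stored mod spawn settings, printing a debug string either way.
; Save and Get functions hold the weapon loadout, skins and armor vanity item.
; The EDTS_VanityEditor spawn is disconnected and never runs.
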(event `self.OnLoadComplete`
  (params (MapName :type String))
  (bind _returnvalue (`GameplayStatics.GetActorOfClass` "/Game/_InEditorTesting/Initialization/EDTS_MainSettings.EDTS_MainSettings_C"))
  (`/Engine/EditorBlueprintResources/StandardMacros.IsValid` _returnvalue
    (:`Is Valid`
      (message `/Game/_InEditorTesting/Initialization/BPI_Initialization.ExecuteLogics` _returnvalue)
      (`KismetSystemLibrary.PrintString` "fdawdawdawHello" true true (struct :`G` 0.66 :`B` 1.0 :`A` 1.0) 15.0))
    (:`Is Not Valid`
      (`|SpawnActorFromClass` "/Game/_InEditorTesting/Initialization/EDTS_MainSettings.EDTS_MainSettings_C" (`KismetMathLibrary.MakeTransform` (0.0 0.0 0.0)) "AlwaysSpawn" "OverrideRootScale" null (`self.Mod Spawn Settings`) true null)
      (`KismetSystemLibrary.PrintString` "fdawdawdawHello" true true (struct :`R` 0.159453 :`G` 1.0 :`A` 1.0) 15.0))))

(fn `GetVanitySettings`
  (returns (`Armor Vanity Item` :type "ArmorVanityItem Object Reference"))
  (return (`self.Armor Vanity Item`)))

(fn `GetWeaponSettings`
  (returns (`Initial Weapon to Equip` :type "Item Class Reference") (`Grenade Class` :type "Grenade Class Reference") (Items :type "Array of Item Class Reference") (`Item Skins` :type "Map of Item Class Reference to ItemSkin Object Reference"))
  (return (`self.Initial Weapon to Equip`) (`self.Grenade Class`) (`self.Items`) (`self.Item Skins`)))

(fn `SaveVanitySettings`
  (params (`Armor Vanity Item` :type "ArmorVanityItem Object Reference"))
  (set `self.Armor Vanity Item` `Armor Vanity Item`))

(fn `SaveWeaponSettings`
  (params (`Initial Weapon to Equip` :type "Item Class Reference") (`Grenade Class` :type "Grenade Class Reference") (Items :type "Array of Item Class Reference") (`Item Skins` :type "Map of Item Class Reference to ItemSkin Object Reference"))
  (set `self.Initial Weapon to Equip` `Initial Weapon to Equip`)
  (set `self.Item Skins` `Item Skins`)
  (set `self.Items` Items)
  (set `self.Grenade Class` `Grenade Class`))