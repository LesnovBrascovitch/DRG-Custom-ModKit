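; In-editor testing Blueprint that gives the player character a configured loadout at BeginPlay, once a valid SBZ player character is obtained.
; It adds each listed item class to the inventory, then applies any mapped skin by blocking-loading its mesh onto the first-person mesh and disabling shadow casting.
; It equips the chosen initial weapon class, falling back to the inventory's second selectable actor if none matches.
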(event `self.ReceiveBeginPlay`
  (bind _returnvalue (`/Game/_DRGModding/_LesnovMods/_SharedAssets/BML_Actor.ValidCheck(Wait | SBZPlayerCharacter)`))
  (set `self.NewVar_0` _returnvalue)
  (`self.Add Items to Inventory Comp`)
  (`self.EquipActorByItemClass` (`self.InitialWeaponToEquip`)))

(fn `Add Items to Inventory Comp`
  (locals (NewLocalVar_0 :type "Item Object Reference"))
  (bind _inventorycomponent (`PlayerCharacter.InventoryComponent` (`self.NewVar_0`)))
  (bind _actorsselectable (`InventoryBase.ActorsSelectable` _inventorycomponent))
  (for _array_element (`self.Items`)
    (`InventoryComponent.AddItemClass` _inventorycomponent _array_element)
    (bind _asanimated_item (cast `AnimatedItem` (`|GetArrayItem` _actorsselectable (`KismetArrayLibrary.Array_LastIndex` _actorsselectable))))
    (bind (_value _returnvalue) (`BlueprintMapLibrary.Map_Find` (`self.NewVar_1`) (`GameplayStatics.GetObjectClass` _asanimated_item)))
    (if _returnvalue
      (bind _asskeletal_mesh_skin_effect (cast `SkeletalMeshSkinEffect` (`ItemSkin.SkinEffect` _value)))
      (bind _mesh (`SkeletalMeshSkinEffect.Mesh` _asskeletal_mesh_skin_effect))
      (`KismetSystemLibrary.LoadAsset_Blocking` _mesh)
      (bind _fpmesh (`AnimatedItem.FPMesh` _asanimated_item))
      (`SkinnedMeshComponent.SetSkinnedAssetAndUpdate` _fpmesh (`|ConvertAsset` _mesh) true)
      (`PrimitiveComponent.SetCastShadow` _fpmesh false))))

(fn `EquipActorByItemClass`
  (params (Item :type "Item Class Reference"))
  (locals (IsFound :type Boolean))
  (bind _inventorycomponent (`PlayerCharacter.InventoryComponent` (`self.NewVar_0`)))
  (bind _actorsselectable (`InventoryBase.ActorsSelectable` (`PlayerCharacter.InventoryComponent` (`self.NewVar_0`))))
  (bind _output (`|GetArrayItem` _actorsselectable 1))
  (for _array_element _actorsselectable
    (if (== (`self.InitialWeaponToEquip`) (`GameplayStatics.GetObjectClass` _array_element))
      (`InventoryComponent.Equip` _inventorycomponent (cast `Item` _array_element :!pure true))
      (set `local.IsFound` true)
      (break)))
  (`/Engine/EditorBlueprintResources/StandardMacros.IsValid` _output
    (:`Is Valid`
      (if (not (`local.IsFound`))
        (`InventoryComponent.Equip` _inventorycomponent (cast `Item` _output :!pure true))))))

(fn `UserConstructionScript`)