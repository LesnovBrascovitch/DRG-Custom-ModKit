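; BP_VanityEditor is an in-editor testing actor that applies an armor vanity item's first-person mesh to the player character.
; On BeginPlay it obtains the SBZ player character through a wait-and-validity check and stores it.
; It then async loads the first value in the item's FPArmorMesh map and sets it on the character's FPMesh, reinitializing the pose.
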(event `self.ReceiveBeginPlay`
  (bind _returnvalue (`/Game/_DRGModding/_LesnovMods/_SharedAssets/BML_Actor.ValidCheck(Wait | SBZPlayerCharacter)`))
  (set `self.NewVar_0` _returnvalue)
  (bind _values (`BlueprintMapLibrary.Map_Values` (`ArmorVanityItem.FPArmorMesh` (`self.ArmorVanityItem`))))
  (bind _output (`|GetArrayItem` _values))
  (`|LoadAsset` _output
    (:`Completed`
      (`SkinnedMeshComponent.SetSkinnedAssetAndUpdate` (`PlayerCharacter.FPMesh` (`self.NewVar_0`)) (`|ConvertAsset` _output) true))))

(fn `UserConstructionScript`)