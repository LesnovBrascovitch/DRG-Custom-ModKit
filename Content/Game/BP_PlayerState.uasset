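; BP_PlayerState is a player state Blueprint with hooks for character selection, late join, respawn and spawning, resupply classes and Deep Dive credit rewards.
; BeginPlay, late-join completion, character selection and the credit reward calculation only forward to the parent class.
; The remaining events, spawn functions and resupply class getters are empty stubs, so the file adds no logic of its own.
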(event `self.ReceiveBeginPlay`
  (`parent.ReceiveBeginPlay`))

(event `OnLoaded_E2B28351414D5B2A20966496F0955946`
  (params (Loaded :type "Object Class Reference")))

(event `OnLoaded_97A4F0694E71C770F24EA6A654B14857`
  (params (Loaded :type "Object Class Reference")))

(event `self.OnLateJoinFinished`
  (`parent.OnLateJoinFinished`))

(event `LogState`)

(event `self.CharacterSelected`
  (`parent.CharacterSelected`))

(event `TestLatjoin`)

(event `RespawnPlayer`)

(fn `GetDeepDiveCreditsReward`
  (params (StagesCompleted :type Integer) (goldCollected :type Integer))
  (returns (ReturnValue :type "Array of CreditsReward Structure"))
  (return (`parent.GetDeepDiveCreditsReward` StagesCompleted goldCollected)))

(fn `GetRessuplySpawnClass`
  (returns (PodSpawnClass :type "RessuplyPodSpawn Class Reference"))
  (return null))

(fn `GetRessupyBeaconClass`
  (returns (PodSpawnClass :type "Actor Class Reference"))
  (return null))

(fn `SpawnPlayerDirectly`
  (params (Player :type "Controller Object Reference")))

(fn `SpawnPlayerInPod`
  (params (Player :type "FSDPlayerController Object Reference")))

(fn `UserConstructionScript`)