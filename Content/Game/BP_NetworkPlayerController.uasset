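; Network player controller Blueprint with an interface for hero selection, client travel, reconnect display and UI cleanup, almost entirely unimplemented here.
; Server and client events for requesting, receiving and confirming a non-taken hero have empty bodies, as do the back, possession and reconnect handlers.
; BeginPlay, pre-client travel, destruction and construction only call the parent, Tick is disabled, and the helper functions are empty or return no value.
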(event `self.ReceiveBeginPlay`
  (`parent.ReceiveBeginPlay`))

(event `OnBack`)

(event `OnPlayerCharacterPossesed_Event`
  (params (pawn :type "Pawn Object Reference")))

(event `Server_RequestNonTakenHero`)

(event `Client_RecieveNonTakenHero`
  (params (`New Character` :type "PlayerCharacterID Object Reference")))

(event `Server_SetCharacterSelected`)

(event `self.RecievePreClientTravel`
  (`parent.RecievePreClientTravel`))

(event `self.ReceiveDestroyed`
  (`parent.ReceiveDestroyed`))

(event `ShowReconnect`
  (params (Show :type Boolean)))

(fn `CleanupUI`)

(fn `CollapseAndRemoveFromParent`
  (params (widget :type "Widget Object Reference")))

(fn `GetLoaderScreenUIClass`
  (returns (ReturnValue :type "UserWidget Class Reference"))
  (return null))

(fn `GetNonTakenHero`
  (returns (SelectedClass :type "PlayerCharacterID Object Reference"))
  (return null))

(fn `UserConstructionScript`
  (`parent.UserConstructionScript`))