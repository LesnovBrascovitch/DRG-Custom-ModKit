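; GM_Motherlode is a game mode Blueprint named for Motherlode, serving as a mostly empty shell over its parent class.
; BeginPlay, mission-critical item spawning and construction only forward to the parent, and Tick is disabled.
; The match start, countdown, rocket launch and spawn-location replication hooks are empty.
; The landing zone getter returns a zero vector, and the mine head getter returns nothing.
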(event `self.ReceiveBeginPlay`
  (`parent.ReceiveBeginPlay`))

(event `OnMatchStarted_`)

(event `OnCountdownFinished`)

(event `RocketLaunched`)

(event `self.SpawnMissionCriticalItems`
  (params (pass :type "ECriticalItemPass Enum (by ref)" :default "LargePass"))
  (`parent.SpawnMissionCriticalItems` pass))

(fn `GetLandingZoneLocation`
  (returns (Output :type "Vector Structure"))
  (return (0.0 0.0 0.0)))

(fn `GetMineHead`
  (returns (Output :type "/Game/LevelElements/Minehead/BP_MineHead Object Reference"))
  (return null))

(fn `OnRep_SelectedSpawnLocation`)

(fn `UserConstructionScript`
  (`parent.UserConstructionScript`))