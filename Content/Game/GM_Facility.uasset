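; GM_Facility is the game mode Blueprint for a facility mission, with hooks for objectives, shield generators, overcharger waves and facility destruction.
; Its events cover generators connecting by tetherline, calling chargers and finishing charging, plus starting and stopping overcharger waves and finding generator and target rooms.
; All bodies are empty stubs or parent calls (begin play, mission-critical item spawning, objective initialization, donkey button), so the file holds no logic of its own.
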(event `self.ReceiveBeginPlay`
  (`parent.ReceiveBeginPlay`))

(event `OnLoaded_363A1A82446FF4B3B30843A806542007`
  (params (Loaded :type "Object Object Reference")))

(event `SetObjective`
  (params (Objective :type "/Game/GameElements/Objectives/Facility/OBJ_1st_Facility Object Reference")))

(event `FacilityActivated`)

(event `OnFacilityDestroyed`)

(event `Damaged`)

(event `self.SpawnMissionCriticalItems`
  (params (pass :type "ECriticalItemPass Enum (by ref)" :default "LargePass"))
  (`parent.SpawnMissionCriticalItems` pass))

(event `GeneratorCharged`
  (params (Generator :type "/Game/GameElements/Objectives/Facility/ShieldGenerator/BP_Facility_PowerStation_GeneratorBase Object Reference")))

(event `OnOverchargerCalled`
  (params (Location :type "Vector Structure") (RoomIndex :type Integer)))

(event `SubscribeToShieldEvents`
  (params (Generator :type "/Game/GameElements/Objectives/Facility/ShieldGenerator/BP_Facility_PowerStation_GeneratorBase Object Reference")))

(event `Recieve_Charged`
  (params (Generator :type "/Game/GameElements/Objectives/Facility/ShieldGenerator/BP_Facility_PowerStation_GeneratorBase Object Reference")))

(event `Recieve_ChargerCalled`
  (params (Location :type "Vector Structure") (RoomIndex :type Integer)))

(event `Recieve_FirstConnected`
  (params (Generator :type "/Game/GameElements/Objectives/Facility/ShieldGenerator/BP_Facility_PowerStation_GeneratorBase Object Reference") (tetherlineStart :type "TetherComponent Object Reference")))

(event `self.OnObjectivesInitialized`
  (`parent.OnObjectivesInitialized`))

(event `self.DonkeyButtonPressed`
  (`parent.DonkeyButtonPressed`))

(event `StartOverChargerWave`
  (params (ShieldGenerator :type "/Game/GameElements/Objectives/Facility/ShieldGenerator/BP_Facility_PowerStation_GeneratorBase Object Reference") (tetherlineStart :type "TetherComponent Object Reference")))

(fn `GetGeneratorRooms`
  (returns (Array :type "Array of Integer"))
  (return))

(fn `GetTargetRooms`)

(fn `StopOverChargerWave`
  (params (WaveOrigin :type "/Game/GameElements/Objectives/Facility/ShieldGenerator/BP_Facility_PowerStation_GeneratorBase Object Reference")))

(fn `UserConstructionScript`
  (`parent.UserConstructionScript`))