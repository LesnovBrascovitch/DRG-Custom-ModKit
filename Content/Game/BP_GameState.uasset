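; BP_GameState is a game state Blueprint that serves mostly as a thin shell over its parent class.
; BeginPlay, Tick, seamless travel handling and the playable character ID getter only forward to the parent.
; StartGame, a placeholder custom event, the construction script, and the animation sharing and random initial hero functions contain no logic.
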(event `self.ReceiveBeginPlay`
  (`parent.ReceiveBeginPlay`))

(event `self.ReceiveTick`
  (params (DeltaSeconds :type "Float (single-precision)"))
  (`parent.ReceiveTick` DeltaSeconds))

(event `StartGame`)

(event `self.HandleSeamlessTravelEvent`
  (`parent.HandleSeamlessTravelEvent`))

(event `CustomEvent_0`)

(fn `GetAnimSharingAssets`
  (params (AnimSharing :type "AnimationSharingSetup Soft Object Reference"))
  (returns (Assets :type "Array of Object Soft Object Reference"))
  (return))

(fn `GetPlayableCharacterIDs`
  (returns (ReturnValue :type "Array of PlayerCharacterID Object Reference"))
  (return (`parent.GetPlayableCharacterIDs`)))

(fn `GetRandomIntialHero`
  (returns (HeroClass :type "PlayerCharacterID Object Reference"))
  (return null))

(fn `UserConstructionScript`)