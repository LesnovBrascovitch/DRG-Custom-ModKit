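; BP_NetworkPlayGameMode is a game mode Blueprint, named for network play, that adds no logic of its own.
; Its all-dwarves-down event, construction script and default pawn class lookup only forward to the parent implementations.
; BeginPlay and Tick are disabled placeholder nodes, so the behavior comes from the parent class.
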(event `self.RecieveAllDwarvesDown`
  (`parent.RecieveAllDwarvesDown`))

(fn `GetDefaultPawnClassForController`
  (params (InController :type "Controller Object Reference"))
  (returns (ReturnValue :type "Object Class Reference"))
  (bind _returnvalue (`parent.GetDefaultPawnClassForController` InController))
  (return _returnvalue))

(fn `UserConstructionScript`
  (`parent.UserConstructionScript`))