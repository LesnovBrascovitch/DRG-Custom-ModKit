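; Game mode that bootstraps a level with a save object, mule, optional drop pod and player-controlled Gunner.
; BeginPlay creates a new save on the game instance, then async-loads and spawns the mule, storing it as Donkey.
; A configured drop pod spawns at its DropHeight linked to the mule, then a Gunner spawns at a PlayerStart and is possessed.
; Other overrides are empty stubs or defer to the parent.
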(event `self.ReceiveBeginPlay`
  (bind _muleclass (`self.MuleClass`))
  (bind _droppodclass (`self.DropPodClass`))
  (bind _output (`|ConvertAsset` _droppodclass))
  (`parent.ReceiveBeginPlay`)
  (`FSDGameInstance.OnLoadComplete` (`GameFunctionLibrary.GetFSDGameInstance`) "")
  (bind _returnvalue (`GameplayStatics.CreateSaveGameObject` "/Script/FSD.FSDSaveGame"))
  (set `FSDGameInstance.SaveGame` _returnvalue (`GameFunctionLibrary.GetFSDGameInstance`))
  (`|LoadAssetClass` _muleclass
    (:`Completed`
      (bind _returnvalue_2 (`|SpawnActorFromClass` (`|ConvertAsset` _muleclass) (`KismetMathLibrary.MakeTransform` (0.0 0.0 0.0)) "AlwaysSpawn" "OverrideRootScale" null null))
      (set `FSDGameInstance.Donkey` _returnvalue_2 (`GameFunctionLibrary.GetFSDGameInstance`))
      (if (`KismetSystemLibrary.IsValidSoftClassReference` (`self.DropPodClass`))
        (`ActorFunctionLibrary.LoadClass` _droppodclass)
        (`|LoadAssetClass` _droppodclass
          (:`Completed`
            (bind _returnvalue_3 (`|SpawnActorFromClass` _output (`KismetMathLibrary.MakeTransform` (`KismetMathLibrary.MakeVector` 0.0 0.0 (defaults `Object` _output))) "AlwaysSpawn" "OverrideRootScale" null null))
            (`TeamTransport.SetMuleInstance` _returnvalue_3 (`FSDGameInstance.Donkey` (`GameFunctionLibrary.GetFSDGameInstance`))))))
      (bind _returnvalue_4 (`GameplayStatics.GetActorOfClass` "/Script/Engine.PlayerStart"))
      (bind _returnvalue_5 (`|SpawnActorFromClass` "/Game/Character/BP_GunnerCharacter.BP_GunnerCharacter_C" (`self.GetTransform` _returnvalue_4) "AlwaysSpawn" "OverrideRootScale" null null))
      (`Controller.Possess` (`GameplayStatics.GetPlayerController` 0) _returnvalue_5))))

(event `self.RecieveEndLevel`
  (`parent.RecieveEndLevel`))

(event `WaitForGeneration`)

(event `self.Recieve_ContinueTimerEnded`
  (`parent.Recieve_ContinueTimerEnded`))

(event `Call DropPod`)

(event `Trigger End Wave`
  (params (cancelAllWaves :type Boolean)))

(event `SpawnBosco`
  (params (Location :type "Transform Structure")))

(event `RemoveBosco`)

(event `Handle Bosco Respawn`)

(event `OnPlayerLeave`
  (params (PlayerState :type "FSDPlayerState Object Reference")))

(event `Loaded`)

(event `self.DonkeyButtonPressed`
  (`parent.DonkeyButtonPressed`))

(event `self.LoadSpaceRig`
  (`parent.LoadSpaceRig`))

(fn `ChoosePlayerStart`
  (params (Player :type "Controller Object Reference"))
  (returns (ReturnValue :type "Actor Object Reference"))
  (bind _returnvalue (`parent.ChoosePlayerStart` Player))
  (return _returnvalue))

(fn `DestroyNetworkedActors`)

(fn `EnableMuleButton`)

(fn `GetDefaultPawnClassForController`
  (params (InController :type "Controller Object Reference"))
  (returns (ReturnValue :type "Object Class Reference"))
  (bind _returnvalue (`parent.GetDefaultPawnClassForController` InController))
  (return _returnvalue))

(fn `GetEditorCharacterClass`
  (returns (`Character Class` :type "PlayerCharacterID Object Reference"))
  (return null))

(fn `GetEscapepodLocation`
  (returns (Location :type "Transform Structure"))
  (return))

(fn `LoadToMission`
  (params (Mission :type "MissionTemplate Object Reference")))

(fn `PreloadMuleClass`)

(fn `TryPreloadCheatMenu`)

(fn `UserConstructionScript`)