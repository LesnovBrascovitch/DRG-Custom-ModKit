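; GM_Salvage is the game mode Blueprint for a salvage mission, outlining repair points, a defend phase, countdowns and drop pod extraction.
; Level generation, objective setup, drop pod calls and donkey button presses forward to the parent class.
; All other events, plus the functions for spawning and enabling repair points and updating failsafe Molly counters, are empty stubs, so this file holds only the mission's interface.
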(event `self.OnLevelGenerationComplete`
  (params (pass :type Integer))
  (`parent.OnLevelGenerationComplete` pass))

(event `/Game/Game/BP_GameMode.Call DropPod`
  (`parent.Call DropPod`))

(event `self.DonkeyButtonPressed`
  (`parent.DonkeyButtonPressed`))

(event `ReachedDropShip`)

(event `RepairPoint_Repaired`
  (params (RepairPoint :type "Actor Object Reference")))

(event `DefendFail`)

(event `DefendDone`)

(event `OnCountdownFinished`)

(event `Countdowncomplete`)

(event `ActivateDonkeyButton`)

(event `OnMuleBayOpenedDispatch_Event_0`)

(event `self.OnObjectivesInitialized`
  (`parent.OnObjectivesInitialized`))

(event `AllActorsSalaged`)

(event `Cheat_ActivateDropPod`)

(event `Cheat_FinishSalvagePoint`)

(fn `EnableNextRepairPoint`)

(fn `SpawnRepairPoints`)

(fn `UpdateFailsafeMollyCounters`
  (params (V2 :type "Vector Structure")))

(fn `UserConstructionScript`
  (`parent.UserConstructionScript`))