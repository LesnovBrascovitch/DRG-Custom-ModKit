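; Player state Blueprint for the Space Rig, declaring an interface for watching, replicating and querying per-player mission stats, plus campaign and health insurance checks.
; Names point to a server update event and a RepNotify for syncing stats.
; All stat functions and events are empty or return defaults, BeginPlay only calls its parent, and Tick is disabled.
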(event `self.ReceiveBeginPlay`
  (`parent.ReceiveBeginPlay`))

(event `WatchStat`
  (params (MissionStat :type "MissionStat Object Reference")))

(event `CheckCampaign`)

(event `OnMissionStatChanged`
  (params (WorldContext :type "Object Object Reference") (MissionStat :type "MissionStat Object Reference") (Value :type "Float (double-precision)")))

(event `Server_UpdateStat`
  (params (`Mission Stat` :type "MissionStat Object Reference") (`Stat Value` :type "Float (double-precision)")))

(fn `GetHealthInsuranceStatus`
  (returns (HealthInsuranceStatus :type Integer))
  (return 0))

(fn `GetMissionStatValue`
  (params (MissionStat :type "MissionStat Object Reference"))
  (returns (StatValue :type Text) (Valid :type Boolean))
  (return "" false))

(fn `IsListeningToMissionStat`
  (params (MissionStat :type "MissionStat Object Reference"))
  (returns (HasStat :type Boolean))
  (return false))

(fn `OnRep_MissionStats`)

(fn `SendMissionStatData`
  (params (MissionStat :type "MissionStat Object Reference") (Value :type "Float (double-precision)")))

(fn `UpdateMissionStat`
  (params (MissionStat :type "MissionStat Object Reference") (Value :type "Float (double-precision)")))

(fn `UserConstructionScript`
  (`parent.UserConstructionScript`))