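; Base Blueprint player controller for the Space Rig, declaring UI-related hooks for character selection, the forge workshop, mission select and crafting.
; ShowCharacterSelectionBackground and ShowForgeWorkshop are empty events, and the three getters for mission select, popup crafting and crafting return nothing.
; It holds no logic of its own: BeginPlay and Tick are disabled, and the construction script only calls its parent.
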(event `ShowCharacterSelectionBackground`
  (params (resetToDefaultWeapon :type Boolean) (cameraLocation :type "ECharselectionCameraLocation Enum" :default "Selection")))

(event `ShowForgeWorkshop`)

(fn `GetCrafting`
  (returns (Widget :type "WindowWidget Object Reference"))
  (return null))

(fn `GetMissionSelect`
  (returns (Widget :type "WindowWidget Object Reference"))
  (return null))

(fn `GetPopupCrafting`
  (returns (Widget :type "WindowWidget Object Reference"))
  (return null))

(fn `UserConstructionScript`
  (`parent.UserConstructionScript`))