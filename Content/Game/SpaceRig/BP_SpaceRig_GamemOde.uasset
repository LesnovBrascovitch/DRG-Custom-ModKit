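; BP_SpaceRig_GamemOde is the game mode Blueprint for the Space Rig, laid out as a skeleton with almost no logic of its own.
; BeginPlay, logout, player restart, restart check, player start and default pawn overrides only forward to the parent class.
; Countdown, instant mission start, privilege check, success/failure callbacks, mission analytics and random class selection are empty stubs, and GetGameState returns no value.
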(event `self.ReceiveBeginPlay`
  (`parent.ReceiveBeginPlay`))

(event `OnFailure_1E75EB674DDE2C1E6C7EC18D18AFDB55`)

(event `OnSuccess_1E75EB674DDE2C1E6C7EC18D18AFDB55`)

(event `OnFailure_509E599D4BB91C15BA2979B190501E9F`)

(event `OnSuccess_509E599D4BB91C15BA2979B190501E9F`)

(event `OnCountdownComplete`)

(event `self.K2_OnLogout`
  (params (ExitingController :type "Controller Object Reference"))
  (`parent.K2_OnLogout` ExitingController))

(event `self.K2_OnRestartPlayer`
  (params (NewPlayer :type "Controller Object Reference"))
  (`parent.K2_OnRestartPlayer` NewPlayer))

(event `ControllerReady`
  (params (Target :type "FSDPlayerController Object Reference")))

(event `InstantlyStartMission`)

(event `On online privilige checked`
  (params (CheckedPlayerState :type "PlayerState Object Reference") (CheckedPrivilege :type "EBlueprintableUserPrivileges Enum" :default "CanPlay") (PrivilegeResult :type "EBlueprintablePrivilegeResults Enum" :default "NoFailures")))

(fn `ChoosePlayerStart`
  (params (Player :type "Controller Object Reference"))
  (returns (ReturnValue :type "Actor Object Reference"))
  (bind _returnvalue (`parent.ChoosePlayerStart` Player))
  (return _returnvalue))

(fn `GetDefaultPawnClassForController`
  (params (InController :type "Controller Object Reference"))
  (returns (ReturnValue :type "Object Class Reference"))
  (bind _returnvalue (`parent.GetDefaultPawnClassForController` InController))
  (return _returnvalue))

(fn `GetGameState`
  (return))

(fn `PlayerCanRestart`
  (params (Player :type "PlayerController Object Reference"))
  (returns (ReturnValue :type Boolean))
  (bind _returnvalue (`parent.PlayerCanRestart` Player))
  (return _returnvalue))

(fn `SelectRandomAvailableClass`
  (params (Player :type "FSDPlayerState Object Reference")))

(fn `SendMissionStartAnalytics`)

(fn `UserConstructionScript`)