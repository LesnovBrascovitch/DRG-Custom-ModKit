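; Player controller Blueprint for the Space Rig hub, declaring the interface for its menus, consoles, character selection, bar rounds, tutorial launch and rig reloads.
; Nearly every event and function is an empty stub, including UI creation, asset preloading and savegame checks.
; A handful of lifecycle events, window openers and widget getters only forward to the parent class.
; HUDVisible always returns false, and Tick is disabled.
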(event `self.ReceiveBeginPlay`
  (`parent.ReceiveBeginPlay`))

(event `OnLoaded_0C1A95084D16C934A469CF8C3B445101`
  (params (Loaded :type "Object Class Reference")))

(event `OnFailure_84F86EB44BDC03B3D4D52D92FC0B069A`)

(event `OnSuccess_84F86EB44BDC03B3D4D52D92FC0B069A`)

(event `OnFailure_FD5D0BC24D561288D20ABE9353DBA180`)

(event `OnSuccess_FD5D0BC24D561288D20ABE9353DBA180`)

(event `ShowServerBrowser`)

(event `ShowMissionSelect`)

(event `Client_OpenMap`)

(event `PlayerChangeCharacter`
  (params (NewCharacter :type "PlayerCharacterID Object Reference")))

(event `self.RecievePreClientTravel`
  (`parent.RecievePreClientTravel`))

(event `ShowCharacterSelect`)

(event `ControllerReady`)

(event `self.RecieveOnControllerReady`
  (`parent.RecieveOnControllerReady`))

(event `ShowBuyItemPopup`
  (params (Item :type "Actor Class Reference") (Upgrade :type "ItemUpgrade Object Reference")))

(event `self.ReceiveDestroyed`
  (`parent.ReceiveDestroyed`))

(event `OnCharacterPossesd`
  (params (pawn :type "Pawn Object Reference")))

(event `ShowCharCustomization`)

(event `ShowCrafting`)

(event `ShowCharacterScreenAndWorld`)

(event `ShowCraftingAndWorld`)

(event `ShowCustomizationAndWorld`)

(event `SpawnPlayer`)

(event `ShowFirstCharacterSelect`)

(event `OpenCharacterSelector`
  (params (OpenVideo :type Boolean) (AllowBack :type Boolean)))

(event `ShowReconnectController`)

(event `OnFirstWindowOpened`)

(event `OnLastWindowClosed`)

(event `ShowNetworkError`)

(event `ShowTrading`)

(event `ShowWindowByClass`
  (params (windowClass :type "WindowWidget Class Reference") (zOrder :type Integer)))

(event `ShowCheatMenu`)

(event `ShowBarMenu`
  (params (Bar :type "SpaceRigBar Object Reference")))

(event `OnRoundSelected_Event`
  (params (Bar :type "SpaceRigBar Object Reference") (RequestedDrink :type "DrinkableDataAsset Object Reference")))

(event `OrderBarRound`
  (params (Bar :type "SpaceRigBar Object Reference") (Drink :type "DrinkableDataAsset Object Reference")))

(event `Deduct Credits On Client`
  (params (Amount :type Integer)))

(event `ShowJobs`)

(event `ShowItemUpgradeScreen`
  (params (CharacterClass :type "PlayerCharacter Class Reference") (ItemClass :type "Actor Class Reference") (ItemCategory :type "EItemCategory Enum" :default "PrimaryWeapon")))

(event `ShowBoscoUpgrades`)

(event `self.OnPlayerSpawnBegin`
  (params (PlayerId :type Integer))
  (`parent.OnPlayerSpawnBegin` PlayerId))

(event `OnDroppodLeave`)

(event `PlayerThrewMugInHoop`)

(event `PlayerPlayedEntireSong`)

(event `HandleDiscordConsole`
  (params (DiscordConsole :type "/Game/UI/HUD_SpaceRig/CommunityTerminal/BP_DiscordConsole Object Reference")))

(event `SetUsableDiscord`
  (params (Usable :type Boolean)))

(event `ShowDeepDives`)

(event `OpenSpacerigConsole`
  (params (Console :type "/Game/UI/HUD_SpaceRig/BP_BaseSpaceRigConsole Object Reference")))

(event `/Game/Game/BP_PlayerControllerBase.SetHasShownCharacterSelector`
  (params (HasShown :type Boolean))
  (`parent.SetHasShownCharacterSelector` HasShown))

(event `/Game/Game/BP_PlayerControllerBase.SetIsEscapeMenuEnabled`
  (params (IsEscapeMenuEnabled :type Boolean))
  (`parent.SetIsEscapeMenuEnabled` IsEscapeMenuEnabled))

(event `/Game/Game/BP_PlayerControllerBase.Reset Player Location`
  (`parent.Reset Player Location`))

(event `Reset Player Scale On Clients`)

(event `Server_PopLooatAtAffliction`)

(event `ShowLookAtConsole`)

(event `LaunchTutorial`)

(event `PromptLaunchTutorial`)

(event `On Prompt`
  (params (Yes :type Boolean)))

(event `self.ShowCharacterSelectionBackground`
  (params (resetToDefaultWeapon :type Boolean) (cameraLocation :type "ECharselectionCameraLocation Enum" :default "Selection"))
  (`parent.ShowCharacterSelectionBackground` resetToDefaultWeapon cameraLocation))

(event `self.ShowForgeWorkshop`
  (`parent.ShowForgeWorkshop`))

(event `ReloadSpacerig`)

(event `OnRestartGame`
  (params (Yes :type Boolean) (CreateModdedSave :type Boolean)))

(event `OnRestartSpacerig`
  (params (Yes :type Boolean) (CreateModdedSave :type Boolean)))

(event `OnPackageMounted`
  (params (Sandbox :type Boolean)))

(event `OnPlayer`
  (params (PlayerState :type "FSDPlayerState Object Reference")))

(event `self.ShowEscapeMenu`
  (`parent.ShowEscapeMenu`))

(event `self.OpenStandaloneMinersManual`
  (params (Section :type "EMinersManualSection Enum" :default "FrontPage") (ID :type "Guid Structure (by ref)"))
  (`parent.OpenStandaloneMinersManual` Section ID))

(event `self.OpenStandaloneMinersManualPage`
  (params (page :type "EMinersManualSinglePage Enum" :default "Mutators"))
  (`parent.OpenStandaloneMinersManualPage` page))

(event `Back_Event_0`)

(event `OnCharacterSelected`)

(event `OnHostTimerChanged`
  (params (NewTime :type "Float (double-precision)")))

(event `OnMissionTimerChanged`
  (params (NewTime :type "Float (double-precision)")))

(event `DoCountDown`
  (params (NewTime :type "Float (double-precision)")))

(event `ShowReconnect`
  (params (Show :type Boolean)))

(event `OnGravityChanged`
  (params (CurrentGravity :type "Float (double-precision)") (Change :type "Float (double-precision)")))

(event `CustomEvent_0`)

(fn `AddWidget`
  (params (Widget :type "UserWidget Object Reference (by ref)") (ZOrder :type Integer) (InVisibility :type "ESlateVisibility Enum" :default "Visible")))

(fn `Change Savegame`)

(fn `ChangeCharacter`
  (params (newCharacter :type "PlayerCharacterID Object Reference")))

(fn `ChangeHUDVisible`
  (params (IsHUDVisible :type Boolean) (reason :type "EHUDVisibilityReason Enum" :default "Invalid")))

(fn `CreateUI`)

(fn `GetCrafting`
  (returns (Widget :type "WindowWidget Object Reference"))
  (return (`parent.GetCrafting`)))

(fn `GetEscapeMenu`
  (returns (ReturnValue :type "EscapeMenuWindow Object Reference"))
  (return (`parent.GetEscapeMenu`)))

(fn `GetMissionSelect`
  (returns (Widget :type "WindowWidget Object Reference"))
  (return (`parent.GetMissionSelect`)))

(fn `GetPopupCrafting`
  (returns (Widget :type "WindowWidget Object Reference"))
  (return (`parent.GetPopupCrafting`)))

(fn `HUDVisible`
  (returns (ReturnValue :type Boolean))
  (return false))

(fn `ModdedSavegameCheck`)

(fn `PreloadAssets`)

(fn `ResetCheats`)

(fn `SelectLastPlayedCharacter`)

(fn `UserConstructionScript`
  (`parent.UserConstructionScript`))