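; BP_PlayerController is a player controller Blueprint with hooks for hero selection, loading screens, level restart and end-of-level flow.
; BeginPlay, generation-done and the end-level events only forward to parent implementations, and Tick is disabled.
; Hero selection, screen, server and async-load events are empty, as are the tutorial and character-destruction functions.
; The HUD visibility and end-screen skip checks always return false.
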(event `self.ReceiveBeginPlay`
  (`parent.ReceiveBeginPlay`))

(event `OnLoaded_0556572242FB261AF5947C9A16CF353A`
  (params (Loaded :type "Object Object Reference")))

(event `SelectNewHero`
  (params (Hero :type "PlayerCharacterID Object Reference")))

(event `self.OnGenerationDone`
  (`parent.OnGenerationDone`))

(event `Server_RestartLevel`)

(event `self.ReceiveEndLevel`
  (`parent.ReceiveEndLevel`))

(event `Server_ClientReady`)

(event `SelectLateJoinCharacter`
  (params (Hero :type "PlayerCharacterID Object Reference")))

(event `RequestLoadScreen`)

(event `ShowSelectCharacterScreen`)

(event `ShowLoadingScrren`)

(event `self.Receive_EndLevel_WaitForData`
  (params (areObjectivesCompleted :type Boolean) (numberOfPlayersInPod :type Integer))
  (`parent.Receive_EndLevel_WaitForData` areObjectivesCompleted numberOfPlayersInPod))

(event `Server_SetLag`)

(fn `DestroyCharacter`)

(fn `IsHUDVisible`
  (returns (Visible :type Boolean))
  (return false))

(fn `ShouldSkipEndscreen`
  (returns (ReturnValue :type Boolean))
  (return false))

(fn `UpdateTutorialComplete`)

(fn `UserConstructionScript`
  (`parent.UserConstructionScript`))