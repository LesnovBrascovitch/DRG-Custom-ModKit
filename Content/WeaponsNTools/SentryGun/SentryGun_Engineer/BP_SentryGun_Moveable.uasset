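; Moveable Engineer sentry gun Blueprint, with hooks for move requests, movement, readiness and state changes.
; Core events and most getters only forward to the parent implementation.
; Audio, outline/icon, ammo, nameplate and item-selection handlers are empty stubs, as is SpawnAudioOnPlayer.
; GetSentryOwner returns no wired value, so any working behavior comes from the parent class.
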(event `self.ReceiveBeginPlay`
  (`parent.ReceiveBeginPlay`))

(event `self.OnMoveRequested`
  (`parent.OnMoveRequested`))

(event `OnStateChanged_Event`
  (params (Sender :type "RedeployableSentryGun Object Reference") (NewState :type "ERedeployableSentryGunState Enum" :default "Deploying")))

(event `self.ReceiveOnSentryReady`
  (params (SentryGun :type "SentryGun Object Reference") (PlayerCharacter :type "PlayerCharacter Object Reference"))
  (`parent.ReceiveOnSentryReady` SentryGun PlayerCharacter))

(event `OnAmmoCountChanged_Event_0`
  (params (ammoCount :type Integer) (change :type Integer)))

(event `AudioReadyToBuild`)

(event `self.OnMoving`
  (`parent.OnMoving`))

(event `self.OnMoveFinished`
  (params (returnedHome :type Boolean))
  (`parent.OnMoveFinished` returnedHome))

(event `AudioBeginMove`)

(event `AudioMoveFinished`)

(event `AudioReturnedHome`)

(event `self.ReceiveOnStateChanged`
  (`parent.ReceiveOnStateChanged`))

(event `Update Outline And Icon`)

(event `OnSentryStateChanged`
  (params (Sender :type "RedeployableSentryGun Object Reference") (NewState :type "ERedeployableSentryGunState Enum" :default "Deploying")))

(event `OnToggleNameplatesEvent_Event_0`
  (params (boolValue :type Boolean)))

(event `OnItemEquipped_Event`
  (params (Item :type "Item Object Reference")))

(event `OnSelectedItemChanged`
  (params (SentryGun :type "RecallableSentryGun Object Reference")))

(fn `GetSentryGun`
  (returns (ReturnValue :type "SentryGun Object Reference"))
  (return (`parent.GetSentryGun`)))

(fn `GetSentryGunClass`
  (returns (ReturnValue :type "SentryGun Class Reference"))
  (return (`parent.GetSentryGunClass`)))

(fn `GetSentryOwner`
  (returns (`AsPlayer Character` :type "PlayerCharacter Object Reference"))
  (return null))

(fn `GetStateDescription`
  (returns (Description :type Text))
  (return (`parent.GetStateDescription`)))

(fn `SpawnAudioOnPlayer`
  (params (Audio :type "SoundBase Object Reference")))

(fn `UserConstructionScript`)