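; Redeployable variant of the Engineer's sentry gun, with deploy, dismantle, ammo and special attack hooks.
; Deploy and dismantle events, owner and ammo changes, special attack activation and deploy progress pass straight through to the parent class.
; Special attack GFX and reset, indicator light, shadow, build mode and timeline handlers are empty, so the Blueprint adds no logic of its own.
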(event `self.ReceiveBeginPlay`
  (`parent.ReceiveBeginPlay`))

(event `Timeline_0__FinishedFunc`)

(event `Timeline_0__UpdateFunc`)

(event `self.ReceiveOnDeploy`
  (`parent.ReceiveOnDeploy`))

(event `self.ReceiveOnDismantle`
  (`parent.ReceiveOnDismantle`))

(event `self.ReceiveOnDismantled`
  (`parent.ReceiveOnDismantled`))

(event `self.ReceiveOnDeployed`
  (`parent.ReceiveOnDeployed`))

(event `self.ReceiveOnSentryGunOwnerChanged`
  (`parent.ReceiveOnSentryGunOwnerChanged`))

(event `self.ActivateSpecialAttack`
  (`parent.ActivateSpecialAttack`))

(event `Multicast Special Attack GFX`)

(event `Reset Special Attack`)

(event `UpdateShadows`)

(event `self.ReceiveAmmoChanged`
  (params (Delta :type Integer) (currentAmount :type Integer))
  (`parent.ReceiveAmmoChanged` Delta currentAmount))

(fn `ConditionallyEnableShadows`)

(fn `GetDeployProgress`
  (returns (ReturnValue :type "Float (double-precision)"))
  (return (`parent.GetDeployProgress`)))

(fn `ToggleBuildMode`
  (params (InBuilding :type Boolean)))

(fn `UpdateIndicatorLight`
  (params (FiredShot :type Boolean)))

(fn `UserConstructionScript`)