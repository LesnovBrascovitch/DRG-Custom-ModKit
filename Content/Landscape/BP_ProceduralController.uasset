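; BP_ProceduralController is a procedural landscape controller that handles requests and transfers of room, obstacle, tunnel, PLS and carver data.
; Its send, receive and request events only forward to the parent class, passing along seed, rooms, obstacles, tunnels and carver pass.
; The Server_RequestPLSData and Server_RequestCarverData events have empty bodies here, and BeginPlay and Tick are disabled, so the Blueprint adds no logic of its own.
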(event `self.SendRoomData`
  (`parent.SendRoomData`))

(event `self.SendTunnelData`
  (`parent.SendTunnelData`))

(event `self.ReceivedRoomData`
  (params (Seed :type Integer) (Rooms :type "Array of RoomNode Structure (by ref)") (Obstacles :type "Array of PathObstacle Structure (by ref)"))
  (`parent.ReceivedRoomData` Seed Rooms Obstacles))

(event `self.ReceivedTunnelData`
  (params (tunnels :type "Array of TunnelNode Structure (by ref)"))
  (`parent.ReceivedTunnelData` tunnels))

(event `Server_RequestPLSData`)

(event `Server_RequestCarverData`
  (params (Pass :type "EDebrisItemPass Enum" :default "PrePlacement")))

(event `self.RequestPLSData`
  (`parent.RequestPLSData`))

(event `self.RequestCarverData`
  (params (pass :type "EDebrisItemPass Enum" :default "PrePlacement"))
  (`parent.RequestCarverData` pass))