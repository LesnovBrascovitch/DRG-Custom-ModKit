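; Snowstorm effect Blueprint for the Ice Caves biome, with start and end events.
; StartEffect and EndEffect only forward to the parent class, and the construction script does the same.
; Fadein and Fadeout timeline events are present but empty, so the graphs here add no behavior of their own.
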(event `Fadein__FinishedFunc`)

(event `Fadein__UpdateFunc`)

(event `Fadeout__FinishedFunc`)

(event `Fadeout__UpdateFunc`)

(event `self.StartEffect`
  (`parent.StartEffect`))

(event `self.EndEffect`
  (`parent.EndEffect`))

(fn `UserConstructionScript`
  (`parent.UserConstructionScript`))