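; Actor for a modded aim-down-sights system that swaps the local player's first-person weapon animations while ADS is held.
; Equipping an ammo-driven weapon that returns valid ADS settings enables it and caches those settings.
; Press and release play start/end montages, gated on little reload time remaining, then swap fire, idle, walk and jump animations.
; Reloading or unequipping restores the default animation set, and possession changes rebind to the new character.
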(event `InputAction|ADS`
  (params (Key :type "Key Structure"))
  (:`Pressed`
    (if (`self.Is ADSable`)
      (`self.NewMacro_0`
        (:`then`
          (set `PlayerCharacter.IsRunning` false (`self.Player Character`))
          (`|PlayMontage` (`PlayerCharacter.FPMesh` (`self.Player Character`)) (`/Game/_DRGModding/_SPGameplayExtender/_CustomWeaponSystem/_Framework/ADSSystem/ADSSettings.GetADSStart` (`self.ADSSettings`))
            (:`OnBlendOut`
              (`self.ChangeAnimsToADS`)))))))
  (:`Released`
    (if (`self.Is ADSable`)
      (`self.NewMacro_0`
        (:`then`
          (`|PlayMontage` (`PlayerCharacter.FPMesh` (`self.Player Character`)) (`/Game/_DRGModding/_SPGameplayExtender/_CustomWeaponSystem/_Framework/ADSSystem/ADSSettings.GetADSEnd` (`self.ADSSettings`))
            (:`then`
              (set `AmmoDrivenWeapon.FP_FireAnimation` (`/Game/_DRGModding/_SPGameplayExtender/_CustomWeaponSystem/_Framework/ADSSystem/ADSSettings.GetDefaultFire` (`self.ADSSettings`)) (`self.As Ammo Driven Weapon`)))
            (:`OnBlendOut`
              (`self.ResetAnimToDefault` true null (`self.ADSSettings`)))))
        (:`false`
          (`self.ResetAnimToDefault` false (`self.As Ammo Driven Weapon`) (`self.ADSSettings`)))))))

(event `OnItemEquipped`
  (params (Item :type "Item Object Reference"))
  ;[1 1 1] OnItemEquipped - Get if the equipped weapon is bashable or not. If true, do bash related logics.
  (bind _adssettings (message `/Game/_DRGModding/_Frameworks/Interface/BPI_CustomWeaponHandling.GetADS` Item))
  (`/Engine/EditorBlueprintResources/StandardMacros.IsValid` _adssettings
    (:`Is Valid`
      (bind _asammo_driven_weapon (cast `AmmoDrivenWeapon` Item))
      (bind _output_get (set `self.As Ammo Driven Weapon` _asammo_driven_weapon))
      (add `AmmoDrivenWeapon.OnReloadingEvent` _output_get (delegate `OnReloadingEvent_Event_0`))
      (set `self.ADSSettings` _adssettings)
      (set `self.Is ADSable` true))
    (:`Is Not Valid`
      (set `self.Is ADSable` false))))

(event `OnReloadingEvent_Event_0`
  ;[1 1 1] OnItemEquipped - Get if the equipped weapon is bashable or not. If true, do bash related logics.
  (`self.ResetAnimToDefault` false (`self.As Ammo Driven Weapon`) (`self.ADSSettings`)))

(event `self.ReceiveBeginPlay`
  (bind _fsdplayercontroller (`/Game/_DRGModding/_Frameworks/BML_Framework.GetLocalPlayerController(Macro)` true)
    (:`Completed`
      (set `self.FSDPlayer Controller` _fsdplayercontroller)
      (add `FSDPlayerController.OnPlayerCharacterPossesed` (`self.FSDPlayer Controller`) (delegate `OnPlayerCharacterPossesed_Event_0`))
      (bind _playercharacter (`/Game/_DRGModding/_Frameworks/BML_Framework.GetLocalPlayerCharacter(Macro)` true :!label _label)
        (:`Exec`
          (bind _output_get (set `self.Player Character` _playercharacter))
          (bind _inventorycomponent (`PlayerCharacter.InventoryComponent` _output_get))
          (add `InventoryComponent.OnItemEquipped` _inventorycomponent (delegate `OnItemEquipped`))
          (add `InventoryComponent.OnItemUnequipped` _inventorycomponent (delegate `OnItemUnequipped_Event_0`))
          (set `self.AnimInstance` (`PlayerCharacter.GetFPAnimInstance` (`self.Player Character`)))
          (`/Engine/EditorBlueprintResources/StandardMacros.DoOnce` false
            (:`Completed`
              (`self.EnableInput` (`self.FSDPlayer Controller`)))))))))

(event `OnPlayerCharacterPossesed_Event_0`
  (params (Pawn :type "Pawn Object Reference"))
  (goto _label))

(event `OnItemUnequipped_Event_0`
  (params (Item :type "Item Object Reference"))
  (set `AmmoDrivenWeapon.ReloadTimeLeft` 0.0 (`self.As Ammo Driven Weapon`))
  (bind _adssettings (message `/Game/_DRGModding/_Frameworks/Interface/BPI_CustomWeaponHandling.GetADS` Item))
  (`/Engine/EditorBlueprintResources/StandardMacros.IsValid` _adssettings
    (:`Is Valid`
      (bind _asammo_driven_weapon (cast `AmmoDrivenWeapon` Item))
      (`self.ResetAnimToDefault` false _asammo_driven_weapon _adssettings)
      (remove `AmmoDrivenWeapon.OnReloadingEvent` _asammo_driven_weapon (delegate `OnReloadingEvent_Event_0`)))))

(event `CustomEvent_0`
  (bind _as_ammo_driven_weapon (`self.As Ammo Driven Weapon`))
  (`/Engine/EditorBlueprintResources/StandardMacros.IsValid` _as_ammo_driven_weapon
    (:`Is Valid`
      (`/Game/_DRGModding/_Frameworks/BML_Framework.PrintViaChat` false (`KismetStringLibrary.Conv_DoubleToString` (`AmmoDrivenWeapon.ReloadTimeLeft` _as_ammo_driven_weapon))))))

(fn `ChangeAnimsToADS`
  (bind _animinstance (`self.AnimInstance`))
  (bind _adssettings (`self.ADSSettings`))
  (bind (_adsanimset_adsstart _adsanimset_adsend _adsanimset_adsfire _adsanimset_adsidle _adsanimset_adswalk _adsanimset_adsjumpstart _adsanimset_adsjumploop _adsanimset_adsjumpland _adsanimset_adsjumplandwithaim) (break `/Game/_DRGModding/_SPGameplayExtender/_CustomWeaponSystem/_Framework/ADSSystem/S_ADSAnimSet` (`/Game/_DRGModding/_SPGameplayExtender/_CustomWeaponSystem/_Framework/ADSSystem/ADSSettings.ADSAnimSet` _adssettings)))
  (`/Engine/EditorBlueprintResources/StandardMacros.IsValid` _adssettings
    (:`Is Valid`
      (set `AmmoDrivenWeapon.FP_FireAnimation` _adsanimset_adsfire (`self.As Ammo Driven Weapon`))
      (set `PlayerFPAnimInstance.FP_Idle` _adsanimset_adsidle _animinstance)
      (set `PlayerFPAnimInstance.FP_Walk` _adsanimset_adswalk _animinstance)
      (set `PlayerFPAnimInstance.FP_JumpStart` _adsanimset_adsjumpstart _animinstance)
      (set `PlayerFPAnimInstance.FP_JumpLoop` _adsanimset_adsjumploop _animinstance)
      (set `PlayerFPAnimInstance.FP_JumpLand` _adsanimset_adsjumpland _animinstance)
      (set `PlayerFPAnimInstance.FP_JumpLand_Aim` _adsanimset_adsjumplandwithaim _animinstance))))

(fn `ResetAnimToDefault`
  (params (IgnoreFireAnim :type Boolean) (Target :type "AmmoDrivenWeapon Object Reference") (ADSSettings :type "/Game/_DRGModding/_SPGameplayExtender/_CustomWeaponSystem/_Framework/ADSSystem/ADSSettings Object Reference"))
  (bind (_defaultanimset_defaultfire _defaultanimset_defaultidle _defaultanimset_defaultwalk _defaultanimset_defaultjumpstart _defaultanimset_defaultjumploop _defaultanimset_defaultjumpland _defaultanimset_defaultjumplandwithaim) (break `/Game/_DRGModding/_SPGameplayExtender/_CustomWeaponSystem/_Framework/ADSSystem/S_DefaultAnimSet` (`/Game/_DRGModding/_SPGameplayExtender/_CustomWeaponSystem/_Framework/ADSSystem/ADSSettings.DefaultAnimSet` ADSSettings)))
  (bind _animinstance (`self.AnimInstance`))
  (if (not IgnoreFireAnim)
    (set `AmmoDrivenWeapon.FP_FireAnimation` _defaultanimset_defaultfire Target))
  (set `PlayerFPAnimInstance.FP_Idle` _defaultanimset_defaultidle _animinstance)
  (set `PlayerFPAnimInstance.FP_Walk` _defaultanimset_defaultwalk _animinstance)
  (set `PlayerFPAnimInstance.FP_JumpStart` _defaultanimset_defaultjumpstart _animinstance)
  (set `PlayerFPAnimInstance.FP_JumpLoop` _defaultanimset_defaultjumploop _animinstance)
  (set `PlayerFPAnimInstance.FP_JumpLand` _defaultanimset_defaultjumpland _animinstance)
  (set `PlayerFPAnimInstance.FP_JumpLand_Aim` _defaultanimset_defaultjumplandwithaim _animinstance))

(fn `UserConstructionScript`)