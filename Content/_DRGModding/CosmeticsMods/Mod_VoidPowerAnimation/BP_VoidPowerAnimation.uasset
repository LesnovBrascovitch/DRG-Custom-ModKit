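; Cosmetic mod actor that turns the local player's first-person charge blaster into bare-hand magic casting with a skull ring.
; On possession it binds inventory events; equipping hides the weapon mesh, swaps animations and attaches the ring to the hand.
; Charge and heat drive the ring's dynamic materials, while camera mode toggles its visibility.
; Montage starts trigger a timed overheat particle burst or a replacement gunsling whose notifies spawn and explode hand effects.
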(event `OnCameraModeChanged_Event_0`
  (params (NewCameraMode :type "ECharacterCameraMode Enum" :default "FirstPerson") (OldCameraMode :type "ECharacterCameraMode Enum" :default "FirstPerson"))
  ;[1 1 1] Hide the skull ring based on the camera mode.
  (switch `ECharacterCameraMode` NewCameraMode
    (:`FirstPerson`
      (`SceneComponent.SetVisibility` (`self.SkullRingRoot`) true true :!label _label))
    (:`ThirdPerson`
      (`SceneComponent.SetVisibility` (`self.SkullRingRoot`) false true :!label _label_2))
    (:`Follow`
      (goto _label_2))
    (:`DownCamera`
      (goto _label_2))
    (:`TerrainScanner`
      (goto _label))
    (:`PhotographyMode`
      (goto _label_2))
    (:`FirstPersonHeadOnly`
      (goto _label))))

(event `OnPlayerCharacterPossesed_Event_0`
  (set `self.IsInitialized` false)
  (bind _playercharacter (`/Game/_DRGModding/_Frameworks/BML_Framework.GetLocalPlayerCharacter(Macro)` true :!label _label_3)
    (:`Exec`
      (bind _output_get (set `self.Player Character` _playercharacter))
      (bind _inventorycomponent (`PlayerCharacter.InventoryComponent` _output_get))
      (add `InventoryComponent.OnItemEquipped` _inventorycomponent (`|CreateDelegate` :!event `OnItemEquipped(Dummy)`))
      (add `InventoryComponent.OnItemUnequipped` _inventorycomponent (`|CreateDelegate` :!event `OnItemUnequipped(Dummy)`))
      (add `PlayerCharacter.OnCameraModeChanged` (`self.Player Character`) (delegate `OnCameraModeChanged_Event_0`))
      (`self.AddEffects` (`self.Player Character`))
      (set `self.IsInitialized` true))))

(event `self.ReceiveBeginPlay`
  (bind _returnvalue (`KismetMaterialLibrary.CreateDynamicMaterialInstance` "/Game/WeaponsNTools/ChargeBlaster/Materials/M_WPN_ChargeBlaster_A_Light.M_WPN_ChargeBlaster_A_Light"))
  (bind _output_get (set `self.DMI(SkullEyes)` _returnvalue))
  (`PrimitiveComponent.SetMaterial` (`self.SkullRingEye_L`) 0 _output_get)
  (`PrimitiveComponent.SetMaterial` (`self.SkullRingEye_R`) 0 _output_get)
  (bind _returnvalue_2 (`KismetMaterialLibrary.CreateDynamicMaterialInstance` "/Game/_DRGModding/CosmeticsMods/Mod_VoidPowerAnimation/M_VoidPower_Overheat.M_VoidPower_Overheat"))
  (bind _output_get_2 (set `self.DMI(Skull)` _returnvalue_2))
  (`PrimitiveComponent.SetMaterial` (`self.SkullRingHeat`) 0 _output_get_2)
  (`|LoadAsset` "/Game/WeaponsNTools/ChargeBlaster/WPN_ChargeBlaster.WPN_ChargeBlaster" ; Make sure WPN_ChargeBlaster is loaded.
    (:`Completed`
      (bind _fsdplayercontroller (`/Game/_DRGModding/_Frameworks/BML_Framework.GetLocalPlayerController(Macro)` true)
        (:`Completed`
          (set `self.FSDPlayer Controller` _fsdplayercontroller)
          (add `FSDPlayerController.OnPlayerCharacterPossesed` (`self.FSDPlayer Controller`) (delegate `OnPlayerCharacterPossesed_Event_0`))
          (goto _label_3))))))

(event `/Game/_DRGModding/_Tools/DummyPlayerCharacter/BPI_DummyEvents.OnItemEquipped(Dummy)`
  (params (Item :type "Item Object Reference"))
  (bind _scene (`self.Scene`))
  (bind _skullringroot (`self.SkullRingRoot`))
  (bind _as_wpn_charge_blaster (`self.As WPN Charge Blaster`))
  (bind _as_wpn_charge_blaster_2 (`self.As WPN Charge Blaster`))
  ;[1 1 1] On Item Equipped - Change animations, bind events.
  (if (`self.IsInitialized`)
    (`/Game/_DRGModding/_Frameworks/BML_Framework.CompareClass(Item)` Item "/Game/WeaponsNTools/ChargeBlaster/WPN_ChargeBlaster.WPN_ChargeBlaster_C"
      (:`Class Match`
        (add `AnimInstance.OnMontageStarted` (`SkeletalMeshComponent.GetAnimInstance` (`PlayerCharacter.FPMesh` (`self.Player Character`))) (`|CreateDelegate` :!event `OnMontageStarted_Event_0`))
        (`SceneComponent.SetVisibility` (`self.SkullRingRoot`) true true)
        (set `self.As WPN Charge Blaster` (cast `/Game/WeaponsNTools/ChargeBlaster/WPN_ChargeBlaster` Item :!pure true))
        (`/Game/_DRGModding/_Frameworks/BML_Framework.UpdateAnims(AnimatedItem)` _as_wpn_charge_blaster "/Game/_DRGModding/CosmeticsMods/Mod_VoidPowerAnimation/IAS_Magical.IAS_Magical" "/Game/_DRGModding/CosmeticsMods/Mod_VoidPowerAnimation/Animations/MagicalPlasma_Equip_Montage.MagicalPlasma_Equip_Montage" false)
        (`/Game/_DRGModding/_Frameworks/BML_Framework.UpdateAnims(AmmoDrivenWeapon)` _as_wpn_charge_blaster "/Game/_DRGModding/CosmeticsMods/Mod_VoidPowerAnimation/Animations/MagicalPlasma_Fire_Normal_Montage.MagicalPlasma_Fire_Normal_Montage" null null (`|MakeArray` (make `ItemAnimationItem` "/Game/CharacterStructure/Gear_Pistol/FP/FP_Pistol_Basic_Gunsling_A_Montage.FP_Pistol_Basic_Gunsling_A_Montage") :!type "ItemAnimationItem Structure"))
        (`/Game/_DRGModding/_Frameworks/BML_Framework.UpdateAnims(ChargedWeapon)` _as_wpn_charge_blaster "/Game/_DRGModding/CosmeticsMods/Mod_VoidPowerAnimation/Animations/MagicalPlasma_Charge_Overheat_Montage.MagicalPlasma_Charge_Overheat_Montage" "/Game/_DRGModding/CosmeticsMods/Mod_VoidPowerAnimation/Animations/MagicalPlasma_Charge_Montage.MagicalPlasma_Charge_Montage")
        (`SceneComponent.K2_AttachToComponent` _scene (`PlayerCharacter.FPMesh` (`self.Player Character`)) "Dwarf_ArmRHand" "SnapToTarget" "SnapToTarget" "KeepRelative" true)
        (`SceneComponent.K2_SetRelativeLocation` _scene (15.680863 7.005105 0.374118) false false)
        (`PrimitiveComponent.SetOwnerNoSee` (`/Game/_DRGModding/_Frameworks/BML_Framework.GetAllFPComps` _as_wpn_charge_blaster) true)
        (`SceneComponent.K2_SetRelativeLocation` (`AnimatedItem.FPMesh` _as_wpn_charge_blaster) (0.0 -14.0 0.0) false false)
        (`SceneComponent.K2_AttachToComponent` _skullringroot (`PlayerCharacter.FPMesh` (`self.Player Character`)) "Dwarf_ArmRDigit05" "SnapToTarget" "SnapToTarget" "SnapToTarget" true)
        (`SceneComponent.K2_SetRelativeTransform` _skullringroot (`KismetMathLibrary.MakeTransform` (3.235015 -1.028818 0.258222) (struct :`Pitch` 90.0 :`Yaw` 1059.44397 :`Roll` 521.316895) (1.345 1.345 1.345)) false false)
        (add `ChargedWeapon.OnChargeChanged` _as_wpn_charge_blaster_2 (delegate `OnChargeChanged_Event_0`))
        (add `ChargedWeapon.OnHeatChanged` _as_wpn_charge_blaster_2 (delegate `OnHeatChanged_Event_0`))))))

(event `OnChargeChanged_Event_0`
  (params (charge :type "Float (double-precision)"))
  ;[1 1 1] On Item Equipped - Change animations, bind events.
  (`MaterialInstanceDynamic.SetScalarParameterValue` (`self.DMI(SkullEyes)`) "SlideParameter" (`KismetMathLibrary.Conv_BoolToDouble` (== charge 1.0))))

(event `OnHeatChanged_Event_0`
  (params (charge :type "Float (double-precision)"))
  ;[1 1 1] On Item Equipped - Change animations, bind events.
  (`MaterialInstanceDynamic.SetScalarParameterValue` (`self.DMI(Skull)`) "Overheat - Phase (0-1)" charge))

(event `/Game/_DRGModding/_Tools/DummyPlayerCharacter/BPI_DummyEvents.OnItemUnequipped(Dummy)`
  (params (Item :type "Item Object Reference"))
  ;[1 1 1] Unequipped - Hide skull ring and disable input, unbind the OnMontage event.
  (if (`self.IsInitialized`)
    (`/Game/_DRGModding/_Frameworks/BML_Framework.CompareClass(Item)` Item "/Game/WeaponsNTools/ChargeBlaster/WPN_ChargeBlaster.WPN_ChargeBlaster_C"
      (:`Class Match`
        (remove `AnimInstance.OnMontageStarted` (`SkeletalMeshComponent.GetAnimInstance` (`PlayerCharacter.FPMesh` (`self.Player Character`))) (`|CreateDelegate` :!event `OnMontageStarted_Event_0`))
        (`SceneComponent.SetVisibility` (`self.SkullRingRoot`) false true)))))

(event `OnMontageStarted_Event_0`
  (params (Montage :type "AnimMontage Object Reference"))
  ;[1 1 1] If playing montage is the same with plasma charger's overheat montage, execute On Overheat.
  (if (== Montage "/Game/_DRGModding/CosmeticsMods/Mod_VoidPowerAnimation/Animations/MagicalPlasma_Charge_Overheat_Montage.MagicalPlasma_Charge_Overheat_Montage")
    (`self.OnOverheat`)
    (elif (== Montage "/Game/CharacterStructure/Gear_Pistol/FP/FP_Pistol_Basic_Gunsling_A_Montage.FP_Pistol_Basic_Gunsling_A_Montage")
      (`self.PlayGunsling`))))

(event `DisableEffect`
  ;[1 1 1] Change overheating niagara effect's spawn rate
  (`FXSystemComponent.SetFloatParameter` (`self.OverheatEffect`) "SpawnRate" 0.0))

(event `OnOverheat`
  ;[1 1 1] Change overheating niagara effect's spawn rate
  (`KismetSystemLibrary.K2_SetTimerDelegate` (delegate `DisableEffect`) 1.0)
  (`FXSystemComponent.SetFloatParameter` (`self.OverheatEffect`) "SpawnRate" 300.0))

(event `PlayGunsling`
  (bind _chargesoundr (`self.ChargeSoundR`))
  (bind _chargesoundl (`self.ChargeSoundL`))
  (bind _chargesoundl_2 (`self.ChargeSoundL`))
  (bind _chargesoundr_2 (`self.ChargeSoundR`))
  ;[1 1 1] CycleItem - Play Overrided gunsling animation for FPMesh
  (bind _notifyname (`|PlayMontage` (`PlayerCharacter.FPMesh` (`self.Player Character`)) (select `bool` (== (`AmmoDrivenWeapon.ClipCount` (`self.As WPN Charge Blaster`)) 0) :`false` "/Game/_DRGModding/CosmeticsMods/Mod_VoidPowerAnimation/Animations/MagicalPlasma_Gunsling_01_Montage.MagicalPlasma_Gunsling_01_Montage" :`true` "/Game/_DRGModding/CosmeticsMods/Mod_VoidPowerAnimation/Animations/MagicalPlasma_Gunsling_01_Empty_Montage.MagicalPlasma_Gunsling_01_Empty_Montage" :!type "AnimMontage Object Reference") :!label _label_4)
    (:`OnCompleted`
      (`ActorComponent.Deactivate` (`self.ChargeEffectL`) :!label _label_5)
      (`ActorComponent.Deactivate` (`self.ChargeEffectR`))
      (`/Engine/EditorBlueprintResources/StandardMacros.IsValid` _chargesoundl
        (:`Is Valid`
          (`AudioComponent.Stop` _chargesoundl))
        (:`Is Not Valid`
          (`/Engine/EditorBlueprintResources/StandardMacros.IsValid` _chargesoundr
            (:`Is Valid`
              (`AudioComponent.Stop` _chargesoundr))))))
    (:`OnBlendOut`
      (goto _label_5))
    (:`OnInterrupted`
      (goto _label_5))
    (:`OnNotifyBegin`
      (switch `name` _notifyname
        (:`Start`
          (`self.SpawnChargeCosmetic`))
        (:`EndL`
          (`self.ExplodeCosmetic` (`self.ChargeEffectL`))
          (`/Engine/EditorBlueprintResources/StandardMacros.IsValid` _chargesoundl_2
            (:`Is Valid`
              (`AudioComponent.Stop` _chargesoundl_2))))
        (:`EndR`
          (`self.ExplodeCosmetic` (`self.ChargeEffectR`))
          (`/Engine/EditorBlueprintResources/StandardMacros.IsValid` _chargesoundr_2
            (:`Is Valid`
              (`AudioComponent.Stop` _chargesoundr_2))))))))

(event `InputAction|Cycleitem`
  (params (Key :type "Key Structure"))
  ;[1 0 0] I think I should not do this. Make a problem for some users.
  (:`Pressed`
    (if (not (`AnimInstance.IsAnyMontagePlaying` (`SkeletalMeshComponent.GetAnimInstance` (`PlayerCharacter.FPMesh` (`self.Player Character`)))))
      (goto _label_4))))

(fn `AddEffects`
  (params (PlayerCharacter :type "Actor Object Reference"))
  (bind _chargeeffectl (`self.ChargeEffectL`))
  (bind _chargeeffectr (`self.ChargeEffectR`))
  (`/Engine/EditorBlueprintResources/StandardMacros.IsValid` (`self.OverheatEffect`)
    (:`Is Valid`
      _)
    (:`Is Not Valid`
      (bind _returnvalue (`AddComponent|NODE_AddFirstPersonNiagaraComponent-0` :`self` PlayerCharacter))
      (set `self.OverheatEffect` _returnvalue)))
  (`SceneComponent.K2_AttachToComponent` (`self.OverheatEffect`) (`PlayerCharacter.FPMesh` (`self.Player Character`)) "None" "SnapToTarget" "SnapToTarget" "SnapToTarget" true)
  (`/Engine/EditorBlueprintResources/StandardMacros.IsValid` (`self.ChargeEffectL`)
    (:`Is Valid`
      _)
    (:`Is Not Valid`
      (bind _returnvalue_2 (`AddComponent|NODE_AddFirstPersonParticleSystemComponent-0` :`self` (`self.Player Character`)))
      (set `self.ChargeEffectL` _returnvalue_2)))
  (`SceneComponent.K2_AttachToComponent` _chargeeffectl (`PlayerCharacter.FPMesh` (`self.Player Character`)) "Dwarf_ArmLHand" "SnapToTarget" "SnapToTarget" "SnapToTarget" true)
  (`SceneComponent.K2_SetRelativeLocation` _chargeeffectl (2.296128 8.111384 0.698794) false false)
  (`/Engine/EditorBlueprintResources/StandardMacros.IsValid` (`self.ChargeEffectR`)
    (:`Is Valid`
      _)
    (:`Is Not Valid`
      (bind _returnvalue_3 (`AddComponent|NODE_AddFirstPersonParticleSystemComponent-1` :`self` (`self.Player Character`)))
      (set `self.ChargeEffectR` _returnvalue_3)))
  (`SceneComponent.K2_AttachToComponent` _chargeeffectr (`PlayerCharacter.FPMesh` (`self.Player Character`)) "Dwarf_ArmRHand" "SnapToTarget" "SnapToTarget" "SnapToTarget" true)
  (`SceneComponent.K2_SetRelativeLocation` _chargeeffectr (2.296128 5.72475 1.0) false false))

(fn `ExplodeCosmetic`
  (params (InputPin :type "FirstPersonParticleSystemComponent Object Reference"))
  (bind _returnvalue (`SceneComponent.K2_GetComponentLocation` InputPin))
  (`ActorComponent.Deactivate` InputPin)
  (`GameplayStatics.SpawnEmitterAtLocation` "/Game/WeaponsNTools/ChargeBlaster/Particles/P_ChargedProjectileHit.P_ChargedProjectileHit" _returnvalue)
  (`GameplayStatics.PlaySoundAtLocation` "/Game/Audio/SFX/WeaponsNTools/WPN_ChargeBlaster/ChargeBlaster_Overheat_Cue.ChargeBlaster_Overheat_Cue" _returnvalue (struct) 1.0 1.0 0.0 null null null))

(fn `SpawnChargeCosmetic`
  (bind _chargeeffectl (`self.ChargeEffectL`))
  (`ActorComponent.Activate` _chargeeffectl true)
  (`ActorComponent.Activate` (`self.ChargeEffectR`) true)
  (bind _returnvalue (`GameplayStatics.SpawnSoundAttached` "/Game/Audio/SFX/WeaponsNTools/WPN_ChargeBlaster/ChargeBlaster_SpinUp_Cue.ChargeBlaster_SpinUp_Cue" _chargeeffectl "None" (0.0 0.0 0.0) (struct) "KeepRelativeOffset" false 1.0 1.0 0.0 null null))
  (set `self.ChargeSoundL` _returnvalue)
  (bind _returnvalue_2 (`GameplayStatics.SpawnSoundAttached` "/Game/Audio/SFX/WeaponsNTools/WPN_ChargeBlaster/ChargeBlaster_SpinUp_Cue.ChargeBlaster_SpinUp_Cue" (`self.ChargeEffectR`) "None" (0.0 0.0 0.0) (struct) "KeepRelativeOffset" false 1.0 1.0 0.0 null null))
  (set `self.ChargeSoundR` _returnvalue_2))

(fn `UserConstructionScript`)