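; Mod actor for the ACVD cosmetic HUD, which creates HUD_ACVD_Main for the local player.
; Outside the space rig it polls for HUD_Main and collapses it first.
; After a short delay it plays startup animations and popups, then enables Tick.
; Tick maps player speed to a smoothed 0–1 scale for the combat HUD; the health-change binding is never run.
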(event `OnInitialize`
  (params (IsInSpacerig :type Boolean))
  (bind _hud_acvd_startup (`/Game/_DRGModding/CosmeticsMods/Mod_ACVDHud/HUD_ACVD_Main.HUD_ACVD_StartUp` (`self.As HUD ACVD Main`)))
  (set `self.Is in Spacerig` IsInSpacerig)
  (bind _playercharacter (`/Game/_DRGModding/_Frameworks/BML_Framework.GetLocalPlayerCharacter(Macro)` true)
    (:`Exec`
      (set `self.Player Character` _playercharacter)
      (if (not (`self.Is in Spacerig`))
        (bind _foundwidgets (`WidgetBlueprintLibrary.GetAllWidgetsOfClass` "/Game/UI/MainOnscreenHUD/HUD_Main.HUD_Main_C" :!label _label))
        (`/Game/_DRGModding/_Frameworks/BML_Framework.IsValid(Array)` _foundwidgets
          (:`IsValid`
            (for _array_element _foundwidgets
              (`Widget.SetVisibility` _array_element "Collapsed")))
          (:`IsNotValid`
            (`KismetSystemLibrary.Delay` 0.4)
            (goto _label))))
      (bind _outputpin (`/Game/_DRGModding/_Frameworks/BML_Framework.WaitUntil(CreateWidge)` "/Game/_DRGModding/CosmeticsMods/Mod_ACVDHud/HUD_ACVD_Main.HUD_ACVD_Main_C")
        (:`true`
          (bind _ashud_acvd_main (cast `/Game/_DRGModding/CosmeticsMods/Mod_ACVDHud/HUD_ACVD_Main` _outputpin))
          (bind _output_get (set `self.As HUD ACVD Main` _ashud_acvd_main))
          (`KismetSystemLibrary.Delay` 1.0)
          (`/Game/_DRGModding/CosmeticsMods/Mod_ACVDHud/HUD_ACVD_Main.PlayStartup` _output_get)
          (bind _hud_acvd_scanner (`/Game/_DRGModding/CosmeticsMods/Mod_ACVDHud/HUD_ACVD_Main.HUD_ACVD_Scanner` _output_get))
          (`UserWidget.PlayAnimation` _hud_acvd_scanner (`/Game/_DRGModding/CosmeticsMods/Mod_ACVDHud/HUD_ACVD_Scanner.StartUp` _hud_acvd_scanner) 0.0 1 "Forward" 1.0 false)
          (`/Game/_DRGModding/CosmeticsMods/Mod_ACVDHud/UI_ACVD_StartUp_Error_Popup.Start` (`/Game/_DRGModding/CosmeticsMods/Mod_ACVDHud/HUD_ACVD_StartUp.UI_ACVD_StartUp_Error_Popup` _hud_acvd_startup))
          (`/Game/_DRGModding/CosmeticsMods/Mod_ACVDHud/UI_ACVD_StartUp_SimpleBox_PopUp.Start` (`/Game/_DRGModding/CosmeticsMods/Mod_ACVDHud/HUD_ACVD_StartUp.UI_ACVD_StartUp_SimpleBox_PopUp` _hud_acvd_startup))
          (`self.SetActorTickEnabled` true))))))

(event `self.ReceiveTick`
  (params (DeltaSeconds :type "Float (single-precision)"))
  (bind _output_get (set `self.Current` (`KismetMathLibrary.FClamp` (`KismetMathLibrary.FInterpTo_Constant` (`self.Current`) (`KismetMathLibrary.MapRangeClamped` (`KismetMathLibrary.VSize` (`MovementComponent.Velocity` (`Character.CharacterMovement` (`self.Player Character`)))) 0.0 600.0 0.0 1.0) (`GameplayStatics.GetWorldDeltaSeconds`) 1.0))))
  (`/Game/_DRGModding/CosmeticsMods/Mod_ACVDHud/HUD_ACVD_Combat.SetScale` (`/Game/_DRGModding/CosmeticsMods/Mod_ACVDHud/HUD_ACVD_Main.HUD_ACVD_Combat` (`self.As HUD ACVD Main`)) _output_get))

(fn `UserConstructionScript`)