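; Pole actor for a cosmetic video player mod that carries a screen which slowly turns to face the local player.
; InitializeWithDonkey spawns a BP_VideoPlayer on the display attach point, applies material and height offset, optionally runs its cave setup, and scales the pole mesh.
; It also caches the local first-person camera.
; Tick interpolates the display toward that camera in actor space, applying only yaw so the screen stays upright.
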(event `InitializeWithDonkey`
  (params (Material :type "MaterialInterface Object Reference") (Scale :type "Float (double-precision)") (ZOffset :type "Float (double-precision)") (DisableInitCave :type Boolean))
  (bind _returnvalue (`|SpawnActorFromClass` "/Game/_DRGModding/CosmeticsMods/VideoPLayer/BP_VideoPlayer.BP_VideoPlayer_C" (`KismetMathLibrary.MakeTransform` (0.0 0.0 0.0) (struct) (`KismetMathLibrary.Conv_DoubleToVector` 0.3)) "AlwaysSpawn" "OverrideRootScale" null null))
  (bind _output_get (set `self.VideoPlayer` _returnvalue))
  (`self.K2_AttachToComponent` _output_get (`self.AP_Display`) "None" "SnapToTarget" "SnapToTarget" "KeepWorld" true)
  (`self.K2_SetActorRelativeRotation` _output_get (struct :`Yaw` 90.0) false false)
  (if (not DisableInitCave)
    (`/Game/_DRGModding/CosmeticsMods/VideoPLayer/BP_VideoPlayer.InitCave` _output_get))
  (`/Game/_DRGModding/CosmeticsMods/VideoPLayer/BP_VideoPlayer.SetMaterial` _output_get Material)
  (`self.SetActorEnableCollision` _output_get false)
  (`self.K2_SetActorRelativeLocation` (`self.VideoPlayer`) (`KismetMathLibrary.MakeVector` 0.0 0.0 ZOffset) false false)
  (bind _playercharacter (`/Game/_DRGModding/_Frameworks/BML_Framework.GetLocalPlayerCharacter(Macro)` true)
    (:`Exec`
      (set `self.First Person Camera` (`PlayerCharacter.FirstPersonCamera` _playercharacter))
      (if (not (`KismetMathLibrary.NearlyEqual_FloatFloat` Scale))
        (`SceneComponent.SetRelativeScale3D` (`self.SM_Pole`) (`KismetMathLibrary.Conv_DoubleToVector` Scale))))))

(event `self.ReceiveTick`
  (params (DeltaSeconds :type "Float (single-precision)"))
  (bind (_returnvalue_roll _returnvalue_pitch _returnvalue_yaw) (`KismetMathLibrary.BreakRotator` (`KismetMathLibrary.MakeRotFromX` (`KismetMathLibrary.InverseTransformDirection` (`self.GetTransform`) (- (`SceneComponent.K2_GetComponentLocation` (`self.First Person Camera`)) (`SceneComponent.K2_GetComponentLocation` (`self.AP_Display`)))))))
  (`/Engine/EditorBlueprintResources/StandardMacros.IsValid` (`self.First Person Camera`)
    (:`Is Valid`
      (bind _output_get (set `self.CacheRotation` (`KismetMathLibrary.RInterpTo` (`self.CacheRotation`) (`KismetMathLibrary.MakeRotator` _returnvalue_roll _returnvalue_pitch (- _returnvalue_yaw 90.0)) (`GameplayStatics.GetWorldDeltaSeconds`) 2.0)))
      (`SceneComponent.K2_SetRelativeRotation` (`self.AP_Display`) (`KismetMathLibrary.MakeRotator` 0.0 0.0 (.yaw _output_get)) false false))))

(fn `UserConstructionScript`)