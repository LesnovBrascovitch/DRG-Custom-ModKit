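; Video player prop for a DRG cosmetics mod that plays randomly picked media sources with attenuated sound.
; Begin play, using the prop, the ChangeVideo input and the end of a video all trigger a new random pick.
; Timers retry invalid sources and check that playback has started.
; InitCave swaps in cave sound attenuation, and SetMaterial changes the display mesh's screen material slot.
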(event `self.ReceiveBeginPlay`
  (bind _mediasource (`self.MediaSource`))
  (bind _target (`self.Target`))
  (`/Game/_DRGModding/_Frameworks/BML_Framework.EnableInput(WaitUntil)`)
  (add `MediaPlayer.OnEndReached` (`self.Target`) (delegate `OnEndReached_Event_0`))
  (set `SynthComponent.AttenuationSettings` "/Game/_DRGModding/CosmeticsMods/VideoPLayer/VideoPlayer.VideoPlayer" (`self.MediaSound`))
  (set `self.MediaSource` (`KismetArrayLibrary.Array_Random` (`self.Media Source`)) :!label _label)
  (if (`MediaSource.Validate` _mediasource)
    (`MediaPlayer.OpenSource` _target _mediasource)
    (`MediaPlayer.Play` _target)
    (`KismetSystemLibrary.K2_ClearAndInvalidateTimerHandle` (stale _returnvalue))
    (`KismetSystemLibrary.K2_SetTimerDelegate` (delegate `CustomEvent_2`) 3.0)
    (else
      (bind _returnvalue (`KismetSystemLibrary.K2_SetTimerDelegate` (delegate `CustomEvent_1`) 1.0)))))

(event `OnEndReached_Event_0`
  (`KismetSystemLibrary.K2_SetTimerDelegate` (delegate `CustomEvent_0`) 2.0)
  (`MediaPlayer.Close` (`self.Target`)))

(event `CustomEvent_0`
  (goto _label))

(event `CustomEvent_2`
  (if (not (`MediaPlayer.IsPlaying` (`self.Target`)))
    (`self.CustomEvent_1`)))

(event `self.InstantUsable.OnUsedBy`
  (params (User :type "PlayerCharacter Object Reference") (Key :type "EInputKeys Enum" :default "Use"))
  (goto _label))

(event `InputAction|ChangeVideo`
  (params (Key :type "Key Structure"))
  (:`Pressed`
    (goto _label)))

(event `self.InstantUsable.OnClientBeginUse`
  (params (User :type "PlayerCharacter Object Reference") (Key :type "EInputKeys Enum" :default "Use"))
  (goto _label))

(event `CustomEvent_1`
  (goto _label))

(fn `InitCave`
  (set `SynthComponent.AttenuationSettings` "/Game/_DRGModding/CosmeticsMods/VideoPLayer/VideoPlayerCave.VideoPlayerCave" (`self.MediaSound`)))

(fn `SetMaterial`
  (params (Material :type "MaterialInterface Object Reference"))
  (`PrimitiveComponent.SetMaterial` (`self.SM_Display`) 4 Material))

(fn `UserConstructionScript`)