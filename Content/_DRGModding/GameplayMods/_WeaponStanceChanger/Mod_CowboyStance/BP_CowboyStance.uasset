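; Cowboy stance modifier for the revolver in a weapon stance changer mod, derived from a parent stance Blueprint.
; It overrides the parent's stat hooks to triple cached fire rate, cut pitch recoil sharply and assign its own hitscan spread curve.
; When it receives a revolver, it enlarges the bounds of the ammo counter mesh and first-person widget to try to prevent culling.
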(event `self.OnReceiveAmmoDrivenWeapon`
  (params (AmmoDrivenWeapon :type "AmmoDrivenWeapon Object Reference"))
  ;[1 1 1] Receive Ammo Driven Weapon - Change bounds scale for Ammo Counter mesh and widget to try preventing culling.
  (bind _aswpn_revolver (cast `/Game/WeaponsNTools/Revolver/WPN_Revolver` AmmoDrivenWeapon))
  (`PrimitiveComponent.SetBoundsScale` (`/Game/WeaponsNTools/Revolver/WPN_Revolver.Mesh_AmmoCounter` _aswpn_revolver) 100.0)
  (`PrimitiveComponent.SetBoundsScale` (`/Game/WeaponsNTools/Revolver/WPN_Revolver.FirstPersonWidget` _aswpn_revolver) 100.0) ; Try to prevent mesh culling from hands.
)

(fn `ChangeHitscanStats`
  (params (Hitscan :type "HitscanComponent Object Reference"))
  (`parent.ChangeHitscanStats` Hitscan)
  (`self.AssignSpreadCurve` Hitscan (`self.Spread Curve`)))

(fn `ChangeWeaponStats`
  (params (AmmoDrivenWeapon :type "AmmoDrivenWeapon Object Reference"))
  (bind _recoil_settings_cache_ (`self.Recoil Settings(Cache)`))
  (`parent.ChangeWeaponStats` AmmoDrivenWeapon)
  (set `AmmoDrivenWeapon.RateOfFire` (* (`self.Rate Of Fire(Cache)`) 3.0) AmmoDrivenWeapon) ; Increase fire rate based on default fire rate
  (set `AmmoDrivenWeapon.RecoilSettings` (make `RecoilSettings` (break `RecoilSettings` _recoil_settings_cache_) (make `RandRange` (* (break `RandRange` (`.RecoilPitch` (break `RecoilSettings` _recoil_settings_cache_))) 0.2) (* (`.Max` (break `RandRange` (`.RecoilPitch` (break `RecoilSettings` _recoil_settings_cache_)))) 0.2)) (`.RecoilYaw` (break `RecoilSettings` _recoil_settings_cache_)) (`.CanRecoilDown` (break `RecoilSettings` _recoil_settings_cache_)) (`.SpringStiffness` (break `RecoilSettings` _recoil_settings_cache_)) (`.CriticalDampening` (break `RecoilSettings` _recoil_settings_cache_)) (`.Mass` (break `RecoilSettings` _recoil_settings_cache_))) AmmoDrivenWeapon) ; Improve recoil
)

(fn `UserConstructionScript`
  (`parent.UserConstructionScript`))