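; Hawkeye weapon stance that gives the player a mark-and-execute shooting ability in slowed time.
; Activation eases global time dilation down and applies a movement penalty; deactivation reverses both and destroys markers.
; CallDonkey spawns markers at line-trace hits.
; Use restores normal time, then steps through markers, lerping control rotation onto each, firing the ammo-driven weapon directly and speeding up the aim timeline after every shot.
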(event `self.OnStanceActivated`
  (`self.SlowgameSpeed` true)
  (`/Game/_DRGModding/_Frameworks/BML_Framework.ToggleStatusEffect` true (`self.Player Character`) "/Game/_DRGModding/GameplayMods/_WeaponStanceChanger/Mod_Hawkeye/STE_HawkeyeMovementPenalty.STE_HawkeyeMovementPenalty_C"))

(event `self.OnPreStanceDeactivated`
  (bind _newvar_0_0 (`self.NewVar_0_0`))
  (`self.SlowgameSpeed` false)
  (`/Game/_DRGModding/_Frameworks/BML_Framework.ToggleStatusEffect` false (`self.Player Character`) "/Game/_DRGModding/GameplayMods/_WeaponStanceChanger/Mod_Hawkeye/STE_HawkeyeMovementPenalty.STE_HawkeyeMovementPenalty_C")
  (`self.K2_DestroyActor` _newvar_0_0)
  (`KismetArrayLibrary.Array_Clear` _newvar_0_0))

(event `SlowgameSpeed`
  (params (SlowStart :type Boolean))
  (if SlowStart
    (bind (_direction _newtrack_0) (`Timeline|Timeline_0` :!via `Reverse` :!label _label)
      (:`Update`
        (`GameplayStatics.SetGlobalTimeDilation` (`KismetMathLibrary.Lerp` 0.1 1.0 _newtrack_0))))
    (else
      (goto _label))))

(event `InputAction|CallDonkey`
  (params (Key :type "Key Structure"))
  (:`Pressed`
    (bind _location (`/Game/_DRGModding/_Frameworks/BML_Framework.QuickLinetrace` (`self.Player Character`))
      (:`OnHit`
        (bind _returnvalue (`|SpawnActorFromClass` "/Game/_DRGModding/GameplayMods/_WeaponStanceChanger/Mod_Hawkeye/BP_HawkeyeMarker.BP_HawkeyeMarker_C" (`KismetMathLibrary.MakeTransform` _location) "AlwaysSpawn" "OverrideRootScale" null null))
        (`KismetArrayLibrary.Array_AddUnique` (`self.NewVar_0_0`) _returnvalue)))))

(event `InputAction|Use`
  (params (Key :type "Key Structure"))
  (bind _timeline_1 (`self.Timeline_1`))
  (bind _as_ammo_driven_weapon (`self.As Ammo Driven Weapon`))
  (bind _output (`|GetArrayItem` (`self.NewVar_0_0`) (`self.NewVar_1`)))
  (bind _weaponfire (`AmmoDrivenWeapon.WeaponFire` _as_ammo_driven_weapon))
  (bind _returnvalue (`SceneComponent.GetSocketTransform` (`AnimatedItem.FPMesh` _as_ammo_driven_weapon) "Muzzle" "RTS_World"))
  (:`Pressed`
    (`GameplayStatics.SetGlobalTimeDilation` 1.0)
    (set `self.NewVar_1` 0)
    (`TimelineComponent.SetPlayRate` (`self.Timeline_1`) 1.0)
    (if (<= (`self.NewVar_1`) (`KismetArrayLibrary.Array_LastIndex` (`self.NewVar_0_0`))) :!label _label_2
      (`/Engine/EditorBlueprintResources/StandardMacros.IsValid` _output
        (:`Is Valid`
          (set `self.CacheOrigin` (`Controller.GetControlRotation` (`self.FSDPlayer Controller`)))
          (set `self.NewVar_2` (`KismetMathLibrary.FindLookAtRotation` (`SceneComponent.K2_GetComponentLocation` (`PlayerCharacter.FirstPersonCamera` (`self.Player Character`))) (`self.K2_GetActorLocation` _output)))
          (bind (_direction _newtrack_0) (`Timeline|Timeline_1` :!via `PlayFromStart`)
            (:`Update`
              (bind (_returnvalue_roll _returnvalue_pitch _returnvalue_yaw) (`KismetMathLibrary.BreakRotator` (`KismetMathLibrary.RLerp` (`self.CacheOrigin`) (`self.NewVar_2`) _newtrack_0 true)))
              (`Controller.SetControlRotation` (`self.FSDPlayer Controller`) (`KismetMathLibrary.MakeRotator` 0.0 _returnvalue_pitch _returnvalue_yaw)))
            (:`Finished`
              (`/Engine/EditorBlueprintResources/StandardMacros.IsValid` _weaponfire
                (:`Is Valid`
                  (`WeaponFireComponent.Fire` _weaponfire (.location _returnvalue) (`FSDConversionLibrary.VectorToNetQuantizeNormal` (`KismetMathLibrary.GetForwardVector` (`SceneComponent.K2_GetComponentRotation` (`PlayerCharacter.FirstPersonCamera` (`self.Player Character`))))) true)
                  (`GameplayStatics.PlaySoundAtLocation` (`AmmoDrivenWeapon.FireSound` (`self.As Ammo Driven Weapon`)) (.location _returnvalue) (struct) 1.0 1.0 0.0 null null null)
                  (`TimelineComponent.SetPlayRate` _timeline_1 (* (`TimelineComponent.GetPlayRate` _timeline_1) 1.3))
                  (`self.K2_DestroyActor` (`|GetArrayItem` (`self.NewVar_0_0`) (`self.NewVar_1`)))
                  (`/Engine/EditorBlueprintResources/StandardMacros.IncrementInt` (`self.NewVar_1`)
                    (:`  `
                      _)))
                (:`Is Not Valid`
                  _))
              (`KismetSystemLibrary.Delay` 0.2)
              (goto _label_2))))))))

(fn `UserConstructionScript`
  (`parent.UserConstructionScript`))