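; Usable console actor for the melee mod that sends the player to the melee customization level.
; On use, it caches the character ID (random in editor), level name and player transform in the MeleeSettingsSaveGame slot, then opens the level after a short delay.
; On BeginPlay, it restores and resets the cached transform, or opens the menu level immediately if EnableInstantInventoryMenu is set.
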(event `self.ReceiveBeginPlay`
  (bind _as_melee_save_game (`self.As Melee Save Game`))
  (if (`self.EnableInstantInventoryMenu`)
    (`GameplayStatics.OpenLevelBySoftObjectPtr` "/Game/_DRGModding/GameplayMods/_MeleeSystem/__InventoryMenu/LVL_CustomizationMelee.LVL_CustomizationMelee")
    (else
      (bind _playercharacter (`/Game/_DRGModding/_Frameworks/BML_Framework.GetLocalPlayerCharacter(Macro)` true)
        (:`Exec`
          (set `self.Player Character` _playercharacter)
          (bind _outputpin (`/Game/_DRGModding/_Frameworks/BML_Framework.HandleSaveGame` "/Game/_DRGModding/GameplayMods/_MeleeSystem/_HandleWeaponEquip/MeleeSaveGame.MeleeSaveGame_C" true "MeleeSettingsSaveGame")
            (:`then`
              (bind _asmelee_save_game (cast `/Game/_DRGModding/GameplayMods/_MeleeSystem/_HandleWeaponEquip/MeleeSaveGame` _outputpin))
              (set `self.As Melee Save Game` _asmelee_save_game)
              (if (not (`KismetMathLibrary.NearlyEqual_TransformTransform` (`/Game/_DRGModding/GameplayMods/_MeleeSystem/_HandleWeaponEquip/MeleeSaveGame.CacheTransform` (`self.As Melee Save Game`)) (`KismetMathLibrary.MakeTransform` (0.0 0.0 0.0))))
                (`self.K2_SetActorTransform` (`self.Player Character`) (`/Game/_DRGModding/GameplayMods/_MeleeSystem/_HandleWeaponEquip/MeleeSaveGame.CacheTransform` _as_melee_save_game) false false)
                (set `/Game/_DRGModding/GameplayMods/_MeleeSystem/_HandleWeaponEquip/MeleeSaveGame.CacheTransform` (`KismetMathLibrary.MakeTransform` (0.0 0.0 0.0)) _as_melee_save_game)
                (`/Game/_DRGModding/_Frameworks/BML_Framework.SaveToSlot(Macro)` (`self.As Melee Save Game`) true "MeleeSettingsSaveGame")))))))))

(event `/Game/_DRGModding/_Tools/DummyPlayerCharacter/BPI_DummyEvents.OnUsedBy`
  (bind _as_melee_save_game (`self.As Melee Save Game`))
  (`/Game/_DRGModding/_Frameworks/BML_Framework.IsInDRG` :!label _label
    (:`In DRG`
      (set `/Game/_DRGModding/GameplayMods/_MeleeSystem/_HandleWeaponEquip/MeleeSaveGame.CachedCharacterID` (`PlayerCharacter.characterID` (`self.Player Character`)) (`self.As Melee Save Game`)))
    (:`In Editor`
      (set `/Game/_DRGModding/GameplayMods/_MeleeSystem/_HandleWeaponEquip/MeleeSaveGame.CachedCharacterID` (`/Game/_DRGModding/_Tools/DummyPlayerCharacter/BML_EditorCompatible.GetCharacterIDByRand`) (`self.As Melee Save Game`))))
  (bind _returnvalue (`GameplayStatics.GetCurrentLevelName` true))
  (set `/Game/_DRGModding/GameplayMods/_MeleeSystem/_HandleWeaponEquip/MeleeSaveGame.CacheLevelName` _returnvalue _as_melee_save_game)
  (set `/Game/_DRGModding/GameplayMods/_MeleeSystem/_HandleWeaponEquip/MeleeSaveGame.CacheTransform` (`self.GetTransform` (`self.Player Character`)) _as_melee_save_game)
  (`/Game/_DRGModding/_Frameworks/BML_Framework.SaveToSlot(Macro)` (`self.As Melee Save Game`) true "MeleeSettingsSaveGame")
  (`KismetSystemLibrary.Delay` 0.2)
  (`GameplayStatics.OpenLevelBySoftObjectPtr` "/Game/_DRGModding/GameplayMods/_MeleeSystem/__InventoryMenu/LVL_CustomizationMelee.LVL_CustomizationMelee"))

(event `self.InstantUsable.OnUsedBy`
  (params (User :type "PlayerCharacter Object Reference") (Key :type "EInputKeys Enum" :default "Use"))
  (goto _label))

(fn `UserConstructionScript`)