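; Inventory scene actor for the melee mod, where the player picks a melee weapon and three upgrade tiers per character class.
; BeginPlay loads the MeleeSaveGame, becomes the view target and binds the Menu_InventoryMelee buttons.
; Cycling weapons or classes saves the current selection, then refreshes the widget, upgrade lists and preview meshes' idle animations.
; Selections persist in nested character-to-weapon-to-upgrade maps, and closing saves and reopens the cached level.
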(event `OnButtonPressed_Event_0`
  (params (IsRight :type Boolean))
  (bind _meleeweapons (`self.MeleeWeapons`))
  (bind _selectedinventoryinfo (`self.SelectedInventoryInfo`))
  (bind _index (`self.Index`))
  (`self.SaveCurrenbt`)
  (if IsRight
    (bind _output (`/Game/_DRGModding/_Tools/DummyPlayerCharacter/BML_EditorCompatible.IncrementArray(EC)` _index _meleeweapons))
    (set `self.SelectedInventoryInfo` _output)
    (else
      (bind _output_2 (`/Game/_DRGModding/_Tools/DummyPlayerCharacter/BML_EditorCompatible.DecrementArray(EC)` _index _meleeweapons))
      (set `self.SelectedInventoryInfo` _output_2)))
  (`/Game/_DRGModding/GameplayMods/_MeleeSystem/__InventoryMenu/Menu_InventoryMelee.OnItemSelected` (`self.As Menu Inventory Melee`) _selectedinventoryinfo)
  (`self.OnItemSelected` _selectedinventoryinfo))

(event `OnItemSelected`
  (params (InventoryInfo :type "/Game/_DRGModding/GameplayMods/_MeleeSystem/__InventoryMenu/InventoryInfoMelee Object Reference"))
  (bind _output_get (set `self.Inventory Info` InventoryInfo))
  (`KismetSystemLibrary.PrintString` (`KismetStringLibrary.Concat_StrStr` "OnItemSelected Event -> Inventory Info -  " (`KismetSystemLibrary.GetDisplayName` _output_get)) true true (struct :`G` 0.66 :`B` 1.0 :`A` 1.0) 10.0)
  (`self.UpdateMeshAnimations` (`self.Inventory Info`))
  (`self.AddUpgradesToList`))

(event `self.ReceiveBeginPlay`
  (bind _outputpin (`/Game/_DRGModding/_Frameworks/BML_Framework.HandleSaveGame` "/Game/_DRGModding/GameplayMods/_MeleeSystem/_HandleWeaponEquip/MeleeSaveGame.MeleeSaveGame_C" true "MeleeSettingsSaveGame")
    (:`then`
      (bind _asmelee_save_game (cast `/Game/_DRGModding/GameplayMods/_MeleeSystem/_HandleWeaponEquip/MeleeSaveGame` _outputpin))
      (bind _output_get (set `self.As Melee Save Game` _asmelee_save_game))
      (set `self.CurrentCharacterID` (`/Game/_DRGModding/GameplayMods/_MeleeSystem/_HandleWeaponEquip/MeleeSaveGame.CachedCharacterID` _output_get))
      (for _array_element (`.EquippedUpgrade_7_5F3F6BF74ADAAA2B0545D8B457747E49` (break `/Game/_DRGModding/GameplayMods/_MeleeSystem/_HandleWeaponEquip/S_MeleeEquippedUpgrade` (`BlueprintMapLibrary.Map_Find` (break `/Game/_DRGModding/GameplayMods/_MeleeSystem/_HandleWeaponEquip/S_MeleeUpgrade` (`BlueprintMapLibrary.Map_Find` (`/Game/_DRGModding/GameplayMods/_MeleeSystem/_HandleWeaponEquip/MeleeSaveGame.Equipped` (`self.As Melee Save Game`)) "/Game/Character/GunnerID.GunnerID")) "/Game/_DRGModding/GameplayMods/_MeleeSystem/__InventoryMenu/IIM_GRBlade.IIM_GRBlade")))
        (`KismetSystemLibrary.PrintString` (`KismetStringLibrary.Concat_StrStr` "Loaded - " (`KismetSystemLibrary.GetDisplayName` (`self.SelectedInventoryInfo`)) " - " (`KismetSystemLibrary.GetDisplayName` _array_element)) true true (struct :`R` 1.0 :`G` 0.778078 :`A` 1.0) 7.0))
      (for _array_element_2 (`|MakeArray` (`self.MeshBody`) (`self.MeshHead`))
        (bind _asabp_inventory_melee (cast `/Game/_DRGModding/GameplayMods/_MeleeSystem/__InventoryMenu/ABP_InventoryMelee` (`SkeletalMeshComponent.GetAnimInstance` _array_element_2)))
        (`KismetArrayLibrary.Array_Add` (`self.As ABP Inventory Melee`) _asabp_inventory_melee))
      (`GameplayStatics.PlaySound2D` "/Game/Audio/SFX/UI/Menu/DeepDiveMenu/TerminalAmbienceFocused_Cue.TerminalAmbienceFocused_Cue" 1.0 1.0 0.0 null null)
      (bind _fsdplayercontroller (`/Game/_DRGModding/_Frameworks/BML_Framework.GetLocalPlayerController(Macro)` true)
        (:`Completed`
          (set `self.FSDPlayer Controller` _fsdplayercontroller)
          (`PlayerController.SetViewTargetWithBlend` _fsdplayercontroller self 0.0 "VTBlend_Linear" 0.0 false)
          (bind _outputpin_2 (`/Game/_DRGModding/_Frameworks/BML_Framework.WaitUntil(CreateWidge)` "/Game/_DRGModding/GameplayMods/_MeleeSystem/__InventoryMenu/Menu_InventoryMelee.Menu_InventoryMelee_C")
            (:`true`
              (bind _asmenu_inventory_melee (cast `/Game/_DRGModding/GameplayMods/_MeleeSystem/__InventoryMenu/Menu_InventoryMelee` _outputpin_2))
              (set `self.As Menu Inventory Melee` _asmenu_inventory_melee)
              (add `/Game/_DRGModding/GameplayMods/_MeleeSystem/__InventoryMenu/UI_InvMelee_WeaponTexts.OnButtonPressed` (`/Game/_DRGModding/GameplayMods/_MeleeSystem/__InventoryMenu/Menu_InventoryMelee.invm` (`self.As Menu Inventory Melee`)) (delegate `OnButtonPressed_Event_0`))
              (add `/Game/_DRGModding/GameplayMods/_MeleeSystem/__InventoryMenu/UI_InvMelee_Close.OnClicked` (`/Game/_DRGModding/GameplayMods/_MeleeSystem/__InventoryMenu/Menu_InventoryMelee.UI_InvMelee_Close` (`self.As Menu Inventory Melee`)) (delegate `OnClicked_Event_0`))
              (add `/Game/_DRGModding/_Frameworks/Widget/CUI_Button_Arrow.OnClicked` (`/Game/_DRGModding/GameplayMods/_MeleeSystem/__InventoryMenu/Menu_InventoryMelee.CharacterButton` (`self.As Menu Inventory Melee`)) (delegate `OnClicked_Event_1`))
              (set `PlayerController.bShowMouseCursor` true (`self.FSDPlayer Controller`))
              (bind _characterid (`self.GetCurrentCharacterClass`))
              (`self.OnCharacterChanged` _characterid))))))))

(event `OnClicked_Event_1`
  (`self.SaveCurrenbt`)
  (bind _output (`/Game/_DRGModding/_Tools/DummyPlayerCharacter/BML_EditorCompatible.DecrementArray(EC)` (`self.CharacterIndex`) (`self.Character ID`)))
  (`self.OnCharacterChanged` _output))

(event `OnClicked_Event_0`
  (`self.SaveCurrenbt`)
  (`KismetSystemLibrary.Delay` 1.0)
  (`GameplayStatics.OpenLevel` (`KismetStringLibrary.Conv_StringToName` (`/Game/_DRGModding/GameplayMods/_MeleeSystem/_HandleWeaponEquip/MeleeSaveGame.CacheLevelName` (`self.As Melee Save Game`)))))

(fn `AddUpgradesToList`
  (locals (NewLocalVar_3 :type "/Game/_DRGModding/GameplayMods/_MeleeSystem/_HandleWeaponEquip/S_MeleeEquippedUpgrade Structure"))
  (bind _as_menu_inventory_melee (`self.As Menu Inventory Melee`))
  (bind _inventory_info (`self.Inventory Info`))
  (bind _newlocalvar_3 (`local.NewLocalVar_3`))
  (bind (_value _returnvalue) (`BlueprintMapLibrary.Map_Find` (break `/Game/_DRGModding/GameplayMods/_MeleeSystem/_HandleWeaponEquip/S_MeleeUpgrade` (`BlueprintMapLibrary.Map_Find` (`/Game/_DRGModding/GameplayMods/_MeleeSystem/_HandleWeaponEquip/MeleeSaveGame.Equipped` (`self.As Melee Save Game`)) (`self.CurrentCharacterID`))) (`self.Inventory Info`)))
  (if _returnvalue
    (set `local.NewLocalVar_3` _value)
    (else
      (`KismetSystemLibrary.PrintString` "EEEEEEEEEEEE" true true (struct :`R` 1.0 :`G` 0.049738 :`A` 1.0))))
  (`/Game/_DRGModding/GameplayMods/_MeleeSystem/__InventoryMenu/UI_InvMelee_Upgrade.OnInitialize` (`/Game/_DRGModding/GameplayMods/_MeleeSystem/__InventoryMenu/Menu_InventoryMelee.UI_InvMelee_Upgrade_Tier1` _as_menu_inventory_melee) (`/Game/_DRGModding/GameplayMods/_MeleeSystem/__InventoryMenu/InventoryInfoMelee.Tier1` _inventory_info) _newlocalvar_3)
  (`/Game/_DRGModding/GameplayMods/_MeleeSystem/__InventoryMenu/UI_InvMelee_Upgrade.OnInitialize` (`/Game/_DRGModding/GameplayMods/_MeleeSystem/__InventoryMenu/Menu_InventoryMelee.UI_InvMelee_Upgrade_Tier2` _as_menu_inventory_melee) (`/Game/_DRGModding/GameplayMods/_MeleeSystem/__InventoryMenu/InventoryInfoMelee.Tier2` _inventory_info) _newlocalvar_3)
  (`/Game/_DRGModding/GameplayMods/_MeleeSystem/__InventoryMenu/UI_InvMelee_Upgrade.OnInitialize` (`/Game/_DRGModding/GameplayMods/_MeleeSystem/__InventoryMenu/Menu_InventoryMelee.UI_InvMelee_Upgrade_Tier3` _as_menu_inventory_melee) (`/Game/_DRGModding/GameplayMods/_MeleeSystem/__InventoryMenu/InventoryInfoMelee.Tier3` _inventory_info) _newlocalvar_3)
  (for _array_element (`.EquippedUpgrade_7_5F3F6BF74ADAAA2B0545D8B457747E49` (break `/Game/_DRGModding/GameplayMods/_MeleeSystem/_HandleWeaponEquip/S_MeleeEquippedUpgrade` (`local.NewLocalVar_3`)))
    (`KismetSystemLibrary.PrintString` (`KismetStringLibrary.Concat_StrStr` "Loaded - " (`KismetSystemLibrary.GetDisplayName` (`self.SelectedInventoryInfo`)) " - " (`KismetSystemLibrary.GetDisplayName` _array_element)))))

(fn `GetCurrentCharacterClass`
  (returns (CharacterID :type "PlayerCharacterID Object Reference"))
  (locals (Local_PlayerID :type "PlayerCharacterID Object Reference"))
  (bind _local_playerid (`local.Local_PlayerID`))
  (bind _output_get (set `local.Local_PlayerID` (`/Game/_DRGModding/GameplayMods/_MeleeSystem/_HandleWeaponEquip/MeleeSaveGame.CachedCharacterID` (`self.As Melee Save Game`))))
  (set `self.CharacterIndex` (`KismetArrayLibrary.Array_Find` (`self.Character ID`) _output_get))
  (set `self.CurrentCharacterID` _local_playerid)
  (return _local_playerid))

(fn `GetEquippedUpgrades`
  (returns (EquippedUpgrades :type "Array of /Game/_DRGModding/GameplayMods/_MeleeSystem/__InventoryMenu/Upgrade/MeleeUpgrade Object Reference"))
  (locals (NewLocalVar_0 :type "Array of /Game/_DRGModding/GameplayMods/_MeleeSystem/__InventoryMenu/Upgrade/MeleeUpgrade Object Reference"))
  (bind _as_menu_inventory_melee (`self.As Menu Inventory Melee`))
  (for _array_element (`|MakeArray` (`/Game/_DRGModding/GameplayMods/_MeleeSystem/__InventoryMenu/Menu_InventoryMelee.UI_InvMelee_Upgrade_Tier1` _as_menu_inventory_melee) (`/Game/_DRGModding/GameplayMods/_MeleeSystem/__InventoryMenu/Menu_InventoryMelee.UI_InvMelee_Upgrade_Tier2` _as_menu_inventory_melee) (`/Game/_DRGModding/GameplayMods/_MeleeSystem/__InventoryMenu/Menu_InventoryMelee.UI_InvMelee_Upgrade_Tier3` _as_menu_inventory_melee))
    (bind (_isvalid _selectedupgrade) (`/Game/_DRGModding/GameplayMods/_MeleeSystem/__InventoryMenu/UI_InvMelee_Upgrade.GetSelectedUpgrade` _array_element))
    (if _isvalid
      (`KismetArrayLibrary.Array_Add` (`local.NewLocalVar_0`) _selectedupgrade)))
  (return (`local.NewLocalVar_0`)))

(fn `NewFunction_0`
  (params (CurrentCharacterID :type "PlayerCharacterID Object Reference") (`Inventory Info` :type "/Game/_DRGModding/GameplayMods/_MeleeSystem/__InventoryMenu/InventoryInfoMelee Object Reference"))
  (locals (Local_EquippedUpgrade :type "Map of /Game/_DRGModding/GameplayMods/_MeleeSystem/__InventoryMenu/InventoryInfoMelee Object Reference to /Game/_DRGModding/GameplayMods/_MeleeSystem/_HandleWeaponEquip/S_MeleeEquippedUpgrade Structure") (NewLocalVar_1 :type "Array of /Game/_DRGModding/GameplayMods/_MeleeSystem/__InventoryMenu/Upgrade/MeleeUpgrade Object Reference") (NewLocalVar_2 :type "Map of PlayerCharacterID Object Reference to /Game/_DRGModding/GameplayMods/_MeleeSystem/_HandleWeaponEquip/S_MeleeUpgrade Structure"))
  (bind _currentcharacterid (`local.CurrentCharacterID`))
  (set `local.NewLocalVar_1` (`self.GetEquippedUpgrades`))
  (set `local.NewLocalVar_2` (`/Game/_DRGModding/GameplayMods/_MeleeSystem/_HandleWeaponEquip/MeleeSaveGame.Equipped` (`self.As Melee Save Game`)))
  (bind _output_get (set `local.Local_EquippedUpgrade` (break `/Game/_DRGModding/GameplayMods/_MeleeSystem/_HandleWeaponEquip/S_MeleeUpgrade` (`BlueprintMapLibrary.Map_Find` (`local.NewLocalVar_2`) _currentcharacterid))))
  (`BlueprintMapLibrary.Map_Add` _output_get (`self.Inventory Info`) (make `/Game/_DRGModding/GameplayMods/_MeleeSystem/_HandleWeaponEquip/S_MeleeEquippedUpgrade` (`local.NewLocalVar_1`)))
  (`BlueprintMapLibrary.Map_Add` (`local.NewLocalVar_2`) _currentcharacterid (make `/Game/_DRGModding/GameplayMods/_MeleeSystem/_HandleWeaponEquip/S_MeleeUpgrade` (`local.Local_EquippedUpgrade`)))
  (set `/Game/_DRGModding/GameplayMods/_MeleeSystem/_HandleWeaponEquip/MeleeSaveGame.Equipped` (`local.NewLocalVar_2`) (`self.As Melee Save Game`))
  (for _array_element (`local.NewLocalVar_1`)
    (`KismetSystemLibrary.PrintString` (`KismetStringLibrary.Concat_StrStr` "Saved Upgrade - " (`KismetSystemLibrary.GetDisplayName` _array_element))))
  (`KismetSystemLibrary.PrintString` (`KismetStringLibrary.Concat_StrStr` "Saved Character - " (`KismetSystemLibrary.GetDisplayName` (`self.CurrentCharacterID`)))))

(fn `OnCharacterChanged`
  (params (Key :type "PlayerCharacterID Object Reference (by ref)"))
  (set `self.CurrentCharacterID` Key)
  (bind _inventoryinfomelee (`/Game/_DRGModding/GameplayMods/_MeleeSystem/_HandleWeaponEquip/MeleeSaveGame.GetMeleeInfoByID` (`self.As Melee Save Game`) Key))
  (`KismetSystemLibrary.PrintString` (`KismetStringLibrary.Concat_StrStr` "OnCharacterChanged Func -> Inventory Info - " (`KismetSystemLibrary.GetDisplayName` _inventoryinfomelee)) true true (struct :`G` 0.66 :`B` 1.0 :`A` 1.0) 10.0)
  (`/Game/_DRGModding/GameplayMods/_MeleeSystem/__InventoryMenu/Menu_InventoryMelee.OnItemSelected` (`self.As Menu Inventory Melee`) _inventoryinfomelee)
  (`self.OnItemSelected` _inventoryinfomelee)
  (set `self.Index` (`KismetArrayLibrary.Array_Find` (`self.MeleeWeapons`) _inventoryinfomelee))
  (`/Game/_DRGModding/GameplayMods/_MeleeSystem/__InventoryMenu/Menu_InventoryMelee.SetClassName` (`self.As Menu Inventory Melee`) (`KismetTextLibrary.Conv_StringToText` (`PlayerCharacterID.AnalyticsID` Key))))

(fn `SaveCurrenbt`
  (if (and (`KismetSystemLibrary.IsValid` (`self.CurrentCharacterID`)) (`KismetSystemLibrary.IsValid` (`self.Inventory Info`)))
    (`BlueprintMapLibrary.Map_Add` (`/Game/_DRGModding/GameplayMods/_MeleeSystem/_HandleWeaponEquip/MeleeSaveGame.EquippedItem` (`self.As Melee Save Game`)) (`self.CurrentCharacterID`) (`self.Inventory Info`))
    (`self.NewFunction_0` (`self.CurrentCharacterID`) (`self.Inventory Info`))
    (`/Game/_DRGModding/_Frameworks/BML_Framework.SaveToSlot(Macro)` (`self.As Melee Save Game`) true "MeleeSettingsSaveGame")
    (`KismetSystemLibrary.PrintString` (`KismetStringLibrary.Concat_StrStr` "Saved -" (`KismetSystemLibrary.GetDisplayName` (`self.CurrentCharacterID`)) " - " (`KismetSystemLibrary.GetDisplayName` (`self.Inventory Info`))))
    (else
      (`KismetSystemLibrary.PrintString` "SAVE FAILED" true true (struct :`R` 1.0 :`G` 0.029525 :`A` 1.0) 5.0))))

(fn `UpdateMeshAnimations`
  (params (self2 :type "/Game/_DRGModding/GameplayMods/_MeleeSystem/__InventoryMenu/InventoryInfoMelee Object Reference"))
  (for _array_element (`self.As ABP Inventory Melee`)
    (set `/Game/_DRGModding/GameplayMods/_MeleeSystem/__InventoryMenu/ABP_InventoryMelee.Sequence` (`/Game/_DRGModding/GameplayMods/_MeleeSystem/__InventoryMenu/InventoryInfoMelee.IdleAnimation` self2) _array_element)))

(fn `UserConstructionScript`)