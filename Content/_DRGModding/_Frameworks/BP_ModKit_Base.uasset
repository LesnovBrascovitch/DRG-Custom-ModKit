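; Base actor for mods built on LB's ModKit framework in Deep Rock Galactic, providing shared setup state and debug logging.
; OnModKitObtained stores the ModKit reference, and OnSpawned records whether the actor is in the Space Rig.
; PrintDebugMessage forwards to the ModKit when that reference is valid, prefixing the sender with the bracketed mod actor name.
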(event `OnModKitObtained`
  (params (LBsModKit :type "/Game/_DRGModding/_Frameworks/FW_LBsModKit_Manager Object Reference"))
  (set `self.LBs Mod Kit` LBsModKit))

(event `OnSpawned`
  (params (IsInSpacerig :type Boolean))
  (set `self.Is in Spacerig` IsInSpacerig))

(fn `PrintDebugMessage`
  (params (`FORCE PRINT` :type Boolean) (Sender :type String) (Text :type String) (SenderType :type "EChatSenderType Enum" :default "NormalUser"))
  (`/Engine/EditorBlueprintResources/StandardMacros.IsValid` (`self.LBs Mod Kit`)
    (:`Is Valid`
      (`/Game/_DRGModding/_Frameworks/FW_LBsModKit_Manager.PrintDebugMessage` (`self.LBs Mod Kit`) `FORCE PRINT` (`KismetStringLibrary.Concat_StrStr` (`KismetStringLibrary.Concat_StrStr` "[" (`self.ModActorName`) "]") Sender) Text SenderType))))

(fn `UserConstructionScript`)