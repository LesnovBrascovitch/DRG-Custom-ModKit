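; Base actor in the DRG modding framework that holds a mod's identity and its hub menu pages.
; StartHubMenu stores the mod's author, name and version, then creates a widget from each supplied class and adds it uniquely to HubPages.
; GetModInfo and GetModPages expose the stored info and created widgets; nothing here displays them.
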(event `StartHubMenu`
  (params (HubMenu :type "Array of /Game/_DRGModding/_Frameworks/Menu_HubMenu_Base Class Reference") (`Mod Author` :type Text) (`Mod Name` :type Text) (`Mod Version` :type Text))
  (`self.SetModInfo` `Mod Author` `Mod Name` `Mod Version`)
  (for _array_element HubMenu
    (bind _returnvalue (`|CreateWidget` _array_element))
    (`KismetArrayLibrary.Array_AddUnique` (`self.Hub Pages`) _returnvalue)))

(fn `GetModInfo`
  (returns (ModName :type Text) (ModAuthor :type Text) (ModVersion :type Text))
  (return (`self.Mod Name`) (`self.Mod Author`) (`self.Mod Version`)))

(fn `GetModPages`
  (returns (HubPages :type "Array of /Game/_ModHub/IHubPageWidget Interface"))
  (return (`self.Hub Pages`)))

(fn `SetModInfo`
  (params (`Mod Author` :type Text) (`Mod Name` :type Text) (`Mod Version` :type Text))
  (set `self.Mod Author` `Mod Author`)
  (set `self.Mod Name` `Mod Name`)
  (set `self.Mod Version` `Mod Version`))

(fn `UserConstructionScript`)