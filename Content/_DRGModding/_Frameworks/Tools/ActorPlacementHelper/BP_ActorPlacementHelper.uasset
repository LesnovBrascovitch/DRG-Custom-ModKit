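; In-game mod developer tool for spawning and positioning actors live, toggled by a console command through the mod kit.
; Its menu lists classes gathered from BPI_ActorPlacementHelper implementers and spawns the selection as a collisionless preview following the player's line trace until locked.
; Held axis keys plus mouse movement move, rotate or scale the preview, with adjustable sensitivity, arrow feedback and interface forwarding.
; Hotkeys stamp copies, remove them or send the transform to the menu.
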(event `CustomEvent_1`
  (`self.EnableInput` (`self.FSDPlayer Controller`)))

(event `self.OnModKitObtained`
  (params (LBsModKit :type "/Game/_DRGModding/_Frameworks/FW_LBsModKit_Manager Object Reference"))
  (add `/Game/_DRGModding/_Frameworks/FW_LBsModKit_Manager.OnConsoleCommandReceieved` LBsModKit (delegate `OnConsoleCommandReceieved_Event_0`)))

(event `self.ReceiveBeginPlay`
  (bind _fsdplayercontroller (`/Game/_DRGModding/_Frameworks/BML_Framework.GetLocalPlayerController(Macro)` true)
    (:`Completed`
      (set `self.FSDPlayer Controller` _fsdplayercontroller)
      (bind _playercharacter (`/Game/_DRGModding/_Frameworks/BML_Framework.GetLocalPlayerCharacter(Macro)` true)
        (:`Exec`
          (set `self.Player Character` _playercharacter))))))

(event `OnConsoleCommandReceieved_Event_0`
  (params (ConsoleCommands :type "Array of String (by ref)"))
  (switch `string` (`|GetArrayItem` ConsoleCommands)
    (:`A1`
      (`self.TogglePlacementHelper`))))

(event `Key|F`
  (params (Key :type "Key Structure"))
  (:`Pressed`
    (`KismetSystemLibrary.PrintString` "ActorPlacement")))

(event `TogglePlacementHelper`
  (bind _as_menu_actor_placement_helper (`self.As Menu Actor Placement Helper`))
  (bind _returnvalue (`Widget.IsVisible` _as_menu_actor_placement_helper))
  ;[1 1 1] Toggle HUD
  (`/Engine/EditorBlueprintResources/StandardMacros.IsValid` (`self.As Menu Actor Placement Helper`)
    (:`Is Valid`
      (if _returnvalue
        (`self.NewFunction_0_0`)
        (`self.DisableInput` (`self.FSDPlayer Controller`))
        (`/Game/_DRGModding/_Frameworks/BML_Framework.ToggleMainHudVisibillity(Spacerig)` "SelfHitTestInvisible"
          (:`Completed`
            _))
        (else
          (`self.EnableInput` (`self.FSDPlayer Controller`))
          (`/Game/_DRGModding/_Frameworks/BML_Framework.ToggleMainHudVisibillity(Spacerig)` "Collapsed"
            (:`Completed`
              _))))
      (`Widget.SetVisibility` _as_menu_actor_placement_helper (select `bool` _returnvalue :`false` "SelfHitTestInvisible" :`true` "Collapsed" :!type "ESlateVisibility Enum")))
    (:`Is Not Valid`
      (bind _outputpin (`/Game/_DRGModding/_Frameworks/BML_Framework.WaitUntil(CreateWidge)` "/Game/_DRGModding/_Frameworks/Tools/ActorPlacementHelper/Menu_ActorPlacementHelper.Menu_ActorPlacementHelper_C" (`self.FSDPlayer Controller`))
        (:`true`
          (bind _asmenu_actor_placement_helper (cast `/Game/_DRGModding/_Frameworks/Tools/ActorPlacementHelper/Menu_ActorPlacementHelper` _outputpin))
          (bind _output_get (set `self.As Menu Actor Placement Helper` _asmenu_actor_placement_helper))
          (add `/Game/_DRGModding/_Frameworks/Tools/ActorPlacementHelper/Menu_ActorPlacementHelper.OnActorClassSelected` _output_get (`|CreateDelegate` :!event `OnPlacementClassSelected`))
          (`self.InitializeWidget`)
          (`self.NewFunction_0_0`)
          (`/Game/_DRGModding/_Frameworks/BML_Framework.ToggleMainHudVisibillity(Spacerig)` "Collapsed"))))))

(event `Key|G`
  (params (Key :type "Key Structure"))
  (:`Pressed`
    (set `self.NewVar_0` (not (`self.NewVar_0`)))
    (if (`self.NewVar_0`)
      (set `self.NewVar_1` (`self.K2_GetActorLocation` (`self.InstancedActor`))))))

(event `self.ReceiveTick`
  (params (DeltaSeconds :type "Float (single-precision)"))
  (`self.IsInstanced`
    (:`Is Valid`
      (if (not (`self.NewVar_0`))
        (bind _location (`/Game/_DRGModding/_Frameworks/BML_Framework.QuickLinetrace` (`self.Player Character`))
          (:`OnHit`
            (`self.K2_SetActorLocation` (`self.InstancedActor`) _location false false))))
      (`self.K2_SetActorLocation` (`self.InstancedActor`) (select `bool` (`self.NewVar_0`) :`false` (+ (`self.LocationOffset`) (`self.K2_GetActorLocation` (`self.InstancedActor`))) :`true` (+ (`self.LocationOffset`) (`self.NewVar_1`))) false false)
      (`self.SetActorScale3D` (`self.InstancedActor`) (`self.ScaleOffset`)))))

(event `Key|LeftControl`
  (params (Key :type "Key Structure"))
  (bind _instancedactor (`self.InstancedActor`))
  (:`Pressed`
    (`self.IsInstanced`
      (:`Is Valid`
        (bind _returnvalue (`|SpawnActorFromClass` (`GameplayStatics.GetObjectClass` _instancedactor) (`self.GetTransform` _instancedactor) "AlwaysSpawn" "OverrideRootScale" null null))
        (`KismetArrayLibrary.Array_Add` (`self.InstancedActors`) _returnvalue)))))

(event `Key|BackSpace`
  (params (Key :type "Key Structure"))
  (bind _instancedactors (`self.InstancedActors`))
  (bind _returnvalue (`KismetArrayLibrary.Array_LastIndex` _instancedactors))
  (bind _output (`|GetArrayItem` _instancedactors _returnvalue))
  (:`Pressed`
    (`/Engine/EditorBlueprintResources/StandardMacros.IsValid` _output
      (:`Is Valid`
        (`self.K2_DestroyActor` _output)
        (`KismetArrayLibrary.Array_Remove` (`self.InstancedActors`) _returnvalue)))))

(event `OnPlacementClassSelected`
  (params (ActorClass :type "Actor Class Reference"))
  (bind _instancedactor (`self.InstancedActor`))
  (`/Engine/EditorBlueprintResources/StandardMacros.IsValid` _instancedactor
    (:`Is Valid`
      (`self.K2_DestroyActor` _instancedactor))
    (:`Is Not Valid`
      _))
  (bind _returnvalue (`|SpawnActorFromClass` ActorClass (`KismetMathLibrary.MakeTransform` (0.0 0.0 0.0)) "AlwaysSpawn" "OverrideRootScale" null null))
  (bind _output_get (set `self.InstancedActor` _returnvalue))
  (`self.SetActorEnableCollision` _output_get false))

(event `InputAxisKey|MouseX` :consume false
  (params (AxisValue :type "Float (single-precision)"))
  (bind _returnvalue (`self.ConvByOffset` AxisValue))
  (`self.IsInstanced` :!label _label
    (:`Is Valid`
      (if (`self.IsV`)
        (`self.NewFunction_1` AxisValue)
        (elif (`self.IsB`)
          (message `/Game/_DRGModding/_Frameworks/Tools/ActorPlacementHelper/BPI_ActorPlacementHelper.ObtainMouseValue(Interface)` (`self.InstancedActor`) (`/Game/_DRGModding/_Frameworks/Tools/ActorPlacementHelper/Menu_ActorPlacementHelper.GetInterfaceString` (`self.As Menu Actor Placement Helper`)) _returnvalue)
          (else
            (`self.IsAnyKeyPressed`
              (:`true`
                (`self.UpdateTransform` _returnvalue (`self.ConvByOffset` (stale `InputAxisKey|MouseY` AxisValue)))))))))))

(event `Key|Enter` :consume false
  (params (Key :type "Key Structure"))
  (:`Pressed`
    (`self.IsInstanced`
      (:`Is Valid`
        (`/Game/_DRGModding/_Frameworks/Tools/ActorPlacementHelper/Menu_ActorPlacementHelper.UpdateTransofrm` (`self.As Menu Actor Placement Helper`) (`self.GetTransform` (`self.InstancedActor`)))))))

(event `Key|Tab`
  (params (Key :type "Key Structure"))
  (:`Pressed`
    (`/Engine/EditorBlueprintResources/StandardMacros.IsValid` (`self.As Menu Actor Placement Helper`)
      (:`Is Valid`
        (if (`PlayerController.bShowMouseCursor` (`self.FSDPlayer Controller`))
          (set `PlayerController.bShowMouseCursor` false (`self.FSDPlayer Controller`))
          (`WidgetBlueprintLibrary.SetFocusToGameViewport`)
          (`Controller.SetIgnoreLookInput` (`self.FSDPlayer Controller`) false)
          (else
            (set `PlayerController.bShowMouseCursor` true (`self.FSDPlayer Controller`))
            (`Widget.SetFocus` (`self.As Menu Actor Placement Helper`))
            (`Controller.SetIgnoreLookInput` (`self.FSDPlayer Controller`) true)))))))

(event `InputAxisKey|MouseY` :consume false
  (params (AxisValue :type "Float (single-precision)"))
  (goto _label))

(event `Key|Z`
  (params (Key :type "Key Structure"))
  (:`Pressed`
    (set `self.IsZ` true)
    (`Controller.SetIgnoreLookInput` (`self.FSDPlayer Controller`) true :!label _label_2)
    (`self.NewFunction_2`))
  (:`Released`
    (set `self.IsZ` false)
    (`Controller.SetIgnoreLookInput` (`self.FSDPlayer Controller`) false :!label _label_3)
    (`self.NewFunction_2`)))

(event `Key|X`
  (params (Key :type "Key Structure"))
  (:`Pressed`
    (set `self.IsX` true)
    (goto _label_2))
  (:`Released`
    (set `self.IsX` false)
    (goto _label_3)))

(event `Key|P`
  (params (Key :type "Key Structure"))
  (:`Pressed`
    (`self.IsInstanced`
      (:`Is Valid`
        (bind _outactors (`GameplayStatics.GetAllActorsOfClass` (`GameplayStatics.GetObjectClass` (`self.InstancedActor`))))
        (for _array_element _outactors
          (if (!= _array_element (`self.InstancedActor`))
            (`self.K2_DestroyActor` _array_element)))))))

(event `Key|C`
  (params (Key :type "Key Structure"))
  (:`Pressed`
    (set `self.IsY` true)
    (goto _label_2))
  (:`Released`
    (set `self.IsY` false)
    (goto _label_3)))

(event `Key|V`
  (params (Key :type "Key Structure"))
  (:`Pressed`
    (set `self.IsV` true)
    (goto _label_2))
  (:`Released`
    (set `self.IsV` false)
    (goto _label_3)))

(event `Key|E`
  (params (Key :type "Key Structure"))
  (:`Pressed`
    (set `self.TransformMode` "NewEnumerator0")
    (`/Game/_DRGModding/_Frameworks/Tools/ActorPlacementHelper/Menu_ActorPlacementHelper.UpdateTransformMode` (`self.As Menu Actor Placement Helper`) (`self.TransformMode`) :!label _label_4)))

(event `Key|B`
  (params (Key :type "Key Structure"))
  (:`Pressed`
    (set `self.IsB` true)
    (goto _label_2))
  (:`Released`
    (set `self.IsB` false)
    (goto _label_3)))

(event `Key|R`
  (params (Key :type "Key Structure"))
  (:`Pressed`
    (set `self.TransformMode` "NewEnumerator1")
    (goto _label_4)))

(event `Key|T`
  (params (Key :type "Key Structure"))
  (:`Pressed`
    (set `self.TransformMode` "NewEnumerator2")
    (goto _label_4)))

(fn `ConvByOffset`
  (params (Base :type "Float (double-precision)"))
  (returns (ReturnValue :type "Float (double-precision)"))
  (return (* Base (`self.Offset`))))

(fn `InitializeWidget`
  (`/Game/_DRGModding/_Frameworks/Tools/ActorPlacementHelper/Menu_ActorPlacementHelper.UpdateValueOffset` (`self.As Menu Actor Placement Helper`) (`self.Offset`))
  (`/Game/_DRGModding/_Frameworks/Tools/ActorPlacementHelper/Menu_ActorPlacementHelper.UpdateTransformMode` (`self.As Menu Actor Placement Helper`) (`self.TransformMode`)))

(fn `NewFunction_0_0`
  (locals (Local_Cache :type "Array of Actor Class Reference"))
  (bind _outactors (`GameplayStatics.GetAllActorsWithInterface` "/Game/_DRGModding/_Frameworks/Tools/ActorPlacementHelper/BPI_ActorPlacementHelper.BPI_ActorPlacementHelper_C"))
  (for _array_element _outactors
    (bind _classes (message `/Game/_DRGModding/_Frameworks/Tools/ActorPlacementHelper/BPI_ActorPlacementHelper.GetPlacementClasses` _array_element))
    (for _array_element_2 _classes
      (`KismetArrayLibrary.Array_AddUnique` (`local.Local_Cache`) _array_element_2)))
  (`/Game/_DRGModding/_Frameworks/Tools/ActorPlacementHelper/Menu_ActorPlacementHelper.AddClassesToSelection` (`self.As Menu Actor Placement Helper`) (`local.Local_Cache`)))

(fn `NewFunction_1`
  (params (A :type "Float (double-precision)"))
  (bind _offset (`self.Offset`))
  (`|VariableSetRef` _offset (`KismetMathLibrary.FClamp` (+ _offset (* A 0.01)) 0.001 5.0))
  (`/Game/_DRGModding/_Frameworks/Tools/ActorPlacementHelper/Menu_ActorPlacementHelper.UpdateValueOffset` (`self.As Menu Actor Placement Helper`) (`self.Offset`)))

(fn `NewFunction_2`
  (bind _rootcomponent (`Actor.RootComponent` (`self.InstancedActor`)))
  (if (`self.IsZ`)
    (`SceneComponent.K2_AttachToComponent` (`self.Arrow`) _rootcomponent "None" "SnapToTarget" "KeepWorld" "KeepRelative" true)
    (`SceneComponent.K2_SetWorldRotation` (`self.Arrow`) (`KismetMathLibrary.Conv_VectorToRotator` (`SceneComponent.GetForwardVector` _rootcomponent)) false false)
    (`ArrowComponent.SetArrowColor` (`self.Arrow`) (struct :`R` 1.0 :`A` 1.0))
    (`SceneComponent.SetHiddenInGame` (`self.Arrow`) false false :!label _label)
    (elif (`self.IsX`)
      (`SceneComponent.K2_AttachToComponent` (`self.Arrow`) (`Actor.RootComponent` (`self.InstancedActor`)) "None" "SnapToTarget" "KeepWorld" "KeepRelative" true)
      (`SceneComponent.K2_SetWorldRotation` (`self.Arrow`) (`KismetMathLibrary.Conv_VectorToRotator` (`SceneComponent.GetRightVector` (`Actor.RootComponent` (`self.InstancedActor`)))) false false)
      (`ArrowComponent.SetArrowColor` (`self.Arrow`) (struct :`G` 1.0 :`A` 1.0))
      (goto _label)
      (elif (`self.IsY`)
        (`SceneComponent.K2_AttachToComponent` (`self.Arrow`) (`Actor.RootComponent` (`self.InstancedActor`)) "None" "SnapToTarget" "KeepWorld" "KeepRelative" true)
        (`SceneComponent.K2_SetWorldRotation` (`self.Arrow`) (`KismetMathLibrary.Conv_VectorToRotator` (`SceneComponent.GetUpVector` (`Actor.RootComponent` (`self.InstancedActor`)))) false false)
        (`ArrowComponent.SetArrowColor` (`self.Arrow`) (struct :`B` 1.0 :`A` 1.0))
        (goto _label)
        (else
          (`SceneComponent.SetHiddenInGame` (`self.Arrow`) true false))))))

(fn `UpdateTransform`
  (params (XValue :type "Float (double-precision)") (YValue :type "Float (double-precision)"))
  (bind _locationoffset (`self.LocationOffset`))
  (switch `/Game/_DRGModding/_Frameworks/Tools/ActorPlacementHelper/E_TransformMode` (`self.TransformMode`)
    (:`NewEnumerator0`
      (set `self.LocationOffset` (`KismetMathLibrary.SelectVector` (+ _locationoffset (`KismetMathLibrary.MakeVector` 0.0 (`local.XValue`))) (`KismetMathLibrary.SelectVector` (+ _locationoffset (`KismetMathLibrary.MakeVector` (`local.YValue`))) (+ _locationoffset (`KismetMathLibrary.MakeVector` 0.0 0.0 (`local.YValue`))) (`self.IsZ`)) (`self.IsX`))))
    (:`NewEnumerator1`
      (`self.K2_AddActorLocalRotation` (`self.InstancedActor`) (`KismetMathLibrary.MakeRotator` (`KismetMathLibrary.SelectFloat` (`local.XValue`) 0.0 (`self.IsZ`)) (`KismetMathLibrary.SelectFloat` (`local.XValue`) 0.0 (`self.IsX`)) (`KismetMathLibrary.SelectFloat` (`local.XValue`) 0.0 (`self.IsY`))) false false))
    (:`NewEnumerator2`
      (if (`self.IsZ`)
        (set `self.ScaleOffset` (`KismetMathLibrary.ClampVectorSize` (+ (`self.ScaleOffset`) (`local.XValue`)) 0.01 999.0))))))

(fn `UserConstructionScript`)