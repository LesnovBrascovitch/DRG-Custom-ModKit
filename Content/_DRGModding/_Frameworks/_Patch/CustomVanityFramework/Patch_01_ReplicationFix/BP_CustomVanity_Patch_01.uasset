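; Custom Vanity Framework replication-fix patch that reapplies the local player's saved vanity per class and loadout slot.
; On spawn it loads a custom savegame, then waits for valid character vanity and permanently applies each saved item, repeating on possession.
; In the space rig it polls for Wardrobe widgets and binds their close event.
; A delayed window handler copies equipped vanity into the matching savegame slot, with no explicit disk save here.
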(event `CustomEvent_0`
  (params (Window :type "WindowWidget Object Reference"))
  (bind _as_custom_vanity_testing_savegame (`self.As Custom Vanity Testing Savegame`))
  (bind _as_custom_vanity_testing_savegame_2 (`self.As Custom Vanity Testing Savegame`))
  (bind _as_custom_vanity_testing_savegame_3 (`self.As Custom Vanity Testing Savegame`))
  (bind _as_custom_vanity_testing_savegame_4 (`self.As Custom Vanity Testing Savegame`))
  (bind _equipped_vanity (`self.Equipped Vanity`))
  (bind _equipped_vanity_2 (`self.Equipped Vanity`))
  (bind _equipped_vanity_3 (`self.Equipped Vanity`))
  (bind _equipped_vanity_4 (`self.Equipped Vanity`))
  (bind _returnvalue (`ActorFunctionLibrary.GetCharacterIDFromCharacter` (`self.Player Character`)))
  (`KismetSystemLibrary.Delay` 1.0)
  (set `self.Equipped Vanity` (`CharacterVanityComponent.EquippedVanity` (`PlayerCharacter.GetCharacterVanity` (`self.Player Character`))))
  (set `self.LoadoutIndex` (`FSDSaveGame.GetSelectedLoadoutIndex` (`FSDGameInstance.SaveGame` (`GameFunctionLibrary.GetFSDGameInstance` self)) _returnvalue))
  (`/Game/_DRGModding/_Frameworks/BML_Framework.SwitchByPlayerCharacterID` _returnvalue
    (:`DrillerID`
      (switch `int` (`self.LoadoutIndex`)
        (:`0`
          (set `/Game/_DRGModding/_Frameworks/_Patch/CustomVanityFramework/Patch_01_ReplicationFix/CustomVanityTestingSavegame.DrillerID_0` _equipped_vanity_3 _as_custom_vanity_testing_savegame_2))
        (:`1`
          (set `/Game/_DRGModding/_Frameworks/_Patch/CustomVanityFramework/Patch_01_ReplicationFix/CustomVanityTestingSavegame.DrillerID_1` _equipped_vanity_3 _as_custom_vanity_testing_savegame_2))
        (:`2`
          (set `/Game/_DRGModding/_Frameworks/_Patch/CustomVanityFramework/Patch_01_ReplicationFix/CustomVanityTestingSavegame.DrillerID_2` _equipped_vanity_3 _as_custom_vanity_testing_savegame_2))
        (:`3`
          (set `/Game/_DRGModding/_Frameworks/_Patch/CustomVanityFramework/Patch_01_ReplicationFix/CustomVanityTestingSavegame.DrillerID_3` _equipped_vanity_3 _as_custom_vanity_testing_savegame_2))
        (:`4`
          (set `/Game/_DRGModding/_Frameworks/_Patch/CustomVanityFramework/Patch_01_ReplicationFix/CustomVanityTestingSavegame.DrillerID_4` _equipped_vanity_3 _as_custom_vanity_testing_savegame_2))
        (:`5`
          (set `/Game/_DRGModding/_Frameworks/_Patch/CustomVanityFramework/Patch_01_ReplicationFix/CustomVanityTestingSavegame.DrillerID_5` _equipped_vanity_3 _as_custom_vanity_testing_savegame_2))))
    (:`EngineerID`
      (switch `int` (`self.LoadoutIndex`)
        (:`0`
          (set `/Game/_DRGModding/_Frameworks/_Patch/CustomVanityFramework/Patch_01_ReplicationFix/CustomVanityTestingSavegame.EngineerID_0` _equipped_vanity_2 _as_custom_vanity_testing_savegame_3))
        (:`1`
          (set `/Game/_DRGModding/_Frameworks/_Patch/CustomVanityFramework/Patch_01_ReplicationFix/CustomVanityTestingSavegame.EngineerID_1` _equipped_vanity_2 _as_custom_vanity_testing_savegame_3))
        (:`2`
          (set `/Game/_DRGModding/_Frameworks/_Patch/CustomVanityFramework/Patch_01_ReplicationFix/CustomVanityTestingSavegame.EngineerID_2` _equipped_vanity_2 _as_custom_vanity_testing_savegame_3))
        (:`3`
          (set `/Game/_DRGModding/_Frameworks/_Patch/CustomVanityFramework/Patch_01_ReplicationFix/CustomVanityTestingSavegame.EngineerID_3` _equipped_vanity_2 _as_custom_vanity_testing_savegame_3))
        (:`4`
          (set `/Game/_DRGModding/_Frameworks/_Patch/CustomVanityFramework/Patch_01_ReplicationFix/CustomVanityTestingSavegame.EngineerID_4` _equipped_vanity_2 _as_custom_vanity_testing_savegame_3))
        (:`5`
          (set `/Game/_DRGModding/_Frameworks/_Patch/CustomVanityFramework/Patch_01_ReplicationFix/CustomVanityTestingSavegame.EngineerID_5` _equipped_vanity_2 _as_custom_vanity_testing_savegame_3))))
    (:`GunnerID`
      (switch `int` (`self.LoadoutIndex`)
        (:`0`
          (set `/Game/_DRGModding/_Frameworks/_Patch/CustomVanityFramework/Patch_01_ReplicationFix/CustomVanityTestingSavegame.GunnerID_0` _equipped_vanity_4 _as_custom_vanity_testing_savegame_4))
        (:`1`
          (set `/Game/_DRGModding/_Frameworks/_Patch/CustomVanityFramework/Patch_01_ReplicationFix/CustomVanityTestingSavegame.GunnerID_1` _equipped_vanity_4 _as_custom_vanity_testing_savegame_4))
        (:`2`
          (set `/Game/_DRGModding/_Frameworks/_Patch/CustomVanityFramework/Patch_01_ReplicationFix/CustomVanityTestingSavegame.GunnerID_2` _equipped_vanity_4 _as_custom_vanity_testing_savegame_4))
        (:`3`
          (set `/Game/_DRGModding/_Frameworks/_Patch/CustomVanityFramework/Patch_01_ReplicationFix/CustomVanityTestingSavegame.GunnerID_3` _equipped_vanity_4 _as_custom_vanity_testing_savegame_4))
        (:`4`
          (set `/Game/_DRGModding/_Frameworks/_Patch/CustomVanityFramework/Patch_01_ReplicationFix/CustomVanityTestingSavegame.GunnerID_4` _equipped_vanity_4 _as_custom_vanity_testing_savegame_4))
        (:`5`
          (set `/Game/_DRGModding/_Frameworks/_Patch/CustomVanityFramework/Patch_01_ReplicationFix/CustomVanityTestingSavegame.GunnerID_5` _equipped_vanity_4 _as_custom_vanity_testing_savegame_4))))
    (:`ScoutID`
      (switch `int` (`self.LoadoutIndex`)
        (:`0`
          (set `/Game/_DRGModding/_Frameworks/_Patch/CustomVanityFramework/Patch_01_ReplicationFix/CustomVanityTestingSavegame.ScoutID_0` _equipped_vanity _as_custom_vanity_testing_savegame))
        (:`1`
          (set `/Game/_DRGModding/_Frameworks/_Patch/CustomVanityFramework/Patch_01_ReplicationFix/CustomVanityTestingSavegame.ScoutID_1` _equipped_vanity _as_custom_vanity_testing_savegame))
        (:`2`
          (set `/Game/_DRGModding/_Frameworks/_Patch/CustomVanityFramework/Patch_01_ReplicationFix/CustomVanityTestingSavegame.ScoutID_2` _equipped_vanity _as_custom_vanity_testing_savegame))
        (:`3`
          (set `/Game/_DRGModding/_Frameworks/_Patch/CustomVanityFramework/Patch_01_ReplicationFix/CustomVanityTestingSavegame.ScoutID_3` _equipped_vanity _as_custom_vanity_testing_savegame))
        (:`4`
          (set `/Game/_DRGModding/_Frameworks/_Patch/CustomVanityFramework/Patch_01_ReplicationFix/CustomVanityTestingSavegame.ScoutID_4` _equipped_vanity _as_custom_vanity_testing_savegame))
        (:`5`
          (set `/Game/_DRGModding/_Frameworks/_Patch/CustomVanityFramework/Patch_01_ReplicationFix/CustomVanityTestingSavegame.ScoutID_5` _equipped_vanity _as_custom_vanity_testing_savegame))))))

(event `self.OnSpawned`
  (params (IsInSpacerig :type Boolean))
  (`parent.OnSpawned` IsInSpacerig)
  (`KismetSystemLibrary.Delay` 1.0)
  (bind _outputpin (`/Game/_DRGModding/_Frameworks/BML_Framework.HandleSaveGame` "/Game/_DRGModding/_Frameworks/_Patch/CustomVanityFramework/Patch_01_ReplicationFix/CustomVanityTestingSavegame.CustomVanityTestingSavegame_C")
    (:`then`
      (bind _ascustom_vanity_testing_savegame (cast `/Game/_DRGModding/_Frameworks/_Patch/CustomVanityFramework/Patch_01_ReplicationFix/CustomVanityTestingSavegame` _outputpin))
      (set `self.As Custom Vanity Testing Savegame` _ascustom_vanity_testing_savegame)
      (bind _fsdplayercontroller (`/Game/_DRGModding/_Frameworks/BML_Framework.GetLocalPlayerController(Macro)` true)
        (:`Completed`
          (add `FSDPlayerController.OnPlayerCharacterPossesed` _fsdplayercontroller (delegate `OnPlayerCharacterPossesed_Event_0`))
          (bind _playercharacter (`/Game/_DRGModding/_Frameworks/BML_Framework.GetLocalPlayerCharacter(Macro)` true :!label _label)
            (:`Exec`
              (set `self.Player Character` _playercharacter)
              (`/Engine/EditorBlueprintResources/StandardMacros.IsValid` (`PlayerCharacter.GetCharacterVanity` _playercharacter) :!label _label_2
                (:`Is Valid`
                  (bind _savedvanity (`self.GetSavedVanity`))
                  (for _array_element (`.Vanity` (break `EquippedVanity` _savedvanity))
                    (`self.ApplyItem` _array_element))
                  (if (`self.Is in Spacerig`)
                    (bind _foundwidgets (`WidgetBlueprintLibrary.GetAllWidgetsOfClass` "/Game/UI/Menu_Wardrobe/_MENU_Wardrobe._MENU_Wardrobe_C" false :!label _label_3))
                    (`/Engine/EditorBlueprintResources/StandardMacros.IsValid` (`|GetArrayItem` _foundwidgets)
                      (:`Is Valid`
                        (for _array_element_2 _foundwidgets
                          (add `WindowWidget.OnWindowClosed` _array_element_2 (`|CreateDelegate` :!event `CustomEvent_0`))
                          (`self.PrintDebugMessage` false "" "Obtained _Menu_Wardrobe Succesfully")))
                      (:`Is Not Valid`
                        (`KismetSystemLibrary.Delay` 1.0)
                        (`self.PrintDebugMessage` false "" "Trying Obtain _Menu_Wardrobe")
                        (goto _label_3)))
                    (else
                      (`self.PrintDebugMessage` false "" "Applied Item Skin(Cave)"))))
                (:`Is Not Valid`
                  (`KismetSystemLibrary.Delay` 0.2)
                  (goto _label_2))))))))))

(event `OnPlayerCharacterPossesed_Event_0`
  (params (Pawn :type "Pawn Object Reference"))
  (goto _label))

(fn `ApplyItem`
  (params (InputPin :type "VanityItem Object Reference"))
  (bind _player_character (`self.Player Character`))
  (`VanityItem.ChangeToItem` InputPin (`PlayerCharacter.GetCharacterVanity` _player_character))
  (`VanityItem.ApplyItem` InputPin _player_character true))

(fn `GetSavedVanity`
  (returns (SavedVanity :type "EquippedVanity Structure"))
  (locals (NewLocalVar_0 :type Integer :default 0))
  (bind _as_custom_vanity_testing_savegame (`self.As Custom Vanity Testing Savegame`))
  (bind _as_custom_vanity_testing_savegame_2 (`self.As Custom Vanity Testing Savegame`))
  (bind _as_custom_vanity_testing_savegame_3 (`self.As Custom Vanity Testing Savegame`))
  (bind _as_custom_vanity_testing_savegame_4 (`self.As Custom Vanity Testing Savegame`))
  (bind _returnvalue (`ActorFunctionLibrary.GetCharacterIDFromCharacter` (`self.Player Character`)))
  (bind _output_get (set `local.NewLocalVar_0` (`FSDSaveGame.GetSelectedLoadoutIndex` (`FSDGameInstance.SaveGame` (`GameFunctionLibrary.GetFSDGameInstance` self)) _returnvalue)))
  (`/Game/_DRGModding/_Frameworks/BML_Framework.SwitchByPlayerCharacterID` _returnvalue
    (:`DrillerID`
      (switch `int` _output_get
        (:`0`
          (return (`/Game/_DRGModding/_Frameworks/_Patch/CustomVanityFramework/Patch_01_ReplicationFix/CustomVanityTestingSavegame.DrillerID_0` _as_custom_vanity_testing_savegame_2)))
        (:`1`
          (return (`/Game/_DRGModding/_Frameworks/_Patch/CustomVanityFramework/Patch_01_ReplicationFix/CustomVanityTestingSavegame.DrillerID_1` _as_custom_vanity_testing_savegame_2)))
        (:`2`
          (return (`/Game/_DRGModding/_Frameworks/_Patch/CustomVanityFramework/Patch_01_ReplicationFix/CustomVanityTestingSavegame.DrillerID_2` _as_custom_vanity_testing_savegame_2)))
        (:`3`
          (return (`/Game/_DRGModding/_Frameworks/_Patch/CustomVanityFramework/Patch_01_ReplicationFix/CustomVanityTestingSavegame.DrillerID_3` _as_custom_vanity_testing_savegame_2)))
        (:`4`
          (return (`/Game/_DRGModding/_Frameworks/_Patch/CustomVanityFramework/Patch_01_ReplicationFix/CustomVanityTestingSavegame.DrillerID_4` _as_custom_vanity_testing_savegame_2)))
        (:`5`
          (return (`/Game/_DRGModding/_Frameworks/_Patch/CustomVanityFramework/Patch_01_ReplicationFix/CustomVanityTestingSavegame.DrillerID_5` _as_custom_vanity_testing_savegame_2)))))
    (:`EngineerID`
      (switch `int` _output_get
        (:`0`
          (return (`/Game/_DRGModding/_Frameworks/_Patch/CustomVanityFramework/Patch_01_ReplicationFix/CustomVanityTestingSavegame.EngineerID_0` _as_custom_vanity_testing_savegame_3)))
        (:`1`
          (return (`/Game/_DRGModding/_Frameworks/_Patch/CustomVanityFramework/Patch_01_ReplicationFix/CustomVanityTestingSavegame.EngineerID_1` _as_custom_vanity_testing_savegame_3)))
        (:`2`
          (return (`/Game/_DRGModding/_Frameworks/_Patch/CustomVanityFramework/Patch_01_ReplicationFix/CustomVanityTestingSavegame.EngineerID_2` _as_custom_vanity_testing_savegame_3)))
        (:`3`
          (return (`/Game/_DRGModding/_Frameworks/_Patch/CustomVanityFramework/Patch_01_ReplicationFix/CustomVanityTestingSavegame.EngineerID_3` _as_custom_vanity_testing_savegame_3)))
        (:`4`
          (return (`/Game/_DRGModding/_Frameworks/_Patch/CustomVanityFramework/Patch_01_ReplicationFix/CustomVanityTestingSavegame.EngineerID_4` _as_custom_vanity_testing_savegame_3)))
        (:`5`
          (return (`/Game/_DRGModding/_Frameworks/_Patch/CustomVanityFramework/Patch_01_ReplicationFix/CustomVanityTestingSavegame.EngineerID_5` _as_custom_vanity_testing_savegame_3)))))
    (:`GunnerID`
      (switch `int` _output_get
        (:`0`
          (return (`/Game/_DRGModding/_Frameworks/_Patch/CustomVanityFramework/Patch_01_ReplicationFix/CustomVanityTestingSavegame.GunnerID_0` _as_custom_vanity_testing_savegame_4)))
        (:`1`
          (return (`/Game/_DRGModding/_Frameworks/_Patch/CustomVanityFramework/Patch_01_ReplicationFix/CustomVanityTestingSavegame.GunnerID_1` _as_custom_vanity_testing_savegame_4)))
        (:`2`
          (return (`/Game/_DRGModding/_Frameworks/_Patch/CustomVanityFramework/Patch_01_ReplicationFix/CustomVanityTestingSavegame.GunnerID_2` _as_custom_vanity_testing_savegame_4)))
        (:`3`
          (return (`/Game/_DRGModding/_Frameworks/_Patch/CustomVanityFramework/Patch_01_ReplicationFix/CustomVanityTestingSavegame.GunnerID_3` _as_custom_vanity_testing_savegame_4)))
        (:`4`
          (return (`/Game/_DRGModding/_Frameworks/_Patch/CustomVanityFramework/Patch_01_ReplicationFix/CustomVanityTestingSavegame.GunnerID_4` _as_custom_vanity_testing_savegame_4)))
        (:`5`
          (return (`/Game/_DRGModding/_Frameworks/_Patch/CustomVanityFramework/Patch_01_ReplicationFix/CustomVanityTestingSavegame.GunnerID_5` _as_custom_vanity_testing_savegame_4)))))
    (:`ScoutID`
      (switch `int` _output_get
        (:`0`
          (return (`/Game/_DRGModding/_Frameworks/_Patch/CustomVanityFramework/Patch_01_ReplicationFix/CustomVanityTestingSavegame.ScoutID_0` _as_custom_vanity_testing_savegame)))
        (:`1`
          (return (`/Game/_DRGModding/_Frameworks/_Patch/CustomVanityFramework/Patch_01_ReplicationFix/CustomVanityTestingSavegame.ScoutID_1` _as_custom_vanity_testing_savegame)))
        (:`2`
          (return (`/Game/_DRGModding/_Frameworks/_Patch/CustomVanityFramework/Patch_01_ReplicationFix/CustomVanityTestingSavegame.ScoutID_2` _as_custom_vanity_testing_savegame)))
        (:`3`
          (return (`/Game/_DRGModding/_Frameworks/_Patch/CustomVanityFramework/Patch_01_ReplicationFix/CustomVanityTestingSavegame.ScoutID_3` _as_custom_vanity_testing_savegame)))
        (:`4`
          (return (`/Game/_DRGModding/_Frameworks/_Patch/CustomVanityFramework/Patch_01_ReplicationFix/CustomVanityTestingSavegame.ScoutID_4` _as_custom_vanity_testing_savegame)))
        (:`5`
          (return (`/Game/_DRGModding/_Frameworks/_Patch/CustomVanityFramework/Patch_01_ReplicationFix/CustomVanityTestingSavegame.ScoutID_5` _as_custom_vanity_testing_savegame)))))))

(fn `UserConstructionScript`)