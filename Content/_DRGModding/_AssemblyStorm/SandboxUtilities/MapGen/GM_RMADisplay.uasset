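; GM_RMADisplay is a map-generation game mode in Sandbox Utilities that sets up a free-camera display view of the generated level.
; Construction disables scripted enemy waves, and a chosen generation pass triggers a scaled cube-mesh carve of the CSG world with a replace-solid filter.
; When the local player registers, an arbitrary one-second delay precedes enabling SandboxUtilities fullbright, toggling free cam and teleporting it to a fixed viewpoint.
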(event `self.OnLevelGenerationComplete`
  (params (pass :type Integer))
  (`parent.OnLevelGenerationComplete` pass)
  (if (`|EnumEquality` (cast `/Game/Landscape/PLS_Passes` (`KismetMathLibrary.Conv_IntToByte` pass)) "NewEnumerator7")
    (`DeepCSGWorld.CarveWithMeshUsingTransform` (`FSDGameState.CSGWorld` (`GameFunctionLibrary.GetFSDGameState` self)) "/Game/Art/Carvers/SM_Cube_1-1-1.SM_Cube_1-1-1" null "ReplaceSolid" (`KismetMathLibrary.MakeTransform` (0.0 0.0 0.0) (struct) (2.0 2.0 2.0)) 0.0 "TurnIntoGems" "CARVE_CELL_SIZE_200")))

(event `self.ReceiveBeginPlay`
  (`parent.ReceiveBeginPlay`)
  (add `FSDGameState.OnPlayerCharacterRegistered` (`GameFunctionLibrary.GetFSDGameState` self) (delegate `CustomEvent_0`)))

(event `CustomEvent_0`
  (params (PlayerCharacter :type "PlayerCharacter Object Reference"))
  (if (`Pawn.IsLocallyControlled` PlayerCharacter)
    (`KismetSystemLibrary.Delay` 1.0) ; Arbitrary delay because reasons?!
    (bind _returnvalue (`GameplayStatics.GetActorOfClass` "/Game/_DRGModding/_AssemblyStorm/SandboxUtilities/SandboxUtilities.SandboxUtilities_C"))
    (`/Game/_DRGModding/_AssemblyStorm/SandboxUtilities/MissionPage.SetFullBright` (`/Game/_DRGModding/_AssemblyStorm/SandboxUtilities/SandboxUtilities.MissionPage` _returnvalue) true)
    (`/Game/_DRGModding/_AssemblyStorm/SandboxUtilities/SandboxUtilities.ToggleFreeCam` _returnvalue)
    (`SceneComponent.K2_SetWorldTransform` (`Actor.RootComponent` (`/Game/_DRGModding/_AssemblyStorm/SandboxUtilities/SandboxUtilities.Cam` _returnvalue)) (`KismetMathLibrary.MakeTransform` (10000.0 70000.0 15000.0) (struct :`Pitch` -22.0 :`Yaw` -119.0)) false true)))

(fn `UserConstructionScript`
  (bind _enemywavemanager (`self.EnemyWaveManager`))
  (`parent.UserConstructionScript`)
  (`EnemyWaveManager.PushDisableScriptedWaves` _enemywavemanager _enemywavemanager))