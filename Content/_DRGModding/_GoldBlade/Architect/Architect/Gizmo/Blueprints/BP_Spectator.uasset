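; BP_Spectator is the input controller for a runtime transform gizmo, letting the player click actors and manipulate them with BP_Gizmo.
; On BeginPlay it shows the mouse cursor in Game and UI input mode and caches the level's single BP_Gizmo, printing an error otherwise.
; Left click attaches the gizmo to the actor under the mouse, while keys cycle translate/rotate/scale, toggle world/local space and enable scale grid snapping.
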(event `self.ReceiveBeginPlay`
  (bind _returnvalue (`GameplayStatics.GetPlayerController` 0))
  (`|ExecutionSequence`
    (:`then_0`
      (set `PlayerController.bShowMouseCursor` true _returnvalue)
      (`WidgetBlueprintLibrary.SetInputMode_GameAndUIEx` _returnvalue null))
    (:`then_1`
      (bind _outactors (`GameplayStatics.GetAllActorsOfClass` "/Game/_DRGModding/_GoldBlade/Architect/Architect/Gizmo/Blueprints/BP_Gizmo.BP_Gizmo_C"))
      (if (!= (`KismetArrayLibrary.Array_Length` _outactors) 1)
        (`KismetSystemLibrary.PrintString` "ERROR: There should be exactly a single instance of BP_Gizmo in the level." true true (struct :`R` 1.0 :`A` 1.0) 10000.0)
        (else
          (set `self.GizmoRef` (`|GetArrayItem` _outactors)))))))

(event `Key|LeftMouseButton`
  (params (Key :type "Key Structure"))
  (bind _gizmoref (`self.GizmoRef`))
  (:`Pressed`
    (bind _hitactor (`/Game/_DRGModding/_GoldBlade/Architect/Architect/Gizmo/Blueprints/BP_Gizmo.GetMouseSelectedActor` _gizmoref))
    (`/Engine/EditorBlueprintResources/StandardMacros.IsValid` _hitactor
      (:`Is Valid`
        (`/Game/_DRGModding/_GoldBlade/Architect/Architect/Gizmo/Blueprints/BP_Gizmo.AttachGizmo` _gizmoref _hitactor)))))

(event `Key|SpaceBar`
  (params (Key :type "Key Structure"))
  (bind _gizmoref (`self.GizmoRef`))
  (:`Pressed`
    (bind _returnvalue (`/Game/_DRGModding/_GoldBlade/Architect/Architect/Gizmo/Blueprints/BP_Gizmo.IsGizmoAttached` _gizmoref))
    (if _returnvalue
      (bind _returnvalue_2 (`/Game/_DRGModding/_GoldBlade/Architect/Architect/Gizmo/Blueprints/BP_Gizmo.GetGizmoMode` _gizmoref))
      (switch `/Game/_DRGModding/_GoldBlade/Architect/Architect/Gizmo/Blueprints/GizmoMode` _returnvalue_2
        (:`NewEnumerator0`
          (`/Game/_DRGModding/_GoldBlade/Architect/Architect/Gizmo/Blueprints/BP_Gizmo.SetGizmoMode` _gizmoref "NewEnumerator1"))
        (:`NewEnumerator1`
          (`/Game/_DRGModding/_GoldBlade/Architect/Architect/Gizmo/Blueprints/BP_Gizmo.SetGizmoMode` _gizmoref "NewEnumerator2"))
        (:`NewEnumerator2`
          (`/Game/_DRGModding/_GoldBlade/Architect/Architect/Gizmo/Blueprints/BP_Gizmo.SetGizmoMode` _gizmoref "NewEnumerator0"))))))

(event `Key|M`
  (params (Key :type "Key Structure"))
  (bind _gizmoref (`self.GizmoRef`))
  (:`Pressed`
    (bind _returnvalue (`/Game/_DRGModding/_GoldBlade/Architect/Architect/Gizmo/Blueprints/BP_Gizmo.IsGizmoAttached` _gizmoref))
    (if _returnvalue
      (bind _coordinatesystem (`/Game/_DRGModding/_GoldBlade/Architect/Architect/Gizmo/Blueprints/BP_Gizmo.GetCoordinateSystem` _gizmoref))
      (switch `/Game/_DRGModding/_GoldBlade/Architect/Architect/Gizmo/Blueprints/GizmoCoordinateSystem` _coordinatesystem
        (:`NewEnumerator0`
          (`/Game/_DRGModding/_GoldBlade/Architect/Architect/Gizmo/Blueprints/BP_Gizmo.SetCoordinateSystem` _gizmoref "NewEnumerator1"))
        (:`NewEnumerator1`
          (`/Game/_DRGModding/_GoldBlade/Architect/Architect/Gizmo/Blueprints/BP_Gizmo.SetCoordinateSystem` _gizmoref "NewEnumerator0"))))))

(event `Key|N`
  (params (Key :type "Key Structure"))
  (:`Pressed`
    (`/Game/_DRGModding/_GoldBlade/Architect/Architect/Gizmo/Blueprints/BP_Gizmo.Set Grid Snap Scale` (`self.GizmoRef`) true 1.0)))

(fn `UserConstructionScript`)