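; Mission director component that runs a 60-second grace period after the drop pod lands, holding its doors shut.
; StartGracePeriod runs once, retrying until it finds the game mode's drop pod, then polls on a looping timer for landing.
; On landing, a fast looping timer re-forces the door state while director messages count down.
; At "Ready!" it clears that timer and, after a short delay, sets the door state one last time.
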(event `StartGracePeriod`
  (`/Engine/EditorBlueprintResources/StandardMacros.DoOnce` false
    (:`Completed`
      (bind _returnvalue (`GameplayStatics.GetActorOfClass` (`FSDGameMode.GetDropPodClass` (cast `FSDGameMode` (`GameplayStatics.GetGameMode`) :!pure true)) :!label _label))
      (`/Engine/EditorBlueprintResources/StandardMacros.IsValid` _returnvalue
        (:`Is Valid`
          (bind _output_get (set `self.TeamTransport` _returnvalue))
          (bind _asbp_drop_pod_base (cast `/Game/LevelElements/Droppod/BP_DropPod_Base` _output_get))
          (set `self.AsDroppod` _asbp_drop_pod_base)
          (bind _returnvalue_2 (`KismetSystemLibrary.K2_SetTimerDelegate` (delegate `CheckForLanding`) 0.1 true))
          (set `self.HasLandedTimer` _returnvalue_2))
        (:`Is Not Valid`
          (`KismetSystemLibrary.Delay` 0.2)
          (goto _label))))))

(event `CheckForLanding`
  (if (`TeamTransport.GetHasLanded` (`self.TeamTransport`))
    (`KismetSystemLibrary.K2_ClearAndInvalidateTimerHandle` (`self.HasLandedTimer`))
    (bind _returnvalue (`KismetSystemLibrary.K2_SetTimerDelegate` (delegate `ForceCloseDoors`) 0.1 true))
    (set `self.ForceCloseTimer` _returnvalue)
    (`/Game/_DRGModding/_GoldBlade/MissionDirector/Libraries/MDFunctions.SendDirectorMessage` "60 second grace period is active.")
    (`KismetSystemLibrary.Delay` 30.0)
    (`/Game/_DRGModding/_GoldBlade/MissionDirector/Libraries/MDFunctions.SendDirectorMessage` "30 seconds remaining...")
    (`KismetSystemLibrary.Delay` 20.0)
    (`/Game/_DRGModding/_GoldBlade/MissionDirector/Libraries/MDFunctions.SendDirectorMessage` "10 seconds remaining...")
    (`KismetSystemLibrary.Delay` 10.0)
    (`/Game/_DRGModding/_GoldBlade/MissionDirector/Libraries/MDFunctions.SendDirectorMessage` "Ready!")
    (`KismetSystemLibrary.K2_ClearAndInvalidateTimerHandle` (`self.ForceCloseTimer`))
    (`KismetSystemLibrary.Delay` 2.0)
    (`/Game/LevelElements/Droppod/BP_DropPod_Base.SetDoorState` (`self.AsDroppod`) "NewEnumerator0" 2)))

(event `ForceCloseDoors`
  (`/Game/LevelElements/Droppod/BP_DropPod_Base.SetDoorState` (`self.AsDroppod`) "NewEnumerator0"))