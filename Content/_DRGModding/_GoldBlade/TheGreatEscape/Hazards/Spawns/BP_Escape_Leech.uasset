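; BP_Escape_Leech is a placed spawner that puts a Cave Leech on the ceiling above it in the Great Escape mod's hazards.
; On BeginPlay it traces straight up and moves to the hit point, then carves the DeepCSGWorld terrain there with a scaled cylinder mesh.
; It spawns ENE_CaveLeech slightly above the hit and destroys itself; if the trace misses, it does nothing.
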(event `self.ReceiveBeginPlay`
  (bind _returnvalue (`self.K2_GetActorLocation`))
  (bind (_segmentstart _segmentend) (`/Game/_DRGModding/_GoldBlade/TheGreatEscape/Libraries/GreatEscapeFunctions.LineSegmentFromDirection` (`self.K2_GetActorLocation`) (`KismetMathLibrary.MakeVector` 0.0 0.0 1.0) 100000.0))
  (bind (_outhit _returnvalue_2) (`KismetSystemLibrary.LineTraceSingle` _segmentstart _segmentend "TraceTypeQuery1" true))
  (if _returnvalue_2
    (`self.K2_SetActorLocation` (`.Location` (`GameplayStatics.BreakHitResult` _outhit)))
    (bind _outactors (`GameplayStatics.GetAllActorsOfClass` "/Script/FSD.DeepCSGWorld"))
    (for _array_element _outactors
      (`DeepCSGWorld.CarveWithMeshUsingTransform` _array_element "/Game/Art/Carvers/SM_Cylinder_1_1_1.SM_Cylinder_1_1_1" null "ReplaceAll" (`KismetMathLibrary.MakeTransform` (- _returnvalue (0.0 0.0 50.0)) (struct) (3.0 3.0 3.0)) 1.0 "TurnIntoGems" "CARVE_CELL_SIZE_25"))
    (`|SpawnActorFromClass` "/Game/Enemies/CaveLeech/ENE_CaveLeech.ENE_CaveLeech_C" (`KismetMathLibrary.MakeTransform` (+ _returnvalue (0.0 0.0 100.0))) "AlwaysSpawn" "OverrideRootScale" null null)
    (`self.K2_DestroyActor`)))

(fn `UserConstructionScript`
  (`parent.UserConstructionScript`))