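; BP_CountdownComponent is a reusable countdown component in the GoldBlade SpawnMenu mod that counts whole seconds down to zero.
; StartCountdown resets any running timer, stores the start value and starts a looping one-second timer that decrements TimeRemaining and stops at zero.
; It broadcasts started, elapsed and stopped notifications carrying the remaining time, and exposes StopCountdown and GetTimeRemaining for outside control.
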(event `StartCountdown`
  (params (StartSeconds :type Integer))
  (set `self.TimeRemaining` StartSeconds)
  (`KismetSystemLibrary.K2_ClearAndInvalidateTimerHandle` (`self.CountTimer`))
  (`self.OnCountdownStarted` (`self.TimeRemaining`))
  (bind _returnvalue (`KismetSystemLibrary.K2_SetTimerDelegate` (delegate `CountdownElapsed`) 1.0 true))
  (set `self.CountTimer` _returnvalue))

(event `CountdownElapsed`
  (`self.DecrementTime`
    (:`  `
      (`self.OnTimeElapsed` (`self.TimeRemaining`))
      (if (<= (`self.TimeRemaining`) 0)
        (`self.StopCountdown`)))))

(fn `GetTimeRemaining`
  (returns (TimeRemaining :type Integer))
  (return (`self.TimeRemaining`)))

(fn `StopCountdown`
  (`KismetSystemLibrary.K2_ClearAndInvalidateTimerHandle` (`self.CountTimer`))
  (`self.OnCountdownStopped` (`self.TimeRemaining`)))