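; Actor component for the SpawnMenu mod that gives a player character a random beer effect on DrinkBeer.
; It adds a random component class from BeerEffects to the owning BP_PlayerCharacter, then waits for that effect's duration.
; Afterwards it clears the character's intoxication, with an IsDrunk flag blocking further drinks until then.
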(event `DrinkBeer`
  (if (not (`self.IsDrunk`))
    (set `self.IsDrunk` true)
    (bind _asbp_player_character (cast `/Game/Character/BP_PlayerCharacter` (`self.GetOwner`)))
    (bind _output_get (set `self.Player` _asbp_player_character))
    (bind _returnvalue (`|AddComponentByClass` _output_get (`KismetArrayLibrary.Array_Random` (`self.BeerEffects`))))
    (`KismetSystemLibrary.Delay` (`DrinkEffectComponent.BeerEffectDurationSeconds` _returnvalue))
    (`CharacterIntoxicationComponent.ClearIntoxication` (`PlayerCharacter.IntoxicationComponent` (`self.Player`)))
    (set `self.IsDrunk` false)))