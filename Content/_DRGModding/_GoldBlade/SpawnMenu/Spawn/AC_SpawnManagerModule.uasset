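; Spawn manager component for the SpawnMenu mod that places data-table-defined items around target actors.
; BeginPlay caches spawn table rows, which are looked up or listed by ID.
; On the server, SpawnItem finds random terrain locations within a distance range and spawns proxy actors, which begin spawning through ISpawnProxy.
; RegisterSpawn optionally adds Nitra kill rewards according to mod settings; AddSpawnItem is an empty stub.
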(event `self.ReceiveBeginPlay`
  (bind _asmod_spawn_menu (cast `/Game/_DRGModding/_GoldBlade/SpawnMenu/Mod_SpawnMenu` (`self.GetOwner`)))
  (set `self.SpawnMenuMod` _asmod_spawn_menu)
  (bind _returnvalue (`/Game/_DRGModding/_GoldBlade/SpawnMenu/Libraries/ModFunctions.GetLocalPlayer`))
  (set `self.LocalPlayer` _returnvalue)
  (bind _outrownames (`DataTableFunctionLibrary.GetDataTableRowNames` "/Game/_DRGModding/_GoldBlade/SpawnMenu/Spawn/Items/SpawnItemsTable.SpawnItemsTable"))
  (for _array_element _outrownames
    (bind _returnvalue_2 (`|GetDataTableRow` "/Game/_DRGModding/_GoldBlade/SpawnMenu/Spawn/Items/SpawnItemsTable.SpawnItemsTable" _array_element)
      (:`then`
        (`KismetArrayLibrary.Array_Add` (`self.SpawnItems`) _returnvalue_2)))))

(event `self.RegisterSpawn`
  (params (Spawn :type "Actor Object Reference (by ref)") (StateContainer :type "Object Object Reference (by ref)") (NitraReward :type Integer))
  (if (`/Game/_DRGModding/_GoldBlade/SpawnMenu/Settings/SAV_SpawnMenuSettings.RewardNitraOnKill` (`/Game/_DRGModding/_GoldBlade/SpawnMenu/Mod_SpawnMenu.ModSettings` (`self.SpawnMenuMod`)))
    (`|AddComponentByClass` Spawn "/Game/_DRGModding/_GoldBlade/SpawnMenu/Components/NitraRewardComponent.NitraRewardComponent_C" NitraReward)))

(event `self.AddSpawnItem`
  (params (ID :type Name) (Name :type String) (Thumbnail :type "Texture2D Object Reference") (SpawnProxyClass :type "Actor Class Reference")))

(fn `FindSpawnLocation`
  (params (Origin :type "Vector Structure") (MinDistance :type "Float (double-precision)") (MaxDistance :type "Float (double-precision)") (MinSlopeDegrees :type "Float (double-precision)") (MaxSlopeDegrees :type "Float (double-precision)"))
  (returns (Location :type "Vector Structure") (Rotation :type "Rotator Structure"))
  (bind (_location _normal _rotation) (`/Game/_DRGModding/_GoldBlade/SpawnMenu/Libraries/SpawnFunctions.Get Random World Transform V5` Origin (`KismetMathLibrary.FClamp` (`KismetMathLibrary.FMin` MinDistance MaxDistance) 100.0 10000.0) (`KismetMathLibrary.FClamp` (`KismetMathLibrary.FMax` MinDistance MaxDistance) 200.0 10000.0) MinSlopeDegrees MaxSlopeDegrees (`|MakeArray`) 0.0 true false false (`|MakeArray`) 0.0 20 15 500.0 "NewEnumerator1"))
  (return _location _rotation))

(fn `GetAllSpawnItems`
  (returns (ItemIDs :type "Array of Name") (ItemNames :type "Array of String"))
  (locals (ids_list :type "Array of Name") (names_list :type "Array of String"))
  (for _array_element (`self.SpawnItems`)
    (bind ((`ID_54_0167813A4319B86EE1499E8A7263EFD4` _id) (`Name_44_2CA643B9450192689AAA65865F355D19` _name)) (break `/Game/_DRGModding/_GoldBlade/SpawnMenu/Spawn/Items/SpawnItem` _array_element))
    (`KismetArrayLibrary.Array_Add` (`local.ids_list`) _id)
    (`KismetArrayLibrary.Array_Add` (`local.names_list`) _name))
  (return (`local.ids_list`) (`local.names_list`)))

(fn `GetSpawnItem`
  (params (ID :type Name))
  (returns (ReturnValue :type Boolean) (Index :type Integer) (SpawnType :type "/Game/_DRGModding/_GoldBlade/SpawnMenu/Spawn/Items/SpawnItem Structure"))
  (for (_array_element _array_index) (`self.SpawnItems`)
    (if (== (`.ID_54_0167813A4319B86EE1499E8A7263EFD4` (break `/Game/_DRGModding/_GoldBlade/SpawnMenu/Spawn/Items/SpawnItem` _array_element)) ID)
      (return true _array_index _array_element)))
  (return false 0))

(fn `SpawnItem`
  (params (ItemID :type Name) (ParentTarget :type "Actor Object Reference (by ref)") (Username :type String) (MinDistance :type "Float (double-precision)") (MaxDistance :type "Float (double-precision)") (Count :type Integer))
  (locals (itemConfig :type " Structure") (loc :type "Vector Structure" :default (0.0 0.0 0.0)) (rot :type "Rotator Structure" :default (struct)) (targets :type "Array of Actor Object Reference"))
  (if (`KismetSystemLibrary.IsServer`)
    (`KismetArrayLibrary.Array_AddUnique` (`local.targets`) ParentTarget)
    (bind (_returnvalue _index _spawntype) (`self.GetSpawnItem` ItemID))
    (if _returnvalue
      (for _array_element (`local.targets`)
        (`/Game/_DRGModding/_GoldBlade/SpawnMenu/Libraries/ModComponentMacros.RepeatN` Count
          (:`LoopBody`
            (bind (_location _rotation) (`self.FindSpawnLocation` (`Actor.K2_GetActorLocation` _array_element) MinDistance MaxDistance 0.0 70.0))
            (`self.SpawnProxyByClass` (`.SpawnProxyClass_82_B2FE6A3C46473777F3CA599BA76CAE1C` (break `/Game/_DRGModding/_GoldBlade/SpawnMenu/Spawn/Items/SpawnItem` _spawntype)) (`KismetMathLibrary.MakeTransform` _location _rotation) _array_element (`local.Username`))))))))

(fn `SpawnProxyByClass`
  (params (ProxyClass :type "Actor Class Reference") (SpawnTransform :type "Transform Structure") (Parent :type "Actor Object Reference (by ref)") (Username :type String))
  (returns (Proxy :type "Actor Object Reference"))
  (locals (proxySpawn :type "Actor Object Reference"))
  (if (`KismetSystemLibrary.IsServer`)
    (bind _returnvalue (`|SpawnActorFromClass` ProxyClass SpawnTransform "AlwaysSpawn" "OverrideRootScale" null null))
    (bind _output_get (set `local.proxySpawn` _returnvalue))
    (bind _asispawn_proxy (cast `/Game/_DRGModding/_GoldBlade/SpawnMenu/ISpawnProxy` _output_get))
    (`/Game/_DRGModding/_GoldBlade/SpawnMenu/ISpawnProxy.BeginSpawn` _asispawn_proxy self (`self.EmptyObj`) (`local.Username`) "" (`local.Parent`) (`|MakeMap`))
    (return (`local.proxySpawn`))))