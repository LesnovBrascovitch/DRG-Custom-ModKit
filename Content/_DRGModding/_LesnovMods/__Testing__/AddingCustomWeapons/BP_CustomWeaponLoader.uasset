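; Test mod actor that loads custom weapons into the game by registering them in save and game data.
; On BeginPlay it waits for the FSD save, unlocks listed items, adds item classes to the local player's inventory, edits unlocked skins and saves to disk.
; A looping timer keeps injecting its ItemData map into the game's ItemSettings.
; CheckItemAdded can stop that timer once all entries exist, but nothing here calls it.
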(event `CheckItemData`
  (bind _keys (`BlueprintMapLibrary.Map_Keys` (`ItemSettings.ItemData` (`GameData.ItemSettings` (`GameFunctionLibrary.GetFSDGameData`)))))
  (for _array_element _keys
    _))

(event `AddItemData`
  (bind _item_data (`self.Item Data`))
  (bind _keys (`BlueprintMapLibrary.Map_Keys` _item_data))
  (for _array_element _keys
    (bind (_value _returnvalue) (`BlueprintMapLibrary.Map_Find` _item_data _array_element))
    (if _returnvalue
      (`BlueprintMapLibrary.Map_Add` (`ItemSettings.ItemData` (`GameData.ItemSettings` (`GameFunctionLibrary.GetFSDGameData`))) _array_element _value))))

(event `self.ReceiveBeginPlay`
  (bind _returnvalue (`GameFunctionLibrary.GetFSDSaveGame`))
  (`/Game/_DRGModding/_LesnovMods/_SharedAssets/BML_Actor.ValidCheck(Wait | FSDSaveGame)`)
  (for _array_element (`InventoryList.GetAllItemsList` (`self.InventoryListToLoad`))
    (bind _savegameid (`SavableDataAsset.SavegameID` _array_element))
    (`KismetArrayLibrary.Array_AddUnique` (`FSDSaveGame.UnlockedItems` _returnvalue) _savegameid)
    (`KismetArrayLibrary.Array_AddUnique` (`FSDSaveGame.OwnedItems` _returnvalue) _savegameid)
    (`FSDCheatManager.Cheat_UnlockWeapon` _array_element))
  (bind _returnvalue_2 (`/Game/_DRGModding/_LesnovMods/_SharedAssets/BML_Actor.ValidCheck(Wait | SBZPlayerCharacter)`))
  (set `self.PlayerCharacter` _returnvalue_2)
  (`self.AddItemClasses` (`self.Item Classes to Add`))
  (bind _values (`BlueprintMapLibrary.Map_Values` (`FSDSaveGame.UnlockedItemSkins` (`GameFunctionLibrary.GetFSDSaveGame`))))
  (for _array_element_2 _values
    (bind _result (`BlueprintSetLibrary.Set_ToArray` (break `SkinList` _array_element_2)))
    (`BlueprintSetLibrary.Set_AddItems` (`self.Array Element Skins`) _result))
  (`BlueprintMapLibrary.Map_Add` (`FSDSaveGame.UnlockedItemSkins` (`GameFunctionLibrary.GetFSDSaveGame`)) (`self.NewVar_0`) (make `SkinList` (`self.NewVar_4`)))
  (`FSDSaveGame.SaveToDisk` (`GameFunctionLibrary.GetFSDSaveGame`))
  (bind _returnvalue_3 (`KismetSystemLibrary.K2_SetTimerDelegate` (delegate `AddItemData`) 2.0 true))
  (set `self.AddItemHandle` _returnvalue_3))

(fn `AddItemClasses`
  (params (ItemClassesToAdd :type "Array of Item Class Reference"))
  (for _array_element ItemClassesToAdd
    (`InventoryComponent.AddItemClass` (`PlayerCharacter.InventoryComponent` (`GameFunctionLibrary.GetLocalPlayerCharacter`)) _array_element)))

(fn `CheckItemAdded`
  (locals (IsInvalid :type Boolean :default false))
  (bind _keys (`BlueprintMapLibrary.Map_Keys` (`self.Item Data`)))
  (for _array_element _keys
    (if (not (`.ReturnValue` (`BlueprintMapLibrary.Map_Find` (`ItemSettings.ItemData` (`GameData.ItemSettings` (`GameFunctionLibrary.GetFSDGameData`))) _array_element)))
      (set `local.IsInvalid` true)
      (break)))
  (if (not (`local.IsInvalid`))
    (`KismetSystemLibrary.K2_ClearAndInvalidateTimerHandle` (`self.AddItemHandle`))))

(fn `UserConstructionScript`)