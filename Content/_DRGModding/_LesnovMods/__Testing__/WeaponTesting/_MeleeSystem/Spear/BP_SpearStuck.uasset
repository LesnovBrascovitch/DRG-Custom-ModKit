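; Stuck-spear pickup actor that stands in for a thrown spear after a hit and lets it be retrieved.
; On initialization it stores its throwable weapon, which transfers its material to the skeletal mesh.
; Capsule collision starts off; when the hit actor is destroyed, collision and physics turn on so the spear drops.
; Using it notifies the weapon of retrieval once and destroys the actor.
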(event `self.ReceiveBeginPlay`
  (`PrimitiveComponent.SetCollisionEnabled` (`self.Capsule`) "NoCollision"))

(event `OnSpearHit`
  (params (Actor :type "Actor Object Reference"))
  (add `self.OnDestroyed` Actor (delegate `CustomEvent_0`)))

(event `CustomEvent_0` :!signature `self.OnDestroyed`
  (params (DestroyedActor :type "Actor Object Reference"))
  (bind _capsule (`self.Capsule`))
  (`PrimitiveComponent.SetCollisionEnabled` _capsule "QueryAndPhysics")
  (`PrimitiveComponent.SetSimulatePhysics` _capsule true))

(event `self.InstantUsable.OnUsedBy`
  (params (User :type "PlayerCharacter Object Reference") (Key :type "EInputKeys Enum" :default "Use"))
  (`/Engine/EditorBlueprintResources/StandardMacros.DoOnce` false
    (:`Completed`
      (`/Game/_DRGModding/_LesnovMods/__Testing__/WeaponTesting/_MeleeSystem/Spear/MWPN_Spear.OnThrowableRetrieved` (`self.ThrowableWeapon`))
      (`self.K2_DestroyActor`))))

(event `OnInitialize`
  (params (ThrowableWeapon :type "/Game/_DRGModding/_LesnovMods/__Testing__/WeaponTesting/_MeleeSystem/Spear/MWPN_Spear Object Reference"))
  (bind _throwableweapon (`self.ThrowableWeapon`))
  (set `self.ThrowableWeapon` ThrowableWeapon)
  (`/Engine/EditorBlueprintResources/StandardMacros.IsValid` _throwableweapon
    (:`Is Valid`
      (`/Game/_DRGModding/_LesnovMods/__Testing__/WeaponTesting/_MeleeSystem/Spear/MWPN_Spear.TransferMaterial` _throwableweapon (`self.SkeletalMesh`)))))

(fn `UserConstructionScript`)