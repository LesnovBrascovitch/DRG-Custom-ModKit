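; Carriable ammo gem for the Full Armor Bosco mod that resupplies Bosco, or the player's weapons when deposited.
; A looping timer checks proximity to Bosco, and a sphere overlap also detects him; either path calls Resupply, plays a sound and destroys the gem.
; Depositing adds ammo and clip to the player's ammo-driven items at Bosco's drop rate.
; Pickup and drop toggle the first-person mesh FOV.
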(event `CustomEvent_0`
  (if (< (`KismetMathLibrary.VSize` (- (`self.K2_GetActorLocation`) (`self.K2_GetActorLocation` (`self.FABosco`)))) 400.0)
    (`/Engine/EditorBlueprintResources/StandardMacros.DoOnce` false
      (:`Completed`
        (`/Game/_DRGModding/_LesnovMods/GameplayMods/Mod_FullArmorBosco/BP_FABosco.Resupply` (`self.FABosco`) 1000 :!label _label)
        (`GameplayStatics.SpawnSoundAtLocation` "/Game/_DRGModding/_LesnovMods/GameplayMods/Mod_FullArmorBosco/SFX/GainedAmmo_Cue.GainedAmmo_Cue" (`self.K2_GetActorLocation`) (struct) 1.0 1.0 0.0 null null)
        (`self.K2_DestroyActor`)))))

(event `self.ReceiveBeginPlay`
  (`parent.ReceiveBeginPlay`)
  (if (`self.`)
    (`KismetSystemLibrary.K2_SetTimerDelegate` (delegate `CustomEvent_0`) 0.4 true)))

(event `self.Carriable.OnPickedUp`
  (set `FirstPersonStaticMeshComponent.EnabledFPFOV` true (`self.FirstPersonStaticMesh1`)))

(event `self.Carriable.OnDropped`
  (set `FirstPersonStaticMeshComponent.EnabledFPFOV` false (`self.FirstPersonStaticMesh1`)))

(event `self.Sphere1.OnComponentBeginOverlap`
  (params (OverlappedComponent :type "PrimitiveComponent Object Reference") (OtherActor :type "Actor Object Reference") (OtherComp :type "PrimitiveComponent Object Reference") (OtherBodyIndex :type Integer) (bFromSweep :type Boolean) (SweepResult :type "HitResult Structure (by ref)"))
  (`/Engine/EditorBlueprintResources/StandardMacros.IsValid` (`self.FABosco`)
    (:`Is Valid`
      (if (`KismetMathLibrary.ClassIsChildOf` (`GameplayStatics.GetObjectClass` OtherActor) "/Game/GameElements/Drone/BP_Bosco.BP_Bosco_C")
        (goto _label)))))

(event `self.Receive_OnDeposited`
  (params (fromPlayer :type "PlayerCharacter Object Reference") (toActor :type "Actor Object Reference"))
  (bind _inventorycomponent (`PlayerCharacter.InventoryComponent` fromPlayer))
  (bind _ammodroprate (`/Game/_DRGModding/_LesnovMods/GameplayMods/Mod_FullArmorBosco/BP_FABosco.AmmoDropRate` (`self.FABosco`)))
  (for _array_element (`|MakeArray` (`InventoryComponent.GetItem` _inventorycomponent "PrimaryWeapon") (`InventoryComponent.GetItem` _inventorycomponent "SecondaryWeapon") (`InventoryComponent.GetItem` _inventorycomponent "TraversalTool") (`InventoryComponent.GetItem` _inventorycomponent "ClassTool"))
    (if (`KismetMathLibrary.ClassIsChildOf` (`GameplayStatics.GetObjectClass` _array_element) "/Script/FSD.AmmoDrivenWeapon")
      (bind _asammo_driven_weapon (cast `AmmoDrivenWeapon` _array_element))
      (`/Game/_DRGModding/_Frameworks/BML_Framework.IncreaseAmmoByRate` _asammo_driven_weapon _ammodroprate)
      (`/Game/_DRGModding/_Frameworks/BML_Framework.IncreaseClipByRate` _asammo_driven_weapon _ammodroprate)
      (`/Game/_DRGModding/_Frameworks/BML_Framework.RefleshAmmoCounters` _asammo_driven_weapon))))

(fn `UserConstructionScript`
  (`parent.UserConstructionScript`))