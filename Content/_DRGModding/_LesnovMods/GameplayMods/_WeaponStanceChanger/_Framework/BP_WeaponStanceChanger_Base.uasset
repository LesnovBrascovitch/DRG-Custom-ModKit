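; Base Blueprint for a Deep Rock Galactic mod that toggles an alternate weapon stance on a key press while a matching weapon is equipped.
; First equip caches original animations and stats and assigns a replacement animation set as a loading workaround.
; Stance-in/out montages lead to animation and stat swaps, with empty hooks for child Blueprints.
; Reloading or unequipping restores defaults, while ledge-grab montages trigger reapplication of an active stance.
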(event `self.ReceiveBeginPlay`
  (bind _inventorycomponent (`PlayerCharacter.InventoryComponent` (`self.Player Character`)))
  ;[1 1 1] Begin Play - Obtain some variables and then bind event.
  (bind _fsdplayercontroller (`/Game/_DRGModding/_Frameworks/BML_Framework.GetLocalPlayerController(Macro)` true)
    (:`Completed`
      (bind _output_get (set `self.FSDPlayer Controller` _fsdplayercontroller))
      (`self.EnableInput` _output_get)
      (add `FSDPlayerController.OnPlayerCharacterPossesed` (`self.FSDPlayer Controller`) (delegate `OnPlayerCharacterPossesed_Event_0`))
      (bind _playercharacter (`/Game/_DRGModding/_Frameworks/BML_Framework.GetLocalPlayerCharacter(Macro)` true :!label _label)
        (:`Exec`
          (set `self.Player Character` _playercharacter)
          (set `self.FPAnimInstance` (`PlayerCharacter.GetFPAnimInstance` (`self.Player Character`)))
          (add `InventoryComponent.OnItemEquipped` _inventorycomponent (`|CreateDelegate` :!event `OnItemEquipped_Event_0`))
          (add `InventoryComponent.OnItemUnequipped` _inventorycomponent (`|CreateDelegate` :!event `OnItemUnequipped_Event_0`))
          (add `PlayerCharacter.OnSaluteEvent` (`self.Player Character`) (`|CreateDelegate` :!event `ResetStance`)))))))

(event `OnPlayerCharacterPossesed_Event_0`
  (params (Pawn :type "Pawn Object Reference"))
  ;[1 1 1] Begin Play - Obtain some variables and then bind event.
  (set `self.ObtainedWeaponInfos` false)
  (`|ExecutionSequence`
    (:`then_0`
      (goto _label))
    (:`then_1`
      (`self.ResetInitialization`))))

(event `OnItemEquipped_Event_0`
  (params (Item :type "Item Object Reference"))
  (bind _as_ammo_driven_weapon (`self.As Ammo Driven Weapon`))
  ;[1 1 1] On Item Equipped - Enable input and call activate stance event
  (`/Game/_DRGModding/_Frameworks/BML_Framework.CompareClass(Item)` Item (`self.ClassToActivateStance`)
    (:`Class Match`
      (`self.EnableInput` (`self.FSDPlayer Controller`))
      (bind _asammo_driven_weapon (cast `AmmoDrivenWeapon` Item))
      (bind _output_get (set `self.As Ammo Driven Weapon` _asammo_driven_weapon))
      (`self.OnReceiveAmmoDrivenWeapon` _output_get)
      (add `AnimInstance.OnMontageEnded` (`self.FPAnimInstance`) (`|CreateDelegate` :!event `OnMontageEnded_Event_0`))
      (`/Engine/EditorBlueprintResources/StandardMacros.DoOnce` false :!label _label_2
        (:`Completed`
          (`self.OnObtainRequiredVars` _as_ammo_driven_weapon)
          (set `AnimatedItem.CharacterAnimationSet` (`self.Character Animation Set`) _as_ammo_driven_weapon) ; New IAS is needed to be assigned. The dwarf's \nABP's anim set is not loaded if the same IAS is detected.\nThe fix is making new IAS and assign.
          (add `AmmoDrivenWeapon.OnReloadingEvent` (`self.As Ammo Driven Weapon`) (`|CreateDelegate` :!event `OnReloadingEvent_Event_1`))
          (set `self.ObtainedWeaponInfos` true))))))

(event `ResetInitialization`
  ;[1 1 1] On Item Equipped - Enable input and call activate stance event
  (goto _label_2 :!via `Reset`))

(event `OnItemUnequipped_Event_0`
  (params (Item :type "Item Object Reference"))
  ;[1 1 1] On Item Unequipped - Disable input and call reset stance event
  (`/Game/_DRGModding/_Frameworks/BML_Framework.CompareClass(Item)` Item (`self.ClassToActivateStance`)
    (:`Class Match`
      (`self.DisableInput` (`self.FSDPlayer Controller`))
      (`self.ResetStance`)
      (set `self.IsCowboyStance` false)
      (remove `AnimInstance.OnMontageEnded` (`self.FPAnimInstance`) (`|CreateDelegate` :!event `OnMontageEnded_Event_0`)))))

(event `InputAction|ChangeStance`
  (params (Key :type "Key Structure"))
  ;[1 1 1] ChangeStance Key - Toggle stance by checking if FP Idle is default or stance. Play stance in, out montage then call Activate Stance, Reset Stance events.
  (:`Pressed`
    (if (`self.ObtainedWeaponInfos`)
      (if (!= (`self.FP Idle`) (`PlayerFPAnimInstance.FP_Idle` (`PlayerCharacter.GetFPAnimInstance` (`self.Player Character`))))
        (`/Game/_DRGModding/_Frameworks/BML_Framework.PlayMontage(FPMesh)` (`self.Player Character`) (`self.Montage_StanceIn`)
          (:`On Blend Out`
            (`self.ActivateStance`)))
        (else
          (`/Game/_DRGModding/_Frameworks/BML_Framework.PlayMontage(FPMesh)` (`self.Player Character`) (`self.Montage_StanceOut`)
            (:`On Blend Out`
              (`self.ResetStance`))))))))

(event `OnMontageEnded_Event_0`
  (params (Montage :type "AnimMontage Object Reference") (bInterrupted :type Boolean))
  ;[1 1 1] On Montage Ended - Try to reactivate stance when ledge montage is played.
  ; Because when the ledge montage is occured, It re-load anim set from the default IAS.
  (if (== Montage "/Game/CharacterStructure/Gear_Unarmed/FP/1P_Unarmed_LedgeGrab_A_Montage.1P_Unarmed_LedgeGrab_A_Montage")
    (if (`self.IsCowboyStance`)
      (`self.ActivateStance`))))

(event `ActivateStance`
  ;[1 1 1] Activate Stance - Called from other events. Change animations and stats to new stance.
  (`/Game/_DRGModding/_Frameworks/BML_Framework.ChangeAnimation(FPMesh)` (`self.Player Character`) (`self.FP Idle`) (`self.FP Walk`) (`self.FP Sprint`) (`self.FP Jump Start`) (`self.FP Jump Loop`) (`self.FP Jump Land`) (`self.FP Jump Land Aim`))
  (`/Game/_DRGModding/_Frameworks/BML_Framework.UpdateAnims(AmmoDrivenWeapon)` (`self.As Ammo Driven Weapon`) (`self.Montage_Fire(FP)`) (`self.Montage_Reload(FP)`) (`self.Montage_Reload(WPN)`) (`self.Gunsling Animations`))
  (`self.ChangeWeaponStats` (`self.As Ammo Driven Weapon`))
  (bind (_isvalid _hitscan) (`self.GetHitscan`))
  (if _isvalid
    (`self.ChangeHitscanStats` _hitscan))
  (set `self.IsCowboyStance` true)
  (`self.OnStanceActivated`))

(event `OnReloadingEvent_Event_1`
  (bind _as_ammo_driven_weapon (`self.As Ammo Driven Weapon`))
  ;[1 1 1] Deactivate Stance - Called from other events. Reset animations and stats to the base.
  (`KismetSystemLibrary.Delay` 0.2)
  (`self.OnPreStanceDeactivated` :!label _label_3)
  (`/Game/_DRGModding/_Frameworks/BML_Framework.ResetAnimation(FPMesh)` (`self.Player Character`) _as_ammo_driven_weapon)
  (`/Game/_DRGModding/_Frameworks/BML_Framework.UpdateAnims(AmmoDrivenWeapon)` _as_ammo_driven_weapon (`self.FP Fire Animation(Cache)`) (`self.FP Reload Animation(Cache)`) (`self.WPN Reload(Cache)`) (`self.Gunsling Animations(Cache)`))
  (`self.ResetWeaponStats` (`self.As Ammo Driven Weapon`))
  (bind (_isvalid _hitscan) (`self.GetHitscan`))
  (if _isvalid
    (`self.ResetHitscanStats` _hitscan))
  (set `self.IsCowboyStance` false)
  (`self.OnStanceDeactivated`))

(event `ResetStance`
  ;[1 1 1] Deactivate Stance - Called from other events. Reset animations and stats to the base.
  (goto _label_3))

(event `OnStanceActivated`
  ;[1 1 1] Placeholder Events - Used within a child BP to expand logics.
)

(event `OnStanceDeactivated`
  ;[1 1 1] Placeholder Events - Used within a child BP to expand logics.
)

(event `OnPreStanceDeactivated`
  ;[1 1 1] Placeholder Events - Used within a child BP to expand logics.
)

(event `OnReceiveAmmoDrivenWeapon`
  (params (AmmoDrivenWeapon :type "AmmoDrivenWeapon Object Reference"))
  ;[1 1 1] Placeholder Events - Used within a child BP to expand logics.
)

(fn `AssignSpreadCurve`
  (params (Hitscan :type "HitscanBaseComponent Object Reference") (`Spread Curve` :type "RuntimeFloatCurve Structure"))
  (set `HitscanBaseComponent.SpreadCurve` `Spread Curve` Hitscan))

(fn `ChangeHitscanStats`
  (params (Hitscan :type "HitscanComponent Object Reference")))

(fn `ChangeWeaponStats`
  (params (AmmoDrivenWeapon :type "AmmoDrivenWeapon Object Reference")))

(fn `GetHitscan`
  (returns (IsValid :type Boolean) (Hitscan :type "HitscanComponent Object Reference"))
  (bind _hitscan (`self.Hitscan`))
  (return (`KismetSystemLibrary.IsValid` _hitscan) _hitscan))

(fn `OnObtainRequiredVars`
  (params (InputPin :type "AmmoDrivenWeapon Object Reference"))
  (bind (_fp_fire_animation_cache_ _fp_reload_animation_cache_ _wpn_reload_cache_ _gunsling_animations_cache_) (`/Game/_DRGModding/_Frameworks/BML_Framework.GetAnimVars(AmmoDrivenWeapon)` InputPin))
  (set `self.FP Fire Animation(Cache)` _fp_fire_animation_cache_)
  (set `self.FP Reload Animation(Cache)` _fp_reload_animation_cache_)
  (set `self.WPN Reload(Cache)` _wpn_reload_cache_)
  (set `self.Gunsling Animations(Cache)` _gunsling_animations_cache_)
  (set `self.Rate Of Fire(Cache)` (`AmmoDrivenWeapon.RateOfFire` InputPin))
  (set `self.Recoil Settings(Cache)` (`AmmoDrivenWeapon.RecoilSettings` InputPin))
  (bind _output_get (set `self.Hitscan` (`self.GetComponentByClass` InputPin "/Script/FSD.HitscanComponent")))
  (`/Engine/EditorBlueprintResources/StandardMacros.IsValid` _output_get
    (:`Is Valid`
      (set `self.Spread Curve(Cache)` (`HitscanBaseComponent.SpreadCurve` _output_get)))
    (:`Is Not Valid`
      _))
  (return))

(fn `ResetHitscanStats`
  (params (Hitscan :type "HitscanComponent Object Reference")))

(fn `ResetSpreadCurve`
  (params (Hitscan :type "HitscanBaseComponent Object Reference"))
  (set `HitscanBaseComponent.SpreadCurve` (`self.Spread Curve(Cache)`) Hitscan))

(fn `ResetWeaponStats`
  (params (AmmoDrivenWeapon :type "AmmoDrivenWeapon Object Reference"))
  (set `AmmoDrivenWeapon.RateOfFire` (`self.Rate Of Fire(Cache)`) AmmoDrivenWeapon)
  (set `AmmoDrivenWeapon.RecoilSettings` (`self.Recoil Settings(Cache)`) AmmoDrivenWeapon)
  (`self.ResetSpreadCurve` null))

(fn `UserConstructionScript`)