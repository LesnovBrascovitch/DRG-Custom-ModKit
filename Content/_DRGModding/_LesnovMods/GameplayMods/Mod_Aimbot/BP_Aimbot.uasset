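; Deep Rock Galactic mod actor providing a toggleable aimbot, zeroed weapon recoil and see-through collectible markers.
; Once player references resolve, Tick sphere-overlaps enemies around the camera trace hit, then interpolates rotation toward visible per-class weakpoint sockets, retaining the last valid target.
; Aiming pauses while running or on empty clips, and item equips switch it automatically.
; A hub slider saves aim speed; multiplayer-detection and enemy-proximity timers are unwired.
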(event `self.ReceiveBeginPlay`
  (bind _returnvalue (`KismetSystemLibrary.K2_SetTimerDelegate` (delegate `Event Initialization`) 1.0 true)))

(event `self.ReceiveTick`
  (params (DeltaSeconds :type "Float (single-precision)"))
  (bind _lastvalidpawn (`self.LastValidPawn`))
  ;[1 1 1] Aimbot
  (if (`self.DetectedHack`)
    _
    (elif (not (`self.IsRunning`))
      (set `self.IsRunning` true)
      (set `self.PlayerCameraLocation` (`SceneComponent.K2_GetComponentLocation` (`self.PlayerCameraComp`)))
      (if (or (`PlayerCharacter.IsRunning` (`self.PlayerCharacter`)) (`self.IsRunKeyDown`))
        (`self.ResetAimbot`)
        (else
          (`/Engine/EditorBlueprintResources/StandardMacros.IsValid` _lastvalidpawn
            (:`Is Valid`
              (bind _issucess (`self.Aimbot` _lastvalidpawn))
              (if (not _issucess)
                (set `self.LastValidPawn` null)
                (bind (_bblockinghit _location) (`self.InitialLineTrace` :!label _label))
                (if _bblockinghit
                  (bind (_outactors _returnvalue) (`KismetSystemLibrary.SphereOverlapActors` _location (`self.Sphere Radius`) (`self.Object Types`) "/Script/FSD.EnemyDeepPathfinderCharacter"))
                  (if _returnvalue
                    (for _array_element _outactors
                      (bind _issucess_2 (`self.Aimbot` _array_element))
                      (if _issucess_2
                        (break)))))))
            (:`Is Not Valid`
              (goto _label)))))
      (`self.ExecuteFinish`))))

(event `Event Initialization`
  (bind _playercharacter (`/Game/_DRGModding/_Frameworks/BML_Framework.GetLocalPlayerCharacter(Macro - GameInstance)`))
  (`KismetSystemLibrary.PrintString` (`KismetStringLibrary.Concat_StrStr` (`KismetSystemLibrary.GetDisplayName` self) " - " "Getting Required Refs"))
  (`/Engine/EditorBlueprintResources/StandardMacros.IsValid` (`self.Menu_Aimbot`)
    (:`Is Valid`
      _)
    (:`Is Not Valid`
      (bind _returnvalue (`|CreateWidget` "/Game/_DRGModding/_LesnovMods/GameplayMods/Mod_Aimbot/Menu_Aimbot.Menu_Aimbot_C"))
      (set `self.Menu_Aimbot` _returnvalue)))
  (`/Engine/EditorBlueprintResources/StandardMacros.IsValid` _playercharacter
    (:`Is Valid`
      (set `self.PlayerCharacter` _playercharacter)
      (set `self.PlayerCameraComp` (`PlayerCharacter.FirstPersonCamera` _playercharacter))
      (set `self.Inventory Component` (`PlayerCharacter.InventoryComponent` _playercharacter))
      (set `self.PlayerController` (`/Game/_DRGModding/_Frameworks/BML_Framework.GetLocalPlayerController(Macro - GameInstance)_0`))
      (`/Game/_DRGModding/_Frameworks/BML_Framework.IsInDRG`
        (:`In DRG`
          (if (and (`KismetSystemLibrary.IsValid` (`self.PlayerCharacter`)) (`KismetSystemLibrary.IsValid` (`self.PlayerCameraComp`)) (`KismetSystemLibrary.IsValid` (`self.PlayerController`)) (`KismetSystemLibrary.IsValid` (`self.Inventory Component`)) (`KismetSystemLibrary.IsValid` (`self.Menu_Aimbot`)))
            (bind _outputpin (`/Game/_DRGModding/_Frameworks/BML_Framework.HandleSaveGame` "/Game/_DRGModding/_LesnovMods/GameplayMods/Mod_Aimbot/AimbotSavegame.AimbotSavegame_C" :!label _label_2)
              (:`then`
                (bind _asaimbot_savegame (cast `/Game/_DRGModding/_LesnovMods/GameplayMods/Mod_Aimbot/AimbotSavegame` _outputpin))
                (set `self.As Aimbot Savegame` _asaimbot_savegame)
                (bind _returnvalue_2 (`|CreateWidget` "/Game/_DRGModding/_LesnovMods/GameplayMods/Mod_Aimbot/HUBMENU_Aimbot.HUBMENU_Aimbot_C"))
                (bind _output_get (set `self.HUBMENU` _returnvalue_2))
                (bind _cui_slider (`/Game/_DRGModding/_LesnovMods/GameplayMods/Mod_Aimbot/HUBMENU_Aimbot.CUI_Slider` _output_get))
                (add `/Game/_DRGModding/_Frameworks/Widget/CUI_Slider.OnSliderValueChanged` _cui_slider (delegate `OnSliderValueChanged_Event_0`))
                (`/Game/_DRGModding/_Frameworks/Widget/CUI_Slider.Initialize` _cui_slider (`/Game/_DRGModding/_LesnovMods/GameplayMods/Mod_Aimbot/AimbotSavegame.AimTransitionRate` (`self.As Aimbot Savegame`)))
                (`KismetSystemLibrary.K2_ClearAndInvalidateTimerHandle` (stale `self.ReceiveBeginPlay` _returnvalue))
                (`self.Event BeginModdingLogic`)))))
        (:`In Editor`
          (goto _label_2))))))

(event `OnSliderValueChanged_Event_0`
  (params (Value :type "Float (double-precision)"))
  (bind _as_aimbot_savegame (`self.As Aimbot Savegame`))
  (set `/Game/_DRGModding/_LesnovMods/GameplayMods/Mod_Aimbot/AimbotSavegame.AimTransitionRate` Value _as_aimbot_savegame)
  (`/Game/_DRGModding/_Frameworks/BML_Framework.SaveToSlot(Macro)` _as_aimbot_savegame))

(event `Key|LeftAlt` :consume false
  (params (Key :type "Key Structure"))
  ;[1 1 1] Toggle Aimbot
  (:`Pressed`
    (`self.Toggle Aimbot` (not (`self.IsActorTickEnabled`)))))

(event `Event BeginModdingLogic`
  (for _array_element (`InputSettings.GetActionMappingByName` (`InputSettings.GetInputSettings`) "Run")
    (`KismetArrayLibrary.Array_AddUnique` (`self.Key`) (`.Key` (break `InputActionKeyMapping` _array_element))))
  (`UserWidget.AddToViewport` (`self.Menu_Aimbot`) 0)
  (`self.SetActorTickEnabled` true)
  (`self.EnableInput` (`self.PlayerController`))
  (`|ExecutionSequence`
    (:`then_0`
      (add `InventoryComponent.OnItemEquipped` (`self.Inventory Component`) (delegate `OnItemEquipped_Event_0`)))
    (:`then_2`
      (for _array_element_2 (`InventoryBase.GetAllItems` (`self.Inventory Component`))
        (bind _asammo_driven_weapon (cast `AmmoDrivenWeapon` _array_element_2))
        (set `AmmoDrivenWeapon.RecoilSettings` (make `RecoilSettings` (make `RandRange` 0.0) (make `RandRange` 0.0) (make `RandRange` 0.0)) _asammo_driven_weapon)))))

(event `OnItemEquipped_Event_0`
  (params (Item :type "Item Object Reference"))
  (bind _returnvalue (`GameplayStatics.GetObjectClass` Item))
  (if (`KismetMathLibrary.ClassIsChildOf` _returnvalue "/Script/FSD.ThrownGrenadeItem")
    (`self.Toggle Aimbot` false)
    (else
      (`self.Toggle Aimbot` (not (`BlueprintSetLibrary.Set_Contains` (`self.SupportItems`) _returnvalue))))))

(event `ExecuteEnemyNear`
  (bind _sphereradiusnearenemy (`self.SphereRadiusNearEnemy`))
  (bind _returnvalue (`self.K2_GetActorLocation` (`self.PlayerCharacter`)))
  ;[1 1 1] Disabled For Now
  (bind _outactors (`KismetSystemLibrary.SphereOverlapActors` _returnvalue _sphereradiusnearenemy (`self.Object Types`) "/Script/FSD.EnemyDeepPathfinderCharacter"))
  (`KismetSystemLibrary.DrawDebugSphere` _returnvalue _sphereradiusnearenemy 12 (struct :`R` 1.0 :`B` 0.910864 :`A` 1.0) (`self.Time`) 1.0)
  (if (!= (`KismetArrayLibrary.Array_Length` _outactors) 0)
    (for _array_element _outactors
      (bind _asenemy_deep_pathfinder_character (cast `EnemyDeepPathfinderCharacter` _array_element))
      (if (not (`HealthComponentBase.IsDead` (`EnemyDeepPathfinderCharacter.HealthComponent` _asenemy_deep_pathfinder_character)))
        (set `self.IsEnemyNear` true)
        (break)))
    (else
      (set `self.IsEnemyNear` false))))

(event `CustomEvent_3`
  ;[1 1 1] Disable based on condition to prevent hack
  (bind _outactors (`GameplayStatics.GetAllActorsOfClass` "/Script/FSD.PlayerCharacter"))
  (for _array_element _outactors
    (if (`KismetMathLibrary.ClassIsChildOf` (`GameplayStatics.GetObjectClass` _array_element) "/Game/Character/BP_Bosco_Character.BP_Bosco_Character_C")
      (set `self.DetectedHack` false :!label _label_3)
      (elif (`Pawn.IsLocallyControlled` _array_element)
        (goto _label_3)
        (else
          (set `self.DetectedHack` true)))))
  (`Widget.SetVisibility` (`/Game/_DRGModding/_LesnovMods/GameplayMods/Mod_Aimbot/Menu_Aimbot.TextBlock_Warning` (`self.Menu_Aimbot`)) (select `bool` (`self.DetectedHack`) :`false` "Collapsed" :`true` "SelfHitTestInvisible" :!type "ESlateVisibility Enum")))

(event `Key|LeftControl`
  (params (Key :type "Key Structure"))
  ;[1 1 1] Left Ctrl - Get Pickable Locations
  (:`Pressed`
    (`/Engine/EditorBlueprintResources/StandardMacros.FlipFlop`
      (:`A`
        (`self.CustomEvent_2`)
        (bind _returnvalue (`KismetSystemLibrary.K2_SetTimerDelegate` (delegate `CustomEvent_2`) 5.0 true)))
      (:`B`
        (`self.DestroyVisualisers`)
        (`KismetSystemLibrary.K2_ClearAndInvalidateTimerHandle` _returnvalue)))))

(event `CustomEvent_2`
  ;[1 1 1] Left Ctrl - Get Pickable Locations
  (`/Engine/EditorBlueprintResources/StandardMacros.DoOnce` false :!label _label_4
    (:`Completed`
      (`self.DestroyVisualisers`)
      (bind _outactors (`GameplayStatics.GetAllActorsOfClass` "/Game/GameElements/Resources/Collectibles/BP_Collectible_Base.BP_Collectible_Base_C"))
      (for _array_element _outactors
        (if (`InstantUsable.Usable` (`/Game/GameElements/Resources/Collectibles/BP_Collectible_Base.InstantUsable` _array_element))
          (bind _returnvalue (`|SpawnActorFromClass` "/Game/_DRGModding/_LesnovMods/GameplayMods/Mod_Aimbot/Assets/BP_SeeThroughObj.BP_SeeThroughObj_C" (`KismetMathLibrary.MakeTransform` (`self.K2_GetActorLocation` _array_element)) "AlwaysSpawn" "OverrideRootScale" null null))
          (`KismetArrayLibrary.Array_Add` (`self.NewVar_0`) _returnvalue)))
      (`self.Reset`))))

(event `Reset`
  ;[1 1 1] Left Ctrl - Get Pickable Locations
  (goto _label_4 :!via `Reset`))

(fn `Aimbot`
  (params (TargetActor :type "Actor Object Reference"))
  (returns (IsSucess :type Boolean))
  (locals (Local_IsSuccess :type Boolean :default false))
  (if (or (`self.Is In Ignore Classes(Enemy)` TargetActor) (`self.Is In IgnoreGameplayTag` TargetActor))
    (set `local.Local_IsSuccess` false :!label _label)
    (elif (`self.Is Weapon Clip Empty`)
      (goto _label)
      (else
        (bind _asenemy_deep_pathfinder_character (cast `EnemyDeepPathfinderCharacter` TargetActor))
        (if (`HealthComponentBase.IsDead` (`EnemyDeepPathfinderCharacter.HealthComponent` _asenemy_deep_pathfinder_character))
          (goto _label)
          (else
            (set `self.Mesh` (`DeepPathfinderCharacter.Mesh` _asenemy_deep_pathfinder_character))
            (`self.GetSocketLocation` (`self.GetWeakpointSocketName` TargetActor) TargetActor)
            (if (`self.CanTargetActorAimed` TargetActor)
              (set `self.LastValidPawn` TargetActor)
              (`self.SetControlRotation`)
              (`self.SetCameraRotation`)
              (set `local.Local_IsSuccess` true)
              (else
                (goto _label))))))))
  (return (`local.Local_IsSuccess`)))

(fn `CanTargetActorAimed`
  (params (CompareActor :type "Object Object Reference"))
  (returns (Condition :type Boolean))
  (bind _outhit (`KismetSystemLibrary.LineTraceSingle` (`self.PlayerCameraLocation`) (`self.TargetActorLocation`) "TraceTypeQuery3" false (`|MakeArray` (`self.PlayerCharacter`) :!type "Actor Object Reference") "ForOneFrame" true (struct :`G` 0.089913 :`B` 1.0 :`A` 1.0)))
  (bind (_bblockinghit _binitialoverlap _time _distance _location _impactpoint _normal _impactnormal _physmat _hitactor _hitcomponent _hitbonename) (`GameplayStatics.BreakHitResult` _outhit))
  (return (and (== CompareActor _hitactor) (select `bool` (`self.ConstraintBone`) :`false` true :`true` (== _hitbonename (`self.WeakpointSocketName`))))))

(fn `DestroyAimbot`
  (`self.Toggle Aimbot` false)
  (`self.K2_DestroyActor`))

(fn `DestroyVisualisers`
  (bind _newvar_0 (`self.NewVar_0`))
  (for _array_element _newvar_0
    (`/Engine/EditorBlueprintResources/StandardMacros.IsValid` _array_element
      (:`Is Valid`
        (`self.K2_DestroyActor` _array_element))))
  (`KismetArrayLibrary.Array_Clear` _newvar_0))

(fn `ExecuteFinish`
  (set `self.IsRunning` false))

(fn `GetModInfo`
  (returns (ModName :type Text) (ModAuthor :type Text) (ModVersion :type Text))
  (return "Aimbot" "Lesnov" "1.0.0"))

(fn `GetModPages`
  (returns (HubPages :type "Array of /Game/_ModHub/IHubPageWidget Interface"))
  (return (`|MakeArray` (`self.HUBMENU`) :!type "/Game/_ModHub/IHubPageWidget Interface")))

(fn `GetSocketLocation`
  (params (InSocketName :type Name) (Target :type "Actor Object Reference"))
  (bind _mesh (`self.Mesh`))
  (set `self.IsSocketValid` (`SceneComponent.DoesSocketExist` _mesh InSocketName))
  (set `self.TargetActorLocation` (select `bool` (`self.IsSocketValid`) :`false` (`self.K2_GetActorLocation` Target) :`true` (`SceneComponent.GetSocketLocation` _mesh InSocketName))))

(fn `GetWeakpointSocketName`
  (params (Actor :type "Actor Object Reference"))
  (returns (WeakpointSocketName :type Name))
  (`self.GetSocketNameByClass` Actor "/Game/Enemies/FlyingBug/Shooter/ENE_Mactera_Shooter_Base.ENE_Mactera_Shooter_Base_C" "ShooterBug_WeakPoint"
    (:`True`
      _)
    (:`False`
      (`self.GetSocketNameByClass` Actor "/Script/FSD.FlyingLifter" "GrabberBug_WeakSpot"
        (:`True`
          _)
        (:`False`
          (`self.GetSocketNameByClass` Actor "/Game/Enemies/Spider/Buffer/ENE_Spider_Buffer.ENE_Spider_Buffer_C" "Warden_Weakspot"
            (:`True`
              _)
            (:`False`
              (`self.GetSocketNameByClass` Actor "/Game/Enemies/Spider/Tank/ENE_Spider_Tank_Generic.ENE_Spider_Tank_Generic_C" "Spider_Back"
                (:`True`
                  _)
                (:`False`
                  (`self.GetSocketNameByClass` Actor "/Game/Enemies/RivalTech/PatrolBot/ENE_PatrolBot.ENE_PatrolBot_C" "Head"
                    (:`True`
                      _)
                    (:`False`
                      (set `self.WeakpointSocketName` "Spider_Head")))))))))))
  (return (`self.WeakpointSocketName`)))

(fn `InitialLineTrace`
  (returns (bBlockingHit :type Boolean) (Location :type "Vector Structure"))
  (bind _playercameralocation (`self.PlayerCameraLocation`))
  (bind _outhit (`KismetSystemLibrary.LineTraceSingle` _playercameralocation (+ _playercameralocation (* (`SceneComponent.GetForwardVector` (`self.PlayerCameraComp`)) 30000.0)) "TraceTypeQuery3" false (`|MakeArray` (`self.PlayerCharacter`) :!type "Actor Object Reference") "ForOneFrame"))
  (bind (_bblockinghit _binitialoverlap _time _distance _location) (`GameplayStatics.BreakHitResult` _outhit))
  (`KismetSystemLibrary.PrintString` (`KismetStringLibrary.Conv_DoubleToString` _distance) true true (struct :`G` 0.66 :`B` 1.0 :`A` 1.0) 0.0)
  (return (and _bblockinghit (select `bool` (`self.IsEnemyNear`) :`false` true :`true` (< _distance (`self.SphereRadiusNearEnemy`)))) _location))

(fn `Is In Ignore Classes(Enemy)`
  (params (Actor :type "Actor Object Reference"))
  (returns (Condition :type Boolean))
  (return (`BlueprintSetLibrary.Set_Contains` (`self.IgnoreActorClasses`) (`GameplayStatics.GetObjectClass` Actor))))

(fn `Is In IgnoreGameplayTag`
  (params (Actor :type "Actor Object Reference"))
  (returns (Condition :type Boolean))
  (locals (Local_Condition :type Boolean :default true))
  (if (`KismetSystemLibrary.IsPackagedForDistribution`)
    (bind _tagcontainer (message `GameplayTagAssetInterface.GetOwnedGameplayTags` Actor))
    (set `local.Local_Condition` (`BlueprintGameplayTagLibrary.HasTag` _tagcontainer (struct :`TagName` "Attitude.Friendly")))
    (else
      (set `local.Local_Condition` false)))
  (return (`local.Local_Condition`)))

(fn `Is Weapon Clip Empty`
  (returns (NewParam :type Boolean))
  (bind _returnvalue (`InventoryComponent.GetEquippedItem` (`self.Inventory Component`)))
  (if (`KismetSystemLibrary.IsPackagedForDistribution`)
    (if (`KismetMathLibrary.ClassIsChildOf` (`GameplayStatics.GetObjectClass` _returnvalue) "/Script/FSD.AmmoDrivenWeapon")
      (bind _asammo_driven_weapon (cast `AmmoDrivenWeapon` _returnvalue)
        (:`then`
          (return (== (`AmmoDrivenWeapon.ClipCount` _asammo_driven_weapon) 0)))
        (:`CastFailed`
          _)))
    (return true)
    (else
      (return false))))

(fn `IsRunKeyDown`
  (returns (ReturnValue :type Boolean))
  (locals (IsKeyDown :type Boolean :default false))
  (for _array_element (`self.Key`)
    (if (`PlayerController.IsInputKeyDown` (`self.PlayerController`) _array_element)
      (set `local.IsKeyDown` true)
      (break)))
  (return (`local.IsKeyDown`)))

(fn `ResetAimbot`
  (set `self.LastValidPawn` null)
  (`self.ResetCameraRotation`))

(fn `ResetCameraRotation`
  (`SceneComponent.K2_SetWorldRotation` (`self.PlayerCameraComp`) (`KismetMathLibrary.MakeRotator` (.roll (`Controller.GetControlRotation` (`self.PlayerController`))) (.pitch (`Controller.GetControlRotation` (`self.PlayerController`))) (.yaw (`Controller.GetControlRotation` (`self.PlayerController`)))) false false))

(fn `SetCameraRotation`)

(fn `SetControlRotation`
  (bind (_returnvalue_roll _returnvalue_pitch _returnvalue_yaw) (`KismetMathLibrary.BreakRotator` (`KismetMathLibrary.RInterpTo_Constant` (`Controller.GetControlRotation` (`self.PlayerController`)) (`KismetMathLibrary.FindLookAtRotation` (`SceneComponent.K2_GetComponentLocation` (`self.PlayerCameraComp`)) (`self.TargetActorLocation`)) (`GameplayStatics.GetGlobalTimeDilation`) (* 2 (`/Game/_DRGModding/_LesnovMods/GameplayMods/Mod_Aimbot/AimbotSavegame.AimTransitionRate` (`self.As Aimbot Savegame`))))))
  (`Controller.SetControlRotation` (`self.PlayerController`) (`KismetMathLibrary.MakeRotator` 0.0 _returnvalue_pitch _returnvalue_yaw))
  (`SceneComponent.K2_SetWorldRotation` (`self.PlayerCameraComp`) (`KismetMathLibrary.MakeRotator` 0.0 _returnvalue_pitch _returnvalue_yaw) false false))

(fn `Toggle Aimbot`
  (params (bEnabled :type Boolean))
  (`self.SetActorTickEnabled` bEnabled)
  (`/Game/_DRGModding/_LesnovMods/GameplayMods/Mod_Aimbot/Option_Aimbot.OnAimbotChanged` (`/Game/_DRGModding/_LesnovMods/GameplayMods/Mod_Aimbot/Menu_Aimbot.Option_Aimbot` (`self.Menu_Aimbot`)) bEnabled)
  (if (not bEnabled)
    (`self.ResetAimbot`)
    (set `self.IsRunning` false)))

(fn `UserConstructionScript`)