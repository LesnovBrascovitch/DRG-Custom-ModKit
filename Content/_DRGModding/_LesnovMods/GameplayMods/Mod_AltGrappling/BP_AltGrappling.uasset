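; Alternate grappling hook mod for Deep Rock Galactic, attached to the local player's first-person camera and driven by the Grenade input.
; Holding arms a looping timer, apparently for the colour-coded trace preview; releasing on a hit launches a timeline-driven projectile and cable.
; Once it lands, Tick applies a capped rope-like force along the anchor line while falling below it, producing a swing.
; Chat commands tune force parameters; debug prints and unused experiments remain.
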(event `OnNewMessage`
  (params (Message :type "FSDChatMessage Structure (by ref)"))
  (bind _msg (`/Game/_DRGModding/_Frameworks/BML_Framework.IgnoreMsgBySender` Message (`self.Player Character`))
    (:`CanProceed`
      (set `self.ConsoleCommands` (`KismetStringLibrary.ParseIntoArray` _msg))
      (switch `string` (`|GetArrayItem` (`self.ConsoleCommands`))
        (:`ST`
          (bind _output_get (set `self.NewVar_0` (`KismetStringLibrary.Conv_StringToDouble` (`|GetArrayItem` (`self.ConsoleCommands`) 1))))
          (bind _returnvalue (`KismetStringLibrary.Conv_DoubleToString` _output_get))
          (`/Game/_DRGModding/_Frameworks/BML_Framework.PrintViaChat` false _returnvalue _returnvalue))
        (:`MAX`
          (bind _output_get_2 (set `self.Max` (`KismetStringLibrary.Conv_StringToDouble` (`|GetArrayItem` (`self.ConsoleCommands`) 1))))
          (bind _returnvalue_2 (`KismetStringLibrary.Conv_DoubleToString` _output_get_2))
          (`/Game/_DRGModding/_Frameworks/BML_Framework.PrintViaChat` false _returnvalue_2 _returnvalue_2))))))

(event `self.ReceiveBeginPlay`
  (bind _root (`self.Root`))
  (bind _fsdplayercontroller (`/Game/_DRGModding/_Frameworks/BML_Framework.GetLocalPlayerController(Macro)` true)
    (:`Completed`
      (bind _output_get (set `self.FSDPlayer Controller` _fsdplayercontroller))
      (`self.EnableInput` _output_get)
      (bind _playercharacter (`/Game/_DRGModding/_Frameworks/BML_Framework.GetLocalPlayerCharacter(Macro)` true)
        (:`Exec`
          (bind _output_get_2 (set `self.Player Character` _playercharacter))
          (`SceneComponent.K2_AttachToComponent` _root (`PlayerCharacter.FirstPersonCamera` _output_get_2) "None" "SnapToTarget" "SnapToTarget" "SnapToTarget" true)
          (`SceneComponent.K2_SetRelativeLocation` _root (16.0 0.0 14.0) false false)
          (`CableComponent.SetAttachEndToComponent` (`self.Cable`) (`self.Projectile`) "None")
          (`CableComponent.SetAttachEndToComponent` (`self.Cable1`) (`self.Projectile1`) "None")
          (`self.ToggleVisibillity(PRJMesh)` false)
          (add `MessagingSubSystem.OnNewMessage` (subsystem `MessagingSubSystem`) (delegate `OnNewMessage`))
          (`SceneComponent.SetHiddenInGame` (`self.Cable1`) true false)
          (`SceneComponent.SetHiddenInGame` (`self.Projectile1`) true false))))))

(event `CustomEvent_1`
  (set `self.IsHookActivated` true)
  (bind _returnvalue (`KismetSystemLibrary.K2_SetTimerDelegate` (`|CreateDelegate` :!event `PreCheckHook`) 0.05 true))
  (set `self.NewVar_4` _returnvalue))

(event `InputAction|Grenade`
  (params (Key :type "Key Structure"))
  (:`Pressed`
    (set `self.IsHookActivated` false)
    (bind _returnvalue (`KismetSystemLibrary.K2_SetTimerDelegate` (delegate `CustomEvent_1`) 0.17))
    (set `self.NewVar_7` _returnvalue))
  (:`Released`
    (`SceneComponent.SetHiddenInGame` (`self.Cable1`) true false)
    (`SceneComponent.SetHiddenInGame` (`self.Projectile1`) true false)
    (`KismetSystemLibrary.K2_ClearAndInvalidateTimerHandle` (`self.NewVar_7`))
    (`KismetSystemLibrary.K2_ClearAndInvalidateTimerHandle` (`self.NewVar_4`))
    (if (`self.IsHookActivated`)
      (`self.RevertPostionHookStop`)
      (if (`self.IsHit`)
        (set `self.IsGrap` true)
        (`self.SetActorEnableCollision` false)
        (bind _location (`/Game/_DRGModding/_Frameworks/BML_Framework.QuickLinetrace` (`self.Player Character`))
          (:`OnHit`
            (set `self.Location` _location)
            (`self.StartWindUp`)
            (`self.PlaySound(Fire)`)
            (`self.PlayEffect(Muzzle)`)
            (`self.ActivateEffect(Thruster)`))))
      (else
        (set `self.IsGrap` false)
        (`self.SetActorTickEnabled` false)
        (`self.ReverseWindUp`)
        (`self.RevertPostionHook`)))))

(event `self.ReceiveTick`
  (params (DeltaSeconds :type "Float (single-precision)"))
  (bind (_location_x _location_y _location_z) (`KismetMathLibrary.BreakVector` (`self.Location`)))
  (bind (_location_x_2 _location_y_2 _location_z_2) (`KismetMathLibrary.BreakVector` (`self.Location`)))
  (bind (_returnvalue_x _returnvalue_y _returnvalue_z) (`KismetMathLibrary.BreakVector` (`self.K2_GetActorLocation` (`self.Player Character`))))
  (bind (_returnvalue_x_2 _returnvalue_y_2 _returnvalue_z_2) (`KismetMathLibrary.BreakVector` (`self.K2_GetActorLocation` (`self.Player Character`))))
  (bind _charactermovement (`Character.CharacterMovement` (`self.Player Character`)))
  (bind _returnvalue (- (`self.K2_GetActorLocation` (`self.Player Character`)) (`self.Location`)))
  (bind _returnvalue_2 (* (* (* (`KismetMathLibrary.Normal` _returnvalue) (`KismetMathLibrary.Dot_VectorVector` (`self.GetVelocity` (`self.Player Character`)) _returnvalue)) -3.0) (`self.NewVar_0`)))
  (if (`NavMovementComponent.IsFalling` (`Character.CharacterMovement` (`self.Player Character`)))
    (if (== (`self.NewVar_0`) 0.0)
      _
      (elif (> (- _location_z _returnvalue_z) 0.0)
        (`KismetSystemLibrary.PrintString` (`KismetStringLibrary.Conv_DoubleToString` (- _location_z_2 _returnvalue_z_2)))
        (if (< (`KismetMathLibrary.VSize` _returnvalue_2) (* (`self.NewVar_8`) (`self.NewVar_0`)))
          (`CharacterMovementComponent.AddForce` _charactermovement _returnvalue_2)
          (`self.UpdateRotation`)
          (set `self.NewVar_2` _returnvalue_2)
          (else
            (`CharacterMovementComponent.AddForce` _charactermovement (`KismetMathLibrary.Vector_ClampSizeMax` _returnvalue_2 839999.0))
            (`self.UpdateRotation`)))))))

(event `ReverseWindUp`
  (`self.SetProjectileSpeed` (`self.ProjectileSpeedPull`))
  (bind (_direction _alpha) (`Timeline|TL_Projectile` :!via `Reverse` :!label _label)
    (:`Update`
      (`SceneComponent.K2_SetWorldLocation` (`self.ProjectileRoot`) (`KismetMathLibrary.VLerp` (`self.Origin`) (`self.Location`) _alpha) false false))
    (:`Finished`
      (switch `ETimelineDirection` _direction
        (:`Forward`
          (`self.SetActorTickEnabled` true))
        (:`Backward`
          (`self.ToggleVisibillity(PRJMesh)` false)
          (`AudioComponent.Stop` (`self.MovingSound`)))))))

(event `StartWindUp`
  (set `self.NewVar_1` 1.0)
  (`AudioComponent.Play` (`self.MovingSound`) 0.0)
  (`self.SetProjectileSpeed` (`self.ProjectileSpeedLaunch`))
  (set `self.RotationForward` (`SceneComponent.K2_GetComponentRotation` (`self.Muzzle`)))
  (set `self.Origin` (`SceneComponent.GetSocketLocation` (`self.FPMesh`) "Muzzle"))
  (`self.ToggleVisibillity(PRJMesh)` true)
  (`SceneComponent.K2_SetWorldRotation` (`self.ProjectileRoot`) (`self.RotationForward`) false false)
  (goto _label :!via `PlayFromStart`))

(event `RevertPostionHook`
  (set `self.Relative Rotation` (`SceneComponent.RelativeRotation` (`self.Root`)))
  (bind (_direction _alpha) (`Timeline|Timeline_1` :!via `PlayFromStart` :!label _label_2)
    (:`Update`
      (`SceneComponent.K2_SetRelativeRotation` (`self.Root`) (`KismetMathLibrary.RLerp` (`self.Relative Rotation`) (struct) _alpha true) false false))))

(event `RevertPostionHookStop`
  (goto _label_2 :!via `Stop`))

(fn `ActivateEffect(Thruster)`
  (`ActorComponent.Activate` (`self.ParticleSystem`) true))

(fn `PlayEffect(Muzzle)`
  (`GameplayStatics.SpawnEmitterAttached` "/Game/WeaponsNTools/GrapplingGun/P_GrapplingGun_Muzzle.P_GrapplingGun_Muzzle" (`self.Muzzle`) "None" (0.0 0.0 0.0) (struct) (1.0 1.0 1.0) "SnapToTargetIncludingScale"))

(fn `PlaySound(Fire)`
  (`GameplayStatics.SpawnSoundAttached` "/Game/Audio/SFX/WeaponsNTools/WPN_GraplingGun/GrapplingGunFire_Cue.GrapplingGunFire_Cue" (`self.FPMesh`) "None" (0.0 0.0 0.0) (struct) "KeepRelativeOffset" false 1.0 1.0 0.0 null null))

(fn `PreCheckHook`
  (locals (Local_EndLocation :type "Vector Structure"))
  (bind _player_character (`self.Player Character`))
  (bind (_start _end) (`/Game/_DRGModding/_Frameworks/BML_Framework.GetLinetracePos` (`PlayerCharacter.FirstPersonCamera` _player_character) 3000))
  (`SceneComponent.SetHiddenInGame` (`self.Cable1`) false false)
  (`SceneComponent.SetHiddenInGame` (`self.Projectile1`) false false)
  (`SceneComponent.K2_SetWorldRotation` (`self.ProjectileRoot`) (`SceneComponent.K2_GetComponentRotation` (`self.Muzzle`)) false false)
  (set `local.Local_EndLocation` _end)
  (bind (_outhit _returnvalue) (`KismetSystemLibrary.LineTraceSingle` _start _end "TraceTypeQuery3" false (`|MakeArray` _player_character :!type "Actor Object Reference")))
  (set `self.IsHit` _returnvalue)
  (`SceneComponent.K2_SetWorldLocation` (`self.ProjectileRoot1`) (`KismetMathLibrary.SelectVector` (`.Location` (`GameplayStatics.BreakHitResult` _outhit)) (`local.Local_EndLocation`) (`self.IsHit`)) false false)
  (`self.SetPreviewColor` (`self.IsHit`)))

(fn `SetPreviewColor`
  (params (CanHook :type Boolean))
  (`MaterialInstanceDynamic.SetVectorParameterValue` (`self.DMI`) "Color" (`KismetMathLibrary.SelectColor` (struct :`G` 0.876673 :`B` 1.0 :`A` 1.0) (struct :`R` 1.0 :`G` 0.006452 :`A` 1.0) CanHook)))

(fn `SetProjectileSpeed`
  (params (ProjectileSpeed :type "Float (double-precision)"))
  (`TimelineComponent.SetPlayRate` (`self.TL_Projectile`) (`KismetMathLibrary.SafeDivide` 1.0 ProjectileSpeed)))

(fn `ToggleVisibillity(PRJMesh)`
  (params (Show :type Boolean))
  (`SceneComponent.SetVisibility` (`self.Projectile`) (select `bool` Show :`true` true) false)
  (`SceneComponent.SetVisibility` (`self.Cable`) (select `bool` Show :`true` true) false))

(fn `UpdateRotation`
  (bind _root (`self.Root`))
  (bind (_relativerotation_roll _relativerotation_pitch _relativerotation_yaw) (`KismetMathLibrary.BreakRotator` (`SceneComponent.RelativeRotation` _root)))
  (bind (_returnvalue_roll _returnvalue_pitch) (`KismetMathLibrary.BreakRotator` (`KismetMathLibrary.FindLookAtRotation` (`SceneComponent.K2_GetComponentLocation` _root) (`self.Location`))))
  (`SceneComponent.K2_SetRelativeRotation` (`self.Root`) (`KismetMathLibrary.MakeRotator` _relativerotation_roll (`KismetMathLibrary.ClampAngle` (`KismetMathLibrary.FInterpTo` _relativerotation_pitch _returnvalue_pitch (`GameplayStatics.GetWorldDeltaSeconds`) 2.0) (`self.Min Angle Degrees`) (`self.Max Angle Degrees`)) _relativerotation_yaw) false false))

(fn `UserConstructionScript`
  (bind _returnvalue (`KismetMaterialLibrary.CreateDynamicMaterialInstance` "/Game/_DRGModding/_LesnovMods/GameplayMods/Mod_AltGrappling/M_AmmoDrop_Inst.M_AmmoDrop_Inst"))
  (bind _output_get (set `self.DMI` _returnvalue))
  (`PrimitiveComponent.SetMaterial` (`self.Cable1`) 0 _output_get)
  (for _index (range 3)
    (`PrimitiveComponent.SetMaterial` (`self.Projectile1`) _index _output_get))
  (`self.SetPreviewColor` true))