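; Gameplay mod actor that adds crouching for the local player, with a Crouch keybinding and menu page registered through the mod hub.
; A timeline lerps the capsule half-height to half and back, toggling a movement-penalty status effect when it finishes.
; Crouch toggles the state and Run stands up, gated by an upward trace for headroom that leaves debug drawing and printing on.
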(event `self.ReceiveBeginPlay`
  (bind _fsdplayercontroller (`/Game/_DRGModding/_Frameworks/BML_Framework.GetLocalPlayerController(Macro)` true)
    (:`Completed`
      (`self.EnableInput` _fsdplayercontroller)
      (`TimelineComponent.SetPlayRate` (`self.Timeline_0`) 3.0)
      (bind _playercharacter (`/Game/_DRGModding/_Frameworks/BML_Framework.GetLocalPlayerCharacter(Macro)` true)
        (:`Exec`
          (bind _output_get (set `self.Player Character` _playercharacter))
          (bind _output_get_2 (set `self.Capsule Half Height` (`CapsuleComponent.CapsuleHalfHeight` (`Character.CapsuleComponent` _output_get))))
          (set `self.NewVar_0` (* _output_get_2 0.5))
          (bind _output_get_3 (set `self.Max Walk Speed` (`CharacterMovementComponent.MaxWalkSpeed` (`Character.CharacterMovement` _output_get))))
          (set `self.NewVar_1` (* _output_get_3 0.5))
          (bind _returnvalue (`|CreateWidget` "/Game/_DRGModding/_LesnovMods/GameplayMods/Mod_Crouch/HUBMENU_Crouch.HUBMENU_Crouch_C"))
          (set `self.HUBMENU` _returnvalue))))))

(event `InputAction|Run` :consume false
  (params (Key :type "Key Structure"))
  (:`Pressed`
    (`self.PreventExecWhenHasNoSpaceAbove` :!label _label)
    (set `self.IsCrouch` false)
    (`self.CrouchEnd`)))

(event `InputAction|Crouch` :consume false
  (params (Key :type "Key Structure"))
  (:`Pressed`
    (if (`self.IsCrouch`)
      (goto _label)
      (else
        (set `self.IsCrouch` true)
        (`self.CrouchStart`)))))

(event `CrouchStart`
  (bind (_direction _newtrack_0) (`Timeline|Timeline_0` :!label _label_2)
    (:`Update`
      (`CapsuleComponent.SetCapsuleHalfHeight` (`Character.CapsuleComponent` (`self.Player Character`)) (`KismetMathLibrary.Lerp` (`self.Capsule Half Height`) (`self.NewVar_0`) _newtrack_0) true))
    (:`Finished`
      (switch `ETimelineDirection` _direction
        (:`Forward`
          (`/Game/_DRGModding/_Frameworks/BML_Framework.ToggleStatusEffect` true (`self.Player Character`) "/Game/_DRGModding/_LesnovMods/GameplayMods/Mod_Crouch/STE_CrouchMovementPenalty.STE_CrouchMovementPenalty_C"))
        (:`Backward`
          (`/Game/_DRGModding/_Frameworks/BML_Framework.ToggleStatusEffect` false (`self.Player Character`) "/Game/_DRGModding/_LesnovMods/GameplayMods/Mod_Crouch/STE_CrouchMovementPenalty.STE_CrouchMovementPenalty_C"))))))

(event `CrouchEnd`
  (goto _label_2 :!via `Reverse`))

(event `/Game/_ModHub/IHubMod.ModRegistered`
  (params (Hub :type "/Game/_ModHub/IHub Interface"))
  (`/Game/_ModHub/IHub.RegisterKeybinding` Hub self "Crouch" "Crouch" (make `InputChord` "None")))

(fn `GetModInfo`
  (returns (ModName :type Text) (ModAuthor :type Text) (ModVersion :type Text))
  (return "Crouch" "Lesnov" "1.0.0"))

(fn `GetModPages`
  (returns (HubPages :type "Array of /Game/_ModHub/IHubPageWidget Interface"))
  (return (`|MakeArray` (`self.HUBMENU`) :!type "/Game/_ModHub/IHubPageWidget Interface")))

(fn `UserConstructionScript`)