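; Base damage-testing prop that visibly reacts to hits; child classes override the target mesh and collision getters.
; SimpleHealth events and projectile collisions feed DamageIndicater, which pushes the target away from the local player and flashes its dynamic material via a timeline.
; It also spawns a throttled Niagara hit effect, line-tracing from the player when the hit location is zero.
; Physics-simulating targets teleport back to their initial transform after a delay.
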(event `self.ReceiveBeginPlay`
  (set `self.InitialSpawnTransform` (`SceneComponent.K2_GetComponentToWorld` (`self.GetTargetCollision(Override)`)))
  (add `PrimitiveComponent.OnComponentHit` (`self.GetTargetCollision(Override)`) (delegate `OnComponentHit_Event_0`))
  (bind _playercharacter (`/Game/_DRGModding/_Frameworks/BML_Framework.GetLocalPlayerCharacter(Macro)` true)
    (:`Exec`
      (set `self.Player Character` _playercharacter))))

(event `OnComponentHit_Event_0`
  (params (HitComponent :type "PrimitiveComponent Object Reference") (OtherActor :type "Actor Object Reference") (OtherComp :type "PrimitiveComponent Object Reference") (NormalImpulse :type "Vector Structure") (Hit :type "HitResult Structure (by ref)"))
  (`self.DamageIndicaterProjectileOnly` OtherActor Hit_Location))

(event `DamageIndicater`
  (params (Location :type "Vector Structure"))
  (bind _player_character (`self.Player Character`))
  (bind _damagecolor (`self.DamageColor`))
  (`/Engine/EditorBlueprintResources/StandardMacros.IsValid` _player_character
    (:`Is Valid`
      (`self.SpawnSystem` Location (`KismetMathLibrary.FindLookAtRotation` Location (`self.K2_GetActorLocation` _player_character)))
      (`/Game/_DRGModding/_Frameworks/BML_Framework.AddImpulseByCalcBetweenActors` (`self.GetTargetCollision(Override)`) (`self.Player Character`) 100000)
      (if (`SceneComponent.IsSimulatingPhysics` (`self.GetTargetCollision(Override)`) "None")
        (`KismetSystemLibrary.K2_SetTimer` null "TeleportInitialSpawnPoint" (`self.WaitTameToRevertPosition`)))
      (`MaterialInstanceDynamic.SetVectorParameterValue` (`self.DMI`) "InnerColor" _damagecolor)
      (`MaterialInstanceDynamic.SetVectorParameterValue` (`self.DMI`) "OuterColor" _damagecolor)
      (bind (_direction _newtrack_0) (`Timeline|TL_DamageIndicater` :!via `PlayFromStart`)
        (:`Update`
          (`MaterialInstanceDynamic.SetScalarParameterValue` (`self.DMI`) "EmitInner" (`KismetMathLibrary.Lerp` (`self.EmitInnerBase`) 15.0 _newtrack_0))
          (`MaterialInstanceDynamic.SetScalarParameterValue` (`self.DMI`) "EmitOuter" (`KismetMathLibrary.Lerp` (`self.EmitOuterBase`) 255.0 _newtrack_0)))
        (:`Finished`
          (`MaterialInstanceDynamic.SetVectorParameterValue` (`self.DMI`) "InnerColor" (`self.InnerColorBase`))
          (`MaterialInstanceDynamic.SetVectorParameterValue` (`self.DMI`) "OuterColor" (`self.OuterColorBase`)))))))

(event `self.SimpleHealth.OnHealthChanged`
  (params (Health :type "Float (single-precision)"))
  (set `self.Damage Data Hit Location` (0.0 0.0 0.0) :!label _label)
  (`self.DamageIndicater` (`self.Damage Data Hit Location`) :!label _label_2))

(event `self.SimpleHealth.OnHit`
  (params (Damage :type "Float (single-precision)") (DamageData :type "DamageData Structure (by ref)") (anyHealthLost :type Boolean))
  (goto _label))

(event `self.OnHit(Dummy)`
  (params (Location :type "Vector Structure"))
  (set `self.Damage Data Hit Location` Location)
  (goto _label_2))

(event `SpawnSystem`
  (params (Location :type "Vector Structure") (Rotation :type "Rotator Structure"))
  (if (not (`self.PreventSystemSpawn`))
    (if (== Location (0.0 0.0 0.0) :`ErrorTolerance` 0.1)
      (bind (_location _normal) (`/Game/_DRGModding/_Frameworks/BML_Framework.QuickLinetrace` (`self.Player Character`))
        (:`OnHit`
          (if (== _location (0.0 0.0 0.0) :`ErrorTolerance` 0.1)
            (set `self.Location` (`SceneComponent.K2_GetComponentLocation` (`self.GetTargetCollision(Override)`)))
            (else
              (set `self.Location` _location)))
          (set `self.Rotation` (`KismetMathLibrary.Conv_VectorToRotator` _normal))))
      (else
        (set `self.Location` Location)
        (set `self.Rotation` Rotation)))
    (set `self.PreventSystemSpawn` true)
    (`NiagaraFunctionLibrary.SpawnSystemAtLocation` "/Game/_DRGModding/_SharedAssets/_Lesnov/NS_HitEffect.NS_HitEffect" (`self.Location`) (`self.Rotation`))
    (`KismetSystemLibrary.K2_SetTimer` null "ActivateSpawn" 0.2)))

(fn `ActivateSpawn`
  (set `self.PreventSystemSpawn` false))

(fn `DamageIndicaterProjectileOnly`
  (params (Object :type "Object Object Reference") (InputPin :type "Vector Structure"))
  (if (`KismetMathLibrary.ClassIsChildOf` (`GameplayStatics.GetObjectClass` Object) "/Script/FSD.Projectile")
    (`self.DamageIndicater` InputPin)))

(fn `GetTargetCollision(Override)`
  (returns (Collision :type "PrimitiveComponent Object Reference"))
  (return null))

(fn `GetTargetMesh(Override)`
  (returns (StaticMesh :type "StaticMeshComponent Object Reference"))
  (return null))

(fn `NewFunction_0`
  (params (Start :type "Vector Structure (by ref)"))
  (`/Engine/EditorBlueprintResources/StandardMacros.IsValid` (`self.Player Character`)))

(fn `TeleportInitialSpawnPoint`
  (`PrimitiveComponent.SetAllPhysicsLinearVelocity` (`self.GetTargetCollision(Override)`) (0.0 0.0 0.0) false)
  (`SceneComponent.K2_SetWorldTransform` (`self.GetTargetCollision(Override)`) (`self.InitialSpawnTransform`) false false))

(fn `UserConstructionScript`
  (bind _dmi (`self.DMI`))
  (bind _dmi_2 (`self.DMI`))
  (bind _returnvalue (`PrimitiveComponent.CreateDynamicMaterialInstance` (`self.GetTargetMesh(Override)`) 0 (`self.Source Material`) "None"))
  (set `self.DMI` _returnvalue)
  (`TimelineComponent.SetPlayRate` (`self.TL_DamageIndicater`) (`self.DamageIndicaterSpeed`))
  (bind _returnvalue_2 (`MaterialInstanceDynamic.K2_GetVectorParameterValue` _dmi_2 "InnerColor"))
  (set `self.InnerColorBase` _returnvalue_2)
  (bind _returnvalue_3 (`MaterialInstanceDynamic.K2_GetScalarParameterValue` _dmi_2 "EmitInner"))
  (set `self.EmitInnerBase` _returnvalue_3)
  (bind _returnvalue_4 (`MaterialInstanceDynamic.K2_GetVectorParameterValue` _dmi "OuterColor"))
  (set `self.OuterColorBase` _returnvalue_4)
  (bind _returnvalue_5 (`MaterialInstanceDynamic.K2_GetScalarParameterValue` _dmi "EmitOuter"))
  (set `self.EmitOuterBase` _returnvalue_5))