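; Elevator prop that moves its mesh between its origin and a target point marked by the Billboard component.
; BeginPlay caches the Billboard's relative location and sets the timeline play rate.
; Each overlap with the floor collider, unfiltered by actor, flip-flops the timeline forward or in reverse to lerp the mesh position.
; Motion audio fades in on overlap and out when the timeline finishes.
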(event `self.ReceiveBeginPlay`
  (set `self.Relative Location` (`SceneComponent.RelativeLocation` (`self.Billboard`)))
  (`TimelineComponent.SetPlayRate` (`self.Timeline_0`) (`self.New Rate`)))

(event `self.Collider_Floor.OnComponentBeginOverlap`
  (params (OverlappedComponent :type "PrimitiveComponent Object Reference") (OtherActor :type "Actor Object Reference") (OtherComp :type "PrimitiveComponent Object Reference") (OtherBodyIndex :type Integer) (bFromSweep :type Boolean) (SweepResult :type "HitResult Structure (by ref)"))
  (`AudioComponent.FadeIn` (`self.MotionAudioController`) 0.1 1.0 0.0 "Linear")
  (`/Engine/EditorBlueprintResources/StandardMacros.FlipFlop`
    (:`A`
      (bind (_direction _newtrack_0) (`Timeline|Timeline_0` :!label _label)
        (:`Update`
          (`SceneComponent.K2_SetRelativeLocation` (`self.Mesh_Elevator`) (`KismetMathLibrary.VLerp` (0.0 0.0 0.0) (`self.Relative Location`) _newtrack_0) false false))
        (:`Finished`
          (`AudioComponent.FadeOut` (`self.MotionAudioController`) 0.5 0.0 "Linear"))))
    (:`B`
      (goto _label :!via `Reverse`))))

(fn `UserConstructionScript`)