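; Test character that previews a combination of vanity items (armor, headgear, facial hair, colors, skin) on a modular skeletal mesh body.
; The construction script blocking-loads soft-referenced assets, then applies meshes, materials and a test animation.
; Head item type and flags drive helmet material, attachment and head, beard and moustache visibility.
; At runtime, Tick forces a velocity override, while a looping timer returns it to spawn when it strays too far.
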(event `CustomEvent_0`
  (bind _spawnpoint (`self.SpawnPoint`))
  (if (> (`KismetMathLibrary.Vector_Distance` (`self.SpawnPoint`) (`self.K2_GetActorLocation`)) 2555.0)
    (if (!= _spawnpoint (0.0 0.0 0.0))
      (`self.K2_SetActorLocation` _spawnpoint))))

(event `self.ReceiveBeginPlay`
  (`KismetSystemLibrary.K2_SetTimerDelegate` (delegate `CustomEvent_0`) 0.2 true)
  (set `self.SpawnPoint` (`self.K2_GetActorLocation`)))

(event `self.ReceiveTick`
  (params (DeltaSeconds :type "Float (single-precision)"))
  (set `MovementComponent.Velocity` (`self.VelocityOverride`) (`self.CharacterMovement`)))

(fn `ApplyAnimation`
  (bind _testanimation (`self.TestAnimation`))
  (set `SkeletalMeshComponent.AnimationData` (make `SingleAnimationPlayData` _testanimation) (`self.Head`))
  (set `SkeletalMeshComponent.AnimationData` (make `SingleAnimationPlayData` _testanimation) (`self.Armor`))
  (set `SkeletalMeshComponent.AnimationData` (make `SingleAnimationPlayData` _testanimation) (`self.Helmet`))
  (set `SkeletalMeshComponent.AnimationData` (make `SingleAnimationPlayData` _testanimation) (`self.Eyebrows`)))

(fn `LoadAssetBySoftReference`
  (params (Array :type "Array of Object Soft Object Reference"))
  (for _array_element Array
    (`KismetSystemLibrary.LoadAsset_Blocking` _array_element)))

(fn `PreLoadVanityAssets`
  (`self.LoadAssetBySoftReference` (`|MakeArray` (`BlueprintMapLibrary.Map_Find` (`ArmorVanityItem.TPArmorMesh` (`self.ArmorVanityItem`)) "Default") (`ArmorVanityItem.MaterialOverride` (`self.ArmorVanityItem`)) :!type "Object Soft Object Reference"))
  (`self.LoadAssetBySoftReference` (`|MakeArray` (`HeadVanityItem.Mesh` (`self.HeadVanityItem`)) (`HeadVanityItem.MaterialOverride` (`self.HeadVanityItem`)) :!type "Object Soft Object Reference"))
  (`self.LoadAssetBySoftReference` (`|MakeArray` (`ArmorMaterialVanityItem.Material` (`self.ArmorMaterialVanityItem`)) :!type "Object Soft Object Reference"))
  (`self.LoadAssetBySoftReference` (`|MakeArray` (`MoustacheVanityItem.Mesh` (`self.MoustacheVanityItem`)) (`BeardVanityItem.Mesh` (`self.BeardVanityItem`)) (`EyeBrowsVanityItem.Mesh` (`self.EyeBrowsVanityItem`)) (`SideburnsVanityItem.Mesh` (`self.SideBurnsVanityItem`)) :!type "Object Soft Object Reference")))

(fn `SetArmor`
  (bind _armor (`self.Armor`))
  (`self.PreLoadVanityAssets`)
  (`SkinnedMeshComponent.SetSkinnedAssetAndUpdate` _armor (`|ConvertAsset` (`BlueprintMapLibrary.Map_Find` (`ArmorVanityItem.TPArmorMesh` (`self.ArmorVanityItem`)) "Default")) true)
  (`PrimitiveComponent.SetMaterial` _armor 0 (`|ConvertAsset` (`ArmorVanityItem.MaterialOverride` (`self.ArmorVanityItem`)))))

(fn `SetArmorMaterial`
  (`PrimitiveComponent.SetMaterial` (`self.Armor`) 0 (`|ConvertAsset` (`ArmorMaterialVanityItem.Material` (`self.ArmorMaterialVanityItem`))))
  (`PrimitiveComponent.SetMaterial` (`self.Helmet`) 0 (select `EHeadVanityType` (`HeadVanityItem.HeadVanityType` (`self.HeadVanityItem`)) :`HeadGearOnly` (`|ConvertAsset` (`HeadVanityItem.MaterialOverride` (`self.HeadVanityItem`))) :`HeadGearOnly_UseArmorMaterial` (`|ConvertAsset` (`ArmorMaterialVanityItem.Material` (`self.ArmorMaterialVanityItem`))))))

(fn `SetBeard`
  (`SkinnedMeshComponent.SetSkinnedAssetAndUpdate` (`self.Beard`) (`|ConvertAsset` (`BeardVanityItem.Mesh` (`self.BeardVanityItem`))) true))

(fn `SetBeardColor`
  (`PrimitiveComponent.SetMaterial` (`self.Beard`) 0 (`BeardColorVanityItem.BeardColor` (`self.BeardColorVanityItem`)))
  (`PrimitiveComponent.SetMaterial` (`self.Moustache`) 0 (`BeardColorVanityItem.MoustacheColor` (`self.BeardColorVanityItem`)))
  (`PrimitiveComponent.SetMaterial` (`self.Eyebrows`) 0 (`BeardColorVanityItem.EyebrowColor` (`self.BeardColorVanityItem`)))
  (`PrimitiveComponent.SetMaterial` (`self.SideBurns`) 0 (`BeardColorVanityItem.SideburnColor` (`self.BeardColorVanityItem`)))
  (switch `EHeadVanityType` (`HeadVanityItem.HeadVanityType` (`self.HeadVanityItem`))
    (:`HairOnly`
      (`PrimitiveComponent.SetMaterial` (`self.Helmet`) 0 (`BeardColorVanityItem.HairColor` (`self.BeardColorVanityItem`))))))

(fn `SetEyebrows`
  (`SkinnedMeshComponent.SetSkinnedAssetAndUpdate` (`self.Eyebrows`) (`|ConvertAsset` (`EyeBrowsVanityItem.Mesh` (`self.EyeBrowsVanityItem`))) true))

(fn `SetHead`
  (bind _helmet (`self.Helmet`))
  (bind _returnvalue (select `bool` (`HeadVanityItem.HideAll` (`self.HeadVanityItem`)) :`false` true))
  (`SkinnedMeshComponent.SetSkinnedAssetAndUpdate` _helmet (`|ConvertAsset` (`HeadVanityItem.Mesh` (`self.HeadVanityItem`))) true)
  (`PrimitiveComponent.SetMaterial` _helmet 0 (select `EHeadVanityType` (`HeadVanityItem.HeadVanityType` (`self.HeadVanityItem`)) :`HeadGearOnly` (`|ConvertAsset` (`HeadVanityItem.MaterialOverride` (`self.HeadVanityItem`))) :`HeadGearOnly_UseArmorMaterial` (`|ConvertAsset` (`ArmorVanityItem.MaterialOverride` (`self.ArmorVanityItem`)))))
  (`SkeletalMeshComponent.SetAnimInstanceClass` (`self.Helmet`) (`|ConvertAsset` (`HeadVanityItem.AnimInstance` (`self.HeadVanityItem`))))
  (if (`KismetSystemLibrary.IsValidSoftClassReference` (`HeadVanityItem.AnimInstance` (`self.HeadVanityItem`)))
    (`SceneComponent.K2_AttachToComponent` (`self.Helmet`) (`self.Armor`) "Beard_Socket" "SnapToTarget" "SnapToTarget" "KeepRelative" true)
    (else
      (`SceneComponent.K2_AttachToComponent` (`self.Helmet`) (`self.Armor`) "None" "SnapToTarget" "SnapToTarget" "KeepWorld" true)))
  (`SceneComponent.SetVisibility` (`self.Head`) (not (`HeadVanityItem.HideHead` (`self.HeadVanityItem`))) false)
  (`SceneComponent.SetVisibility` (`self.Beard`) _returnvalue false)
  (`SceneComponent.SetVisibility` (`self.Moustache`) _returnvalue false)
  (if (`HeadVanityItem.HideBeard` (`self.HeadVanityItem`))
    (`SceneComponent.SetVisibility` (`self.Beard`) false false))
  (if (`HeadVanityItem.HideMoustache` (`self.HeadVanityItem`))
    (`SceneComponent.SetVisibility` (`self.Moustache`) false false)))

(fn `SetMoustache`
  (`SkinnedMeshComponent.SetSkinnedAssetAndUpdate` (`self.Moustache`) (`|ConvertAsset` (`MoustacheVanityItem.Mesh` (`self.MoustacheVanityItem`))) true))

(fn `SetSideBurns`
  (`SkinnedMeshComponent.SetSkinnedAssetAndUpdate` (`self.SideBurns`) (`|ConvertAsset` (`SideburnsVanityItem.Mesh` (`self.SideBurnsVanityItem`))) true))

(fn `SetSkinColor`
  (bind _material (`SkinColorVanityItem.Material` (`self.SkinColorVanityItem`)))
  (`/Engine/EditorBlueprintResources/StandardMacros.IsValid` (`PrimitiveComponent.GetMaterial` (`self.Armor`) 1)
    (:`Is Valid`
      _)
    (:`Is Not Valid`
      (`PrimitiveComponent.SetMaterial` (`self.Armor`) 1 _material)))
  (`PrimitiveComponent.SetMaterial` (`self.Head`) 0 _material))

(fn `UserConstructionScript`
  (`self.SetArmor`)
  (`self.SetHead`)
  (`self.SetArmorMaterial`)
  (`self.SetBeard`)
  (`self.ApplyAnimation`)
  (`self.SetMoustache`)
  (`self.SetEyebrows`)
  (`self.SetBeardColor`)
  (`self.SetSideBurns`)
  (`self.SetSkinColor`))