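; BP_VictoryPosePlayer is a usable tool actor that previews the victory pose assigned to it.
; Its construction script labels it with the pose's display name, and its skeletal mesh is hidden in game, supplying only the spawn transform.
; On use it plays a click sound and spawns a rotated, lifespan-limited BP_VictoryPoseCharacter with that pose.
; The spawned character is cached, so the next use can optionally destroy it first.
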(event `self.ReceiveBeginPlay`
  (`SceneComponent.SetHiddenInGame` (`self.SkeletalMesh`) true false))

(event `self.InstantUsable.OnUsedBy`
  (params (User :type "PlayerCharacter Object Reference") (Key :type "EInputKeys Enum" :default "Use"))
  (`self.DestroyCachedPose`)
  (`/Game/_DRGModding/_LesnovMods/_SharedAssets/BML_Actor.PlaySoundAtSelf` "/Game/Audio/SFX/Donkey/Molly/Dwarf_Click_Button_Cue.Dwarf_Click_Button_Cue")
  (bind _returnvalue (`|SpawnActorFromClass` "/Game/_DRGModding/_LesnovMods/_SharedAssets/Tool/VictoryPosePlayer/BP_VictoryPoseCharacter.BP_VictoryPoseCharacter_C" (`SceneComponent.K2_GetComponentToWorld` (`self.SkeletalMesh`)) "AdjustIfPossibleButAlwaysSpawn" "OverrideRootScale" null (`self.Victory Pose`) null))
  (`self.K2_SetActorRelativeRotation` _returnvalue (struct :`Yaw` -90.0) false false)
  (`self.SetLifeSpan` _returnvalue (`self.In Lifespan`))
  (set `self.CachedPose` _returnvalue))

(fn `DestroyCachedPose`
  (`/Engine/EditorBlueprintResources/StandardMacros.IsValid` (`self.CachedPose`)
    (:`Is Valid`
      (if (`self.DestoryCache`)
        (`self.K2_DestroyActor` (`self.CachedPose`))))))

(fn `UserConstructionScript`
  (`TextRenderComponent.K2_SetText` (`self.TextRender`) (`KismetTextLibrary.Conv_StringToText` (`KismetSystemLibrary.GetDisplayName` (`self.Victory Pose`)))))