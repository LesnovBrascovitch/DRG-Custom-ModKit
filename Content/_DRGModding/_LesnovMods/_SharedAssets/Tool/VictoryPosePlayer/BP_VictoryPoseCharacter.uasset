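; BP_VictoryPoseCharacter is a modular character that plays a victory pose animation, built from Armor, Head and Eyebrows meshes.
; The construction script slaves Head and Eyebrows to Armor through master pose, so one AnimInstance drives all three.
; BeginPlay async-loads a random walk and the pose from VictoryPose, waiting only on the pose load's completion.
; It then passes both, plus an unarmed idle, to Armor's ABP_VictoryPose at normal play rate.
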(event `self.ReceiveBeginPlay`
  (`parent.ReceiveBeginPlay`)
  (bind _object (`|LoadAsset` (`KismetArrayLibrary.Array_Random` (`VictoryPose.Walks` (`self.VictoryPose`))))
    (:`then`
      (bind _object_2 (`|LoadAsset` (`VictoryPose.pose` (`self.VictoryPose`)))
        (:`Completed`
          (bind _asabp_victory_pose (cast `/Game/_DRGModding/_LesnovMods/_SharedAssets/Tool/VictoryPosePlayer/ABP_VictoryPose` (`SkeletalMeshComponent.GetAnimInstance` (`self.Armor`))))
          (bind _asanim_sequence (cast `AnimSequence` _object))
          (bind _asanim_sequence_2 (cast `AnimSequence` _object_2))
          (set `/Game/_DRGModding/_LesnovMods/_SharedAssets/Tool/VictoryPosePlayer/ABP_VictoryPose.AnimVictoryPoseStart` _asanim_sequence _asabp_victory_pose)
          (set `/Game/_DRGModding/_LesnovMods/_SharedAssets/Tool/VictoryPosePlayer/ABP_VictoryPose.AnimVictoryPose` _asanim_sequence_2 _asabp_victory_pose)
          (set `/Game/_DRGModding/_LesnovMods/_SharedAssets/Tool/VictoryPosePlayer/ABP_VictoryPose.AnimVictoryPoseIdle` "/Game/CharacterStructure/Gear_Unarmed/TP/TP_Unarmed_Idle_A.TP_Unarmed_Idle_A" _asabp_victory_pose)
          (set `/Game/_DRGModding/_LesnovMods/_SharedAssets/Tool/VictoryPosePlayer/ABP_VictoryPose.Play Rate` 1.0 _asabp_victory_pose))))))

(fn `UserConstructionScript`
  (bind _armor (`self.Armor`))
  (`parent.UserConstructionScript`)
  (`SkinnedMeshComponent.SetLeaderPoseComponent` (`self.Head`) _armor false)
  (`SkinnedMeshComponent.SetLeaderPoseComponent` (`self.Eyebrows`) _armor false))