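; Preview actor that plays a chosen animation on a third-person dwarf rig, with a held skeletal mesh or Blueprint actor.
; Construction script and BeginPlay both apply the same animation and material to head and body, then attach HeadMesh1 at a configurable socket.
; With UseBlueprint set, HeadMesh1 is hidden in game and BeginPlay spawns the given class, snapped to the right-hand socket.
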(event `self.ReceiveBeginPlay`
  (bind _newvar_0 (`self.NewVar_0`))
  (bind _class (`self.Class`))
  (bind _animation_data_playing (`self.Animation Data Playing`))
  (bind _animation_data_initial_position (`self.Animation Data Initial Position`))
  (bind _headmesh1 (`self.HeadMesh1`))
  (`|ExecutionSequence`
    (:`then_0`
      (if (`self.UseBlueprint`)
        (if (`KismetSystemLibrary.IsValidClass` _class)
          (bind _returnvalue (`|SpawnActorFromClass` _class (`KismetMathLibrary.MakeTransform` (0.0 0.0 0.0)) "AlwaysSpawn" "OverrideRootScale" null null))
          (`self.K2_AttachToComponent` _returnvalue (`self.BodyMesh`) "Dwarf_HandR_Attach" "SnapToTarget" "SnapToTarget" "SnapToTarget" true))))
    (:`then_1`
      (set `SkeletalMeshComponent.AnimationData` (make `SingleAnimationPlayData` _newvar_0 true _animation_data_playing _animation_data_initial_position) (`self.HeadMesh`))
      (set `SkeletalMeshComponent.AnimationData` (make `SingleAnimationPlayData` _newvar_0 true _animation_data_playing _animation_data_initial_position) (`self.BodyMesh`))
      (`SceneComponent.K2_AttachToComponent` (`self.HeadMesh1`) (`self.BodyMesh`) (`self.Socket Name`) "SnapToTarget" "SnapToTarget" "KeepWorld" true)
      (if (`self.UseBlueprint`)
        (`SceneComponent.SetHiddenInGame` _headmesh1 true false)
        (else
          (`SceneComponent.SetHiddenInGame` _headmesh1 false false)))
      (`PrimitiveComponent.SetMaterial` (`self.HeadMesh`) 0 (`self.Material`))
      (`PrimitiveComponent.SetMaterial` (`self.BodyMesh`) 0 (`self.Material`))
      (`SkinnedMeshComponent.SetSkinnedAssetAndUpdate` (`self.HeadMesh1`) (`self.New Mesh`) true))))

(fn `UserConstructionScript`
  (bind _newvar_0 (`self.NewVar_0`))
  (bind _animation_data_playing (`self.Animation Data Playing`))
  (bind _animation_data_initial_position (`self.Animation Data Initial Position`))
  (bind _headmesh1 (`self.HeadMesh1`))
  (set `SkeletalMeshComponent.AnimationData` (make `SingleAnimationPlayData` _newvar_0 true _animation_data_playing _animation_data_initial_position) (`self.HeadMesh`))
  (set `SkeletalMeshComponent.AnimationData` (make `SingleAnimationPlayData` _newvar_0 true _animation_data_playing _animation_data_initial_position) (`self.BodyMesh`))
  (`SceneComponent.K2_AttachToComponent` (`self.HeadMesh1`) (`self.BodyMesh`) (`self.Socket Name`) "SnapToTarget" "SnapToTarget" "KeepWorld" true)
  (if (`self.UseBlueprint`)
    (`SceneComponent.SetHiddenInGame` _headmesh1 true false)
    (else
      (`SceneComponent.SetHiddenInGame` _headmesh1 false false)))
  (`PrimitiveComponent.SetMaterial` (`self.HeadMesh`) 0 (`self.Material`))
  (`PrimitiveComponent.SetMaterial` (`self.BodyMesh`) 0 (`self.Material`))
  (`SkinnedMeshComponent.SetSkinnedAssetAndUpdate` (`self.HeadMesh1`) (`self.New Mesh`) true))