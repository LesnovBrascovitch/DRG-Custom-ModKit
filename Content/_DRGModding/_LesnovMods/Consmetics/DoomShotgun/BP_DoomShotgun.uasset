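; Cosmetic Deep Rock Galactic mod actor that displays a Doom Super Shotgun in place of the first-person sawed-off shotgun.
; On equip, it hides the FP mesh and item, then attaches material billboards to the camera, overriding fire sound and binding weapon events.
; Timelines drive dynamic material parameters for fire and reload animation, plus muzzle flash and reload sounds.
; Tick adds a speed-scaled sine walk bob, and non-first-person cameras hide the billboard.
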(event `OnPlayerCharacterPossed`
  (params (Pawn :type "Pawn Object Reference"))
  (bind _inventorycomponent (`PlayerCharacter.InventoryComponent` (`self.Player Character`)))
  ;[1 1 1] BeginPlay
  (`self.Reset`)
  (bind _playercharacter (`/Game/_DRGModding/_Frameworks/BML_Framework.GetLocalPlayerCharacter(Macro)` true :!label _label)
    (:`Exec`
      (set `self.Player Character` _playercharacter)
      (add `InventoryComponent.OnItemEquipped` _inventorycomponent (`|CreateDelegate` :!event `CustomEvent_0`))
      (add `InventoryComponent.OnItemUnequipped` _inventorycomponent (`|CreateDelegate` :!event `CustomEvent_1`))
      (add `PlayerCharacter.OnCameraModeChanged` (`self.Player Character`) (`|CreateDelegate` :!event `OnCameraModeChanged`))
      (add `PlayerCharacter.OnCameraModeChanged` (`self.Player Character`) (`|CreateDelegate` :!event `OnCameraModeChanged`))
      (`SceneComponent.SetHiddenInGame` (`self.SuperShotgunBase`) true false))))

(event `self.ReceiveBeginPlay`
  ;[1 1 1] BeginPlay
  (bind _returnvalue (`KismetMaterialLibrary.CreateDynamicMaterialInstance` "/Game/_DRGModding/_LesnovMods/Consmetics/DoomShotgun/M_DoomSuperShotgun.M_DoomSuperShotgun"))
  (bind _output_get (set `self.DMI` _returnvalue))
  (`MaterialBillboardComponent.SetElements` (`self.SuperShotgunBase`) (`|MakeArray` (make `MaterialSpriteElement` _output_get) :!type "MaterialSpriteElement Structure"))
  (bind _returnvalue_2 (`KismetMaterialLibrary.CreateDynamicMaterialInstance` "/Game/_DRGModding/_LesnovMods/Consmetics/DoomShotgun/M_DoomSuperShotgun_Emissive.M_DoomSuperShotgun_Emissive"))
  (bind _output_get_2 (set `self.DMI_ShotEmissive` _returnvalue_2))
  (`MaterialBillboardComponent.SetElements` (`self.SuperShotgunEmissive`) (`|MakeArray` (make `MaterialSpriteElement` _output_get_2) :!type "MaterialSpriteElement Structure"))
  (bind _fsdplayercontroller (`/Game/_DRGModding/_Frameworks/BML_Framework.GetLocalPlayerController(Macro)` true)
    (:`Completed`
      (add `FSDPlayerController.OnPlayerCharacterPossesed` _fsdplayercontroller (delegate `OnPlayerCharacterPossed`))
      (goto _label))))

(event `self.ReceiveTick`
  (params (DeltaSeconds :type "Float (single-precision)"))
  (bind (_new_location_x _new_location_y _new_location_z) (`KismetMathLibrary.BreakVector` (`self.GetLocation`)))
  (bind _degreey (`self.DegreeY`))
  (bind _degreez (`self.DegreeZ`))
  ;[1 1 1] Tick - Walk Movement (I think I should use WPO from material side to achieve this.)
  (set `self.AlphaMovement` (select `bool` (`NavMovementComponent.IsFalling` (`Character.CharacterMovement` (`self.Player Character`))) :`false` (`KismetMathLibrary.MapRangeClamped` (`KismetMathLibrary.VSizeXY` (`MovementComponent.Velocity` (`Character.CharacterMovement` (`self.Player Character`)))) 0.0 600.0 0.0 1.0)))
  (`|VariableSetRef` _degreez (+ (* (`KismetMathLibrary.FTrunc` (* 1111.0 (`KismetMathLibrary.FClamp` (`self.AlphaMovement`) 0.1))) (`GameplayStatics.GetWorldDeltaSeconds`)) _degreez))
  (`|VariableSetRef` _degreey (+ (* (`KismetMathLibrary.FTrunc` (* 555.0 (`self.AlphaMovement`))) (`GameplayStatics.GetWorldDeltaSeconds`)) _degreey))
  (`SceneComponent.K2_SetRelativeLocation` (`self.SuperShotgunBase`) (`KismetMathLibrary.MakeVector` _new_location_x (+ _new_location_y (* (`KismetMathLibrary.DegSin` (`self.DegreeY`)) (`self.MoveOffset(DegreeY)`))) (+ _new_location_z (* (`KismetMathLibrary.DegSin` (`self.DegreeZ`)) (`self.MoveOffset(DegreeZ)`)))) false false)
  (if (> (`self.DegreeZ`) 360.0)
    (set `self.DegreeZ` 0.0))
  (if (> (`self.DegreeY`) 360.0)
    (set `self.DegreeY` 0.0)))

(event `OnCameraModeChanged`
  (params (NewCameraMode :type "ECharacterCameraMode Enum" :default "FirstPerson") (OldCameraMode :type "ECharacterCameraMode Enum" :default "FirstPerson"))
  (bind _supershotgunbase (`self.SuperShotgunBase`))
  ;[1 1 1] OnCameraModeChanged - Hide super shotgun material when camera is changed.
  (switch `ECharacterCameraMode` NewCameraMode
    (:`FirstPerson`
      (`self.IsClassSawedOff` (`/Game/_DRGModding/_Frameworks/BML_Framework.GetCurrentItem` (`self.Player Character`)))
      (`SceneComponent.SetHiddenInGame` _supershotgunbase false true))
    (:`ThirdPerson`
      (`SceneComponent.SetHiddenInGame` _supershotgunbase true true :!label _label_2))
    (:`Follow`
      (goto _label_2))
    (:`DownCamera`
      (goto _label_2))
    (:`TerrainScanner`
      (goto _label_2))
    (:`PhotographyMode`
      (goto _label_2))))

(event `PlayReload`
  ;[1 1 1] Reload Animation
  (`MaterialInstanceDynamic.SetScalarParameterValue` (`self.DMI`) "Reload" 1.0)
  (`GameplayStatics.SpawnSoundAttached` "/Game/_DRGModding/_LesnovMods/Consmetics/DoomShotgun/DoomSuperShotgun_Reload_01_Cue.DoomSuperShotgun_Reload_01_Cue" (`self.SuperShotgunBase`) "None" (0.0 0.0 0.0) (struct) "KeepRelativeOffset" false 1.0 1.0 0.0 null null)
  (bind (_direction _newtrack_0) (`Timeline|TL_Reload` :!via `PlayFromStart`)
    (:`Update`
      (`MaterialInstanceDynamic.SetScalarParameterValue` (`self.DMI`) "Animation  Phase Reload(0-1) (S)" (`KismetMathLibrary.Lerp` 0.0 0.75 _newtrack_0))
      (if (> _newtrack_0 0.5)
        (`/Engine/EditorBlueprintResources/StandardMacros.DoOnce` false :!label _label_3
          (:`Completed`
            (`GameplayStatics.SpawnSoundAttached` "/Game/_DRGModding/_LesnovMods/Consmetics/DoomShotgun/DoomSuperShotgun_Reload_02_Cue.DoomSuperShotgun_Reload_02_Cue" (`self.SuperShotgunBase`) "None" (0.0 0.0 0.0) (struct) "KeepRelativeOffset" false 1.0 1.0 0.0 null null)))))
    (:`Finished`
      (`MaterialInstanceDynamic.SetScalarParameterValue` (`self.DMI`) "Reload" 0.0)
      (`GameplayStatics.SpawnSoundAttached` "/Game/_DRGModding/_LesnovMods/Consmetics/DoomShotgun/DoomSuperShotgun_Reload_03_Cue.DoomSuperShotgun_Reload_03_Cue" (`self.SuperShotgunBase`) "None" (0.0 0.0 0.0) (struct) "KeepRelativeOffset" false 1.0 1.0 0.0 null null)
      (goto _label_3 :!via `Reset`))))

(event `CustomEvent_0`
  (params (Item :type "Item Object Reference"))
  ;[1 1 1] OnItemEquipped - Show Super Shotgun material, Change some stats from WPN_SawedOffShotgun as AmmoDrivenWeapon.
  (`self.IsClassSawedOff` Item)
  (`self.SetVisibillity(DoomBased)` Item)
  (`self.SetActorTickEnabled` true)
  (`/Engine/EditorBlueprintResources/StandardMacros.DoOnce` false :!label _label_4
    (:`Completed`
      (bind _asammo_driven_weapon (cast `AmmoDrivenWeapon` Item))
      (set `AmmoDrivenWeapon.FireSound` "/Game/_DRGModding/_LesnovMods/Consmetics/DoomShotgun/DoomSuperShotgun_Fire_Cue.DoomSuperShotgun_Fire_Cue" _asammo_driven_weapon)
      (`TimelineComponent.SetPlayRate` (`self.TL_Reload`) (`KismetMathLibrary.SafeDivide` 1.0 (`AmmoDrivenWeapon.ReloadDuration` _asammo_driven_weapon)))
      (add `AmmoDrivenWeapon.OnReloadingEvent` _asammo_driven_weapon (`|CreateDelegate` :!event `PlayReload`))
      (add `AmmoDrivenWeapon.OnShotFiredEvent` _asammo_driven_weapon (`|CreateDelegate` :!event `PlayFire`)))))

(event `PlayFire`
  ;[1 1 1] Fire Animation
  (`MaterialInstanceDynamic.SetScalarParameterValue` (`self.DMI`) "Reload" 0.0)
  (bind (_direction _newtrack_0) (`Timeline|TL_Fire` :!via `PlayFromStart`)
    (:`Update`
      (`MaterialInstanceDynamic.SetScalarParameterValue` (`self.DMI`) "Animation  Phase (0-1) (S)" _newtrack_0)
      (`MaterialInstanceDynamic.SetScalarParameterValue` (`self.DMI_ShotEmissive`) "Animation  Phase (0-1) (S)" _newtrack_0)
      (`LightComponent.SetIntensity` (`self.MuzzleFlash`) (`KismetMathLibrary.Lerp` 15000.0 0.0 _newtrack_0)))))

(event `Reset`
  ;[1 1 1] OnItemEquipped - Show Super Shotgun material, Change some stats from WPN_SawedOffShotgun as AmmoDrivenWeapon.
  (goto _label_4 :!via `Reset`))

(event `CustomEvent_1`
  (params (Item :type "Item Object Reference"))
  ;[1 1 1] OnItemUnequipped - Hide Super Shotgun
  (`self.IsClassSawedOff` Item)
  (`self.SetVisibillity(DoomBased)` null true)
  (`self.SetActorTickEnabled` false))

(fn `GetLocation`
  (returns (`New Location` :type "Vector Structure"))
  (bind _baselocation (`self.BaseLocation`))
  (return (select `bool` (`/Game/_DRGModding/_Frameworks/BML_Framework.IsInDRG(Pure)`) :`false` _baselocation :`true` (`KismetMathLibrary.MakeVector` (.x _baselocation) (.y _baselocation) (+ (.z _baselocation) -15.0)))))

(fn `SetVisibillity(DoomBased)`
  (params (Item :type "Actor Object Reference") (Hide :type Boolean))
  (bind _supershotgunbase (`self.SuperShotgunBase`))
  (if Hide
    (`SceneComponent.SetHiddenInGame` (`PlayerCharacter.FPMesh` (`self.Player Character`)) false false)
    (`SceneComponent.SetHiddenInGame` (`self.SuperShotgunBase`) true true)
    (else
      (`SceneComponent.SetHiddenInGame` (`PlayerCharacter.FPMesh` (`self.Player Character`)) true false)
      (`self.SetActorHiddenInGame` (`local.Item`) true)
      (`SceneComponent.SetHiddenInGame` (`self.SuperShotgunBase`) false true)
      (`SceneComponent.K2_AttachToComponent` _supershotgunbase (`PlayerCharacter.FirstPersonCamera` (`self.Player Character`)) "None" "SnapToTarget" "SnapToTarget" "KeepRelative" true)
      (`SceneComponent.K2_SetRelativeLocation` _supershotgunbase (`self.GetLocation`) false false))))

(fn `UserConstructionScript`
  (`TimelineComponent.SetPlayRate` (`self.TL_Fire`) 3.0))