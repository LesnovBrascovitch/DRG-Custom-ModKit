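; Cosmetic mod actor that shows the local player's first-person weapons left-handed, with a saved toggle for right-handed view.
; On item equip it mirrors FPMesh with negative Y scale, flipped yaw and inverted AimRate, skipping banned items.
; Item-ID filters fix widget scales and pivots per weapon, and cached per-class defaults restore them for right-handed view.
; Chat messages starting with !LH act as console commands for settings, help and a reset.
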(event `CustomEvent_0`
  (`/Engine/EditorBlueprintResources/StandardMacros.IsValid` (`self.FPMesh`)
    (:`Is Valid`
      (`self.Debug Message` "FPMESH[PlayerChara]" "Is Valid"))
    (:`Is Not Valid`
      (`self.Debug Message` "FPMESH[PlayerChara]" "Is not valid"))))

(event `OnNewMessage`
  (params (Message :type "FSDChatMessage Structure (by ref)"))
  (bind _consolecommandslist (`self.ConsoleCommandsList`))
  (bind _as_lhwsavegame (`self.As LHWSavegame`))
  (bind _msg (`/Game/_DRGModding/_Frameworks/BML_Framework.IgnoreMsgBySender` Message (`self.Player Character`))
    (:`CanProceed`
      (bind (_lefts _rights _returnvalue) (`KismetStringLibrary.Split` _msg " "))
      (switch `string` (select `bool` _returnvalue :`false` _msg :`true` _lefts)
        (:`!LH_SP`
          (set `/Game/_DRGModding/_LesnovMods/Consmetics/LeftHandedWeapon/LHWSavegame.PivotIndex` (`KismetStringLibrary.Conv_StringToInt` _rights) _as_lhwsavegame)
          (`/Game/_DRGModding/_Frameworks/BML_Framework.PrintViaChat` false "QCC" (`KismetStringLibrary.Concat_StrStr` "Pivot Index Changed To " (`KismetStringLibrary.Conv_IntToString` (`/Game/_DRGModding/_LesnovMods/Consmetics/LeftHandedWeapon/LHWSavegame.PivotIndex` _as_lhwsavegame))))
          (`self.Save` :!label _label))
        (:`!LH_HELP`
          (bind _keys (`BlueprintMapLibrary.Map_Keys` _consolecommandslist))
          (for _array_element _keys
            (`/Game/_DRGModding/_Frameworks/BML_Framework.PrintViaChat` false "QCC" (`KismetStringLibrary.Concat_StrStr` _array_element " - " (`BlueprintMapLibrary.Map_Find` _consolecommandslist _array_element)))))
        (:`!LH_DBM`
          (`/Game/_DRGModding/_Frameworks/BML_Framework.SetBoolean` (`/Game/_DRGModding/_LesnovMods/Consmetics/LeftHandedWeapon/LHWSavegame.DisableDBMsg` (`self.As LHWSavegame`)) "Disable Debug Message")
          (goto _label))
        (:`!LH_FIX`
          (`SceneComponent.SetRelativeScale3D` (`self.FPMesh`) (0.6 0.6 0.6))
          (set `PlayerCharacter.AimSettings` (`self.Aim Settings`) (`self.Player Character`))
          (`SceneComponent.K2_SetRelativeRotation` (`self.FPMesh`) (`KismetMathLibrary.MakeRotator` 0.0 0.0 -90.0) false false)
          (`/Game/_DRGModding/_Frameworks/BML_Framework.PrintViaChat` false "[Mod Error - LHW] " "Tried to fix the problem."))
        (:`!LH_DISM`
          (`/Game/_DRGModding/_Frameworks/BML_Framework.SetBoolean` (`/Game/_DRGModding/_LesnovMods/Consmetics/LeftHandedWeapon/LHWSavegame.IsRightSided` (`self.As LHWSavegame`)) "Right-Handed View")
          (goto _label))
        (:`!LH_VERSION`
          (`/Game/_DRGModding/_Frameworks/BML_Framework.PrintViaChat` false "LHW VERSION" "1.0.1"))))))

(event `self.ReceiveBeginPlay`
  (bind _outputpin (`/Game/_DRGModding/_Frameworks/BML_Framework.HandleSaveGame` "/Game/_DRGModding/_LesnovMods/Consmetics/LeftHandedWeapon/LHWSavegame.LHWSavegame_C" :!label _label_2)
    (:`then`
      (bind _aslhwsavegame (cast `/Game/_DRGModding/_LesnovMods/Consmetics/LeftHandedWeapon/LHWSavegame` _outputpin))
      (set `self.As LHWSavegame` _aslhwsavegame)
      (add `MessagingSubSystem.OnNewMessage` (subsystem `MessagingSubSystem`) (delegate `OnNewMessage`))
      (bind _fsdplayercontroller (`/Game/_DRGModding/_Frameworks/BML_Framework.GetLocalPlayerController(Macro)` true)
        (:`Completed`
          (add `FSDPlayerController.OnPlayerCharacterPossesed` _fsdplayercontroller (delegate `OnPossessed`))
          (bind _playercharacter (`/Game/_DRGModding/_Frameworks/BML_Framework.GetLocalPlayerCharacter(Macro)` true :!label _label_3)
            (:`Exec`
              (bind _output_get (set `self.Player Character` _playercharacter))
              (bind _output_get_2 (set `self.FPMesh` (`PlayerCharacter.FPMesh` _output_get)))
              (set `self.Relative Rotation` (`SceneComponent.RelativeRotation` _output_get_2))
              (set `self.Aim Settings` (`PlayerCharacter.AimSettings` (`self.Player Character`)))
              (add `InventoryComponent.OnItemEquipped` (`PlayerCharacter.InventoryComponent` (`self.Player Character`)) (delegate `OnItemEquipped`))
              (`KismetSystemLibrary.K2_SetTimerDelegate` (delegate `CustomEvent_0`) 5.0 true))))))
    (:`ERROR`
      (`KismetSystemLibrary.Delay` 0.2)
      (goto _label_2))))

(event `OnItemEquipped`
  (params (Item :type "Item Object Reference"))
  (`/Engine/EditorBlueprintResources/StandardMacros.IsValid` Item
    (:`Is Valid`
      (set `self.CurrentItemClass` (`GameplayStatics.GetObjectClass` Item))
      (`self.FillFPWidgetInfos` Item)
      (if (`/Game/_DRGModding/_LesnovMods/Consmetics/LeftHandedWeapon/LHWSavegame.IsRightSided` (`self.As LHWSavegame`))
        (`self.ConvertItemToRightSide` Item)
        (else
          (`self.ConvertItemToLeftSide` Item))))))

(event `OnPossessed`
  (params (Pawn :type "Pawn Object Reference"))
  (goto _label_3))

(fn `ConvertItemToLeftSide`
  (params (TargetItem :type "Item Object Reference"))
  (locals (Local_Item :type "Item Object Reference") (Local_Index :type Integer :default 0))
  (bind _local_item (`local.Local_Item`))
  (bind _pivotindex (`/Game/_DRGModding/_LesnovMods/Consmetics/LeftHandedWeapon/LHWSavegame.PivotIndex` (`self.As LHWSavegame`)))
  (bind _aimsettings (`PlayerCharacter.AimSettings` (`self.Player Character`)))
  (`/Engine/EditorBlueprintResources/StandardMacros.IsValid` TargetItem
    (:`Is Valid`
      (set `local.Local_Item` TargetItem)
      (`self.Debug Message` (`KismetSystemLibrary.GetDisplayName` (`local.Local_Item`)) "LHS")
      (if (`BlueprintSetLibrary.Set_Contains` (`self.ItemList_Banned`) (`Item.ItemID` (`local.Local_Item`)))
        (`SceneComponent.SetRelativeScale3D` (`self.FPMesh`) (0.6 0.6 0.6) :!label _label)
        (set `PlayerCharacter.AimSettings` (`self.Aim Settings`) (`self.Player Character`))
        (`SceneComponent.K2_SetRelativeRotation` (`self.FPMesh`) (`KismetMathLibrary.MakeRotator` 0.0 0.0 -90.0) false false)
        (else
          (bind _output_get (set `local.Local_Index` (`self.GetFilterIndexByItemID` (`local.Local_Item`))))
          (`self.Debug Message` "Selected Index" (`KismetStringLibrary.Conv_IntToString` _output_get))
          (if (== (`local.Local_Index`) 3)
            (goto _label)
            (else
              (`SceneComponent.SetRelativeScale3D` (`self.FPMesh`) (0.6 -0.6 0.6))
              (`/Engine/EditorBlueprintResources/StandardMacros.IsValid` (`self.Player Character`)
                (:`Is Valid`
                  (set `PlayerCharacter.AimSettings` (make `AnalogAimSettings` (`KismetMathLibrary.MakeVector2D` (* -1 (`KismetMathLibrary.BreakVector2D` (break `AnalogAimSettings` _aimsettings))) (* -1 (`.Y` (`KismetMathLibrary.BreakVector2D` (break `AnalogAimSettings` _aimsettings))))) (`.SensitivityCurve` (break `AnalogAimSettings` _aimsettings)) (`.LookAtStickyness` (break `AnalogAimSettings` _aimsettings)) (`.StickynessRecoverySpeed` (break `AnalogAimSettings` _aimsettings)) (`.StickynessMaxSensitivity` (break `AnalogAimSettings` _aimsettings)) (`.ThirdPersonLookRate` (break `AnalogAimSettings` _aimsettings))) (`self.Player Character`))
                  (`SceneComponent.K2_SetRelativeRotation` (`self.FPMesh`) (`KismetMathLibrary.MakeRotator` 0.0 0.0 90.0) false false)
                  (if (== (`local.Local_Index`) 2)
                    (bind _aswpn_cryospray (cast `/Game/WeaponsNTools/Cryospray/WPN_Cryospray` (`local.Local_Item`)))
                    (`SceneComponent.SetRelativeScale3D` (`/Game/WeaponsNTools/Cryospray/WPN_Cryospray.FPwidget_Ammo` _aswpn_cryospray) (0.061297 0.061297 0.061297))
                    (else
                      (for _array_element (`self.K2_GetComponentsByClass` (`local.Local_Item`) "/Script/FSD.FirstPersonWidgetComponent")
                        (`/Engine/EditorBlueprintResources/StandardMacros.IsValid` _array_element
                          (:`Is Valid`
                            (`SceneComponent.SetRelativeScale3D` _array_element (* (`KismetMathLibrary.Vector_GetAbs` (`SceneComponent.RelativeScale3D` _array_element)) (1.0 -1.0 1.0)))
                            (bind (_returnvalue_x _returnvalue_y) (`KismetMathLibrary.BreakVector2D` (`WidgetComponent.GetPivot` _array_element)))
                            (`WidgetComponent.SetPivot` _array_element (`KismetMathLibrary.MakeVector2D` (select `int` (`local.Local_Index`) :`0` 1.0 :`1` 0.5 :!type "Float (single-precision)") _returnvalue_y))
                            (if (== (`Item.ItemID` _local_item) "/Game/WeaponsNTools/ChargeBlaster/ID_ChargeBlaster.ID_ChargeBlaster")
                              (bind _aswpn_charge_blaster (cast `/Game/WeaponsNTools/ChargeBlaster/WPN_ChargeBlaster` _local_item))
                              (`WidgetComponent.SetPivot` (`/Game/WeaponsNTools/ChargeBlaster/WPN_ChargeBlaster.Widget_ChargeNew` _aswpn_charge_blaster) (1.0 1.0))
                              (elif (== (`local.Local_Index`) 10)
                                (`WidgetComponent.SetPivot` _array_element (`KismetMathLibrary.MakeVector2D` (select `int` _pivotindex :`0` 1.0 :`1` 0.5 :!type "Float (single-precision)") _returnvalue_y))
                                (`self.Debug Message` "index" (`KismetStringLibrary.Conv_IntToString` _pivotindex))))))))))
                (:`Is Not Valid`
                  (`self.Debug Message` "Player Character" "Is Not Valid"))))))))))

(fn `ConvertItemToRightSide`
  (params (TargetItem :type "Item Object Reference"))
  (locals (Local_Item :type "Item Object Reference") (Local_Index :type Integer :default 0))
  (bind (_value _returnvalue) (`BlueprintMapLibrary.Map_Find` (`self.DefaultFPWidgetInfos`) (`GameplayStatics.GetObjectClass` (`local.Local_Item`))))
  (bind (_fpwidget _pivot _scale) (break `/Game/_DRGModding/_LesnovMods/Consmetics/LeftHandedWeapon/S_SavedFPWidgetLocations` _value))
  (`/Engine/EditorBlueprintResources/StandardMacros.IsValid` TargetItem
    (:`Is Valid`
      (set `local.Local_Item` TargetItem)
      (`self.Debug Message` (`KismetSystemLibrary.GetDisplayName` (`local.Local_Item`)) "RHS")
      (`SceneComponent.SetRelativeScale3D` (`self.FPMesh`) (0.6 0.6 0.6))
      (set `PlayerCharacter.AimSettings` (`self.Aim Settings`) (`self.Player Character`))
      (`SceneComponent.K2_SetRelativeRotation` (`self.FPMesh`) (`KismetMathLibrary.MakeRotator` 0.0 0.0 -90.0) false false)
      (if _returnvalue
        (for (_array_element _array_index) _fpwidget
          (`/Engine/EditorBlueprintResources/StandardMacros.IsValid` _array_element
            (:`Is Valid`
              (`SceneComponent.SetRelativeScale3D` _array_element (`|GetArrayItem` _scale _array_index))
              (`WidgetComponent.SetPivot` _array_element (`|GetArrayItem` _pivot _array_index)))))))))

(fn `Debug Message`
  (params (Sender :type String) (Text :type String))
  (`/Game/_DRGModding/_Frameworks/BML_Framework.PrintViaChat` (`/Game/_DRGModding/_LesnovMods/Consmetics/LeftHandedWeapon/LHWSavegame.DisableDBMsg` (`self.As LHWSavegame`)) Sender Text))

(fn `FillFPWidgetInfos`
  (params (Object :type "Item Object Reference"))
  (locals (NewLocalVar_1 :type "Array of FirstPersonWidgetComponent Object Reference") (NewLocalVar_2 :type "Array of Vector2D Structure") (NewLocalVar_3 :type "Array of Vector Structure"))
  (if (not (`.ReturnValue` (`BlueprintMapLibrary.Map_Find` (`self.DefaultFPWidgetInfos`) (`self.CurrentItemClass`))))
    (for _array_element (`self.K2_GetComponentsByClass` Object "/Script/FSD.FirstPersonWidgetComponent")
      (bind _returnvalue (`KismetArrayLibrary.Array_AddUnique` (`local.NewLocalVar_1`) _array_element))
      (if (!= _returnvalue -1)
        (`KismetArrayLibrary.Array_Add` (`local.NewLocalVar_2`) (`WidgetComponent.GetPivot` _array_element))
        (`KismetArrayLibrary.Array_Add` (`local.NewLocalVar_3`) (`SceneComponent.RelativeScale3D` _array_element))))
    (`BlueprintMapLibrary.Map_Add` (`self.DefaultFPWidgetInfos`) (`self.CurrentItemClass`) (make `/Game/_DRGModding/_LesnovMods/Consmetics/LeftHandedWeapon/S_SavedFPWidgetLocations` (`local.NewLocalVar_1`) (`local.NewLocalVar_2`) (`local.NewLocalVar_3`)))))

(fn `GetFilterIndexByItemID`
  (params (Item :type "Item Object Reference"))
  (returns (SelectedIndex :type Integer))
  (locals (NewLocalVar_0 :type Integer))
  (bind _itemid (`Item.ItemID` Item))
  (if (`BlueprintSetLibrary.Set_Contains` (`self.ItemList_Index1`) _itemid)
    (set `local.NewLocalVar_0` 0)
    (elif (`BlueprintSetLibrary.Set_Contains` (`self.ItemList_Index0`) _itemid)
      (set `local.NewLocalVar_0` 1)
      (elif (== _itemid "/Game/WeaponsNTools/Cryospray/ID_Cryospray.ID_Cryospray")
        (set `local.NewLocalVar_0` 2)
        (elif (== (`GameplayStatics.GetObjectClass` Item) "/Game/WeaponsNTools/HackingTool/ITM_HackingTool.ITM_HackingTool_C")
          (set `local.NewLocalVar_0` 1)
          (else
            (set `local.NewLocalVar_0` 10))))))
  (return (`local.NewLocalVar_0`)))

(fn `Save`
  (`/Game/_DRGModding/_Frameworks/BML_Framework.SaveToSlot(Macro)` (`self.As LHWSavegame`)))

(fn `UserConstructionScript`)