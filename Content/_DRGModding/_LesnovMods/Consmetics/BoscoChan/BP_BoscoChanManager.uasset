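; Manager for the BoscoChan cosmetic mod, which adjusts Bosco in the space rig and in caves.
; StartManager waits for the player; in the space rig it destroys SK_Bosco skeletal mesh actors and overrides item name, description and category.
; In caves, if Bosco is allowed, it polls for BP_Bosco, renames it and binds its state changes to face texture switching.
; Every listed state currently maps to the same face.
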(event `OnStateChanged_Event_0`
  (params (aCurrentState :type "EDroneAIState Enum" :default "Follow"))
  ;[1 1 1] Change Face Texture Based On Bosco's State
  (`/Game/_DRGModding/_LesnovMods/Consmetics/BoscoChan/BFL_BoscoChan.ChangeFaceType` (`Bosco.BoscoMesh` (`self.BP_Bosco`)) (select `EDroneAIState` aCurrentState :!type "Byte")))

(event `StartManager`
  (params (IsInSpacerig :type Boolean))
  (set `self.Is in Spacerig` IsInSpacerig)
  (bind _returnvalue (`/Game/_DRGModding/_LesnovMods/_SharedAssets/BML_Actor.ValidCheck(Wait | SBZPlayerCharacter)`))
  (set `self.Player Character` _returnvalue)
  (`self.RemoveMeshesFromSpacerig`)
  (`self.ChangeSpacerigInfos`)
  (if (`self.Is in Spacerig`)
    _
    (elif (`FSDSaveGame.GetBoscoAllowed` (`GameFunctionLibrary.GetFSDSaveGame` self))
      (bind _returnvalue_2 (`GameplayStatics.GetActorOfClass` "/Game/GameElements/Drone/BP_Bosco.BP_Bosco_C" :!label _label))
      (bind _output_get (set `self.BP_Bosco` _returnvalue_2))
      (`/Engine/EditorBlueprintResources/StandardMacros.IsValid` _output_get
        (:`Is Valid`
          (add `Bosco.OnStateChanged` (`self.BP_Bosco`) (`|CreateDelegate` :!event `OnStateChanged_Event_0`))
          (`self.ChangeCaveInfos`))
        (:`Is Not Valid`
          (`KismetSystemLibrary.Delay` 1.0)
          (goto _label))))))

(fn `ChangeCaveInfos`
  (bind _simpleobjectinfo (`/Game/GameElements/Drone/BP_Bosco.SimpleObjectInfo` (`self.BP_Bosco`)))
  (if (not (`self.Is in Spacerig`))
    (`/Engine/EditorBlueprintResources/StandardMacros.IsValid` (`self.BP_Bosco`)
      (:`Is Valid`
        (`SimpleObjectInfoComponent.SetInGameName` _simpleobjectinfo (`self.Name(Cave)`))
        (`SimpleObjectInfoComponent.SetInGameDescription` _simpleobjectinfo (`self.Description(Cave)`))))))

(fn `ChangeSpacerigInfos`
  (bind _itemdata (`self.ItemData`))
  (if (`self.Is in Spacerig`)
    (set `ItemData.Name` (`self.Name`) _itemdata)
    (set `ItemData.Description` (`self.Description`) _itemdata)
    (set `ItemData.Category` (`self.Category`) _itemdata)))

(fn `RemoveMeshesFromSpacerig`
  (if (`self.Is in Spacerig`)
    (bind _outactors (`GameplayStatics.GetAllActorsOfClass` "/Script/Engine.SkeletalMeshActor"))
    (for _array_element _outactors
      (if (`KismetStringLibrary.Contains` (`KismetSystemLibrary.GetObjectName` _array_element) "SK_Bosco")
        (`self.K2_DestroyActor` _array_element)))))

(fn `UserConstructionScript`)