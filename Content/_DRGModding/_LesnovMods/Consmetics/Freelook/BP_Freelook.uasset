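; Deep Rock Galactic mod actor that lets the local player look around independently of aim, via a hold or toggle Freelook key.
; It switches the view to its own camera attached to the first-person camera, blocks look input, and rotates that camera from mouse axes on Tick within clamped limits.
; Release eases rotation back by timeline before restoring the character view.
; A hub menu page saves toggle mode and sensitivity.
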(event `OnButtonPressed_Event_0`
  (params (IsChecked :type Boolean))
  (bind _as_save_game_freelook (`self.As Save Game Freelook`))
  (set `/Game/_DRGModding/_LesnovMods/Consmetics/Freelook/SaveGameFreelook.IsToggle` IsChecked _as_save_game_freelook)
  (`/Game/_DRGModding/_Frameworks/BML_Framework.SaveToSlot(Macro)` _as_save_game_freelook))

(event `OnSliderValueChanged_Event_0`
  (params (Value :type "Float (double-precision)"))
  (bind _as_save_game_freelook (`self.As Save Game Freelook`))
  (set `/Game/_DRGModding/_LesnovMods/Consmetics/Freelook/SaveGameFreelook.FreelookSensitive` Value _as_save_game_freelook)
  (`/Game/_DRGModding/_Frameworks/BML_Framework.SaveToSlot(Macro)` _as_save_game_freelook))

(event `CustomEvent_0`
  (params (Pawn :type "Pawn Object Reference"))
  (bind _playercharacter (`/Game/_DRGModding/_Frameworks/BML_Framework.GetLocalPlayerCharacter(Macro)` true :!label _label)
    (:`Exec`
      (set `self.Player Character` _playercharacter)
      (`self.NewFunction_1`)
      (`PrimitiveComponent.SetOnlyOwnerSee` (`PlayerCharacter.FPMesh` (`self.Player Character`)) false)
      (if (not (`KismetSystemLibrary.IsValidClass` "/Game/_DRGModding/_LesnovMods/Consmetics/ForceFirstPerson/BP_ForceFirstPerson.BP_ForceFirstPerson_C"))
        (add `PlayerCharacter.OnCameraModeChanged` (`self.Player Character`) (delegate `OnCameraModeChanged_Event_0`))))))

(event `self.ReceiveBeginPlay`
  (bind _hubmenu (`self.HUBMENU`))
  (bind _cui_button_toggle (`/Game/_DRGModding/_LesnovMods/Consmetics/Freelook/HUBMENU_Freelook.CUI_Button_Toggle` _hubmenu))
  (bind _cui_slider_1 (`/Game/_DRGModding/_LesnovMods/Consmetics/Freelook/HUBMENU_Freelook.CUI_Slider_1` _hubmenu))
  (bind _returnvalue (`|CreateWidget` "/Game/_DRGModding/_LesnovMods/Consmetics/Freelook/HUBMENU_Freelook.HUBMENU_Freelook_C"))
  (set `self.HUBMENU` _returnvalue)
  (bind _outputpin (`/Game/_DRGModding/_Frameworks/BML_Framework.HandleSaveGame` "/Game/_DRGModding/_LesnovMods/Consmetics/Freelook/SaveGameFreelook.SaveGameFreelook_C")
    (:`then`
      (bind _assave_game_freelook (cast `/Game/_DRGModding/_LesnovMods/Consmetics/Freelook/SaveGameFreelook` _outputpin))
      (set `self.As Save Game Freelook` _assave_game_freelook)
      (`/Game/_DRGModding/_Frameworks/Widget/CUI_Button.Initialize` _cui_button_toggle (`/Game/_DRGModding/_LesnovMods/Consmetics/Freelook/SaveGameFreelook.IsToggle` (`self.As Save Game Freelook`)))
      (add `/Game/_DRGModding/_Frameworks/Widget/CUI_Button.OnButtonPressed` _cui_button_toggle (delegate `OnButtonPressed_Event_0`))
      (add `/Game/_DRGModding/_Frameworks/Widget/CUI_Slider.OnSliderValueChanged` _cui_slider_1 (delegate `OnSliderValueChanged_Event_0`))
      (`/Game/_DRGModding/_Frameworks/Widget/CUI_Slider.Initialize` _cui_slider_1 (`/Game/_DRGModding/_LesnovMods/Consmetics/Freelook/SaveGameFreelook.FreelookSensitive` (`self.As Save Game Freelook`)))
      (bind _fsdplayercontroller (`/Game/_DRGModding/_Frameworks/BML_Framework.GetLocalPlayerController(Macro)` true)
        (:`Completed`
          (bind _output_get (set `self.FSDPlayer Controller` _fsdplayercontroller))
          (`self.EnableInput` _output_get)
          (add `FSDPlayerController.OnPlayerCharacterPossesed` (`self.FSDPlayer Controller`) (delegate `CustomEvent_0`))
          (goto _label))))))

(event `OnCameraModeChanged_Event_0`
  (params (NewCameraMode :type "ECharacterCameraMode Enum" :default "FirstPerson") (OldCameraMode :type "ECharacterCameraMode Enum" :default "FirstPerson"))
  (bind _player_character (`self.Player Character`))
  (switch `ECharacterCameraMode` NewCameraMode
    (:`ThirdPerson`
      _)
    (:`Follow`
      _)
    (:`DownCamera`
      _)
    (:`PhotographyMode`
      _))
  (`SceneComponent.SetVisibility` (`Character.Mesh` _player_character) true true)
  (if (not (`PlayerCharacter.IsStandingDown` _player_character))
    (bind _asbp_player_character (cast `/Game/Character/BP_PlayerCharacter` _player_character))
    (`SceneComponent.SetVisibility` (`/Game/Character/BP_PlayerCharacter.EmergencyLight` _asbp_player_character) false false)))

(event `InputAction|Freelook`
  (params (Key :type "Key Structure"))
  (:`Pressed`
    (`self.NewFunction_0`)
    (if (`/Game/_DRGModding/_LesnovMods/Consmetics/Freelook/SaveGameFreelook.IsToggle` (`self.As Save Game Freelook`))
      (`/Engine/EditorBlueprintResources/StandardMacros.FlipFlop`
        (:`A`
          (`self.SetOnlyOwnerSee(EquippedItem)` :!label _label_2)
          (`SceneComponent.SetVisibility` (`Character.Mesh` (`self.Player Character`)) false true)
          (`PlayerController.SetViewTargetWithBlend` (`self.FSDPlayer Controller`) self 0.0 "VTBlend_Linear" 0.0 false)
          (`Controller.SetIgnoreLookInput` (`self.FSDPlayer Controller`) true)
          (`SceneComponent.K2_SetRelativeRotation` :`self` (`self.FreelookCamera`))
          (`self.SetActorTickEnabled` true))
        (:`B`
          (`self.SetActorTickEnabled` false :!label _label_3)
          (`Controller.SetIgnoreLookInput` (`self.FSDPlayer Controller`) false)
          (bind (_direction _newtrack_0) (`Timeline|TL_BackToNormalRotation` :!via `PlayFromStart`)
            (:`Update`
              (`SceneComponent.K2_SetRelativeRotation` (`self.GetTargetCamera`) (`KismetMathLibrary.RLerp` (`SceneComponent.RelativeRotation` (`self.GetTargetCamera`)) (struct) _newtrack_0 true) false false))
            (:`Finished`
              (`PlayerController.SetViewTargetWithBlend` (`self.FSDPlayer Controller`) (`self.Player Character`) 0.0 "VTBlend_Linear" 0.0 false)
              (`Controller.SetIgnoreLookInput` (`self.FSDPlayer Controller`) false)))))
      (else
        (goto _label_2))))
  (:`Released`
    (if (not (`/Game/_DRGModding/_LesnovMods/Consmetics/Freelook/SaveGameFreelook.IsToggle` (`self.As Save Game Freelook`)))
      (goto _label_3))))

(event `self.ReceiveTick`
  (params (DeltaSeconds :type "Float (single-precision)"))
  (bind (_relativerotation_roll _relativerotation_pitch _relativerotation_yaw) (`KismetMathLibrary.BreakRotator` (`SceneComponent.RelativeRotation` (`self.FreelookCamera`))))
  (bind (_returnvalue_roll _returnvalue_pitch) (`KismetMathLibrary.BreakRotator` (`SceneComponent.K2_GetComponentRotation` (`PlayerCharacter.FirstPersonCamera` (`self.Player Character`)))))
  ;[1 1 1] Event Tick - Set Freelook camera's rotation by mouse X and Y.
  (`SceneComponent.K2_SetRelativeRotation` (`self.FreelookCamera`) (`KismetMathLibrary.MakeRotator` 0.0 (`KismetMathLibrary.FClamp` (`self.GetFreelookRotation` (`self.GetInputAxisKeyValue`) _relativerotation_pitch) (select `bool` (< _returnvalue_pitch 0.0) :`false` -89.0 :`true` (+ (* -1 _returnvalue_pitch) -89.0)) (select `bool` (> _returnvalue_pitch 0.0) :`false` 89.0 :`true` (- 89.0 _returnvalue_pitch))) (`KismetMathLibrary.FClamp` (`self.GetFreelookRotation` (`self.GetInputAxisKeyValue`) _relativerotation_yaw) -179.0 179.0)) false false))

(fn `GetFreelookRotation`
  (params (Value :type "Float (double-precision)") (RotationFrom :type "Float (double-precision)"))
  (returns (ReturnValue :type "Float (double-precision)"))
  (return (+ (* (* (`GameplayStatics.GetWorldDeltaSeconds`) Value) (`/Game/_DRGModding/_LesnovMods/Consmetics/Freelook/SaveGameFreelook.FreelookSensitive` (`self.As Save Game Freelook`))) RotationFrom)))

(fn `GetModInfo`
  (returns (ModName :type Text) (ModAuthor :type Text) (ModVersion :type Text))
  (return "Freelook" "Lesnov" "1.0.0"))

(fn `GetModPages`
  (returns (HubPages :type "Array of /Game/_ModHub/IHubPageWidget Interface"))
  (return (`|MakeArray` (`self.HUBMENU`) :!type "/Game/_ModHub/IHubPageWidget Interface")))

(fn `GetTargetCamera`
  (returns (FreelookCamera :type "CameraComponent Object Reference"))
  (return (`self.FreelookCamera`)))

(fn `NewFunction_0`
  (`/Engine/EditorBlueprintResources/StandardMacros.IsValid` (`self.FreelookCamera`)
    (:`Is Valid`
      (`SceneComponent.K2_AttachToComponent` (`self.FreelookCamera`) (`PlayerCharacter.FirstPersonCamera` (`self.Player Character`)) "None" "SnapToTarget" "SnapToTarget" "SnapToTarget" true)
      (for _array_element (`self.K2_GetComponentsByClass` "/Script/Engine.CameraComponent")
        (if (!= _array_element (`self.FreelookCamera`))
          (`ActorComponent.Deactivate` _array_element))))
    (:`Is Not Valid`
      (`self.NewFunction_1`))))

(fn `NewFunction_1`
  (bind _returnvalue (`AddComponent|NODE_AddCameraComponent-2`))
  (bind _output_get (set `self.FreelookCamera` _returnvalue))
  (`SceneComponent.K2_AttachToComponent` _output_get (`PlayerCharacter.FirstPersonCamera` (`self.Player Character`)) "None" "SnapToTarget" "SnapToTarget" "SnapToTarget" true)
  (for _array_element (`self.K2_GetComponentsByClass` "/Script/Engine.CameraComponent")
    (if (!= _array_element (`self.FreelookCamera`))
      (`ActorComponent.Deactivate` _array_element))))

(fn `SetOnlyOwnerSee(EquippedItem)`
  (bind _returnvalue (`/Game/_DRGModding/_Frameworks/BML_Framework.GetCurrentItem` (`self.Player Character`)))
  (for _array_element (`self.K2_GetComponentsByClass` _returnvalue "/Script/FSD.FirstPersonSkeletalMeshComponent")
    (`/Engine/EditorBlueprintResources/StandardMacros.IsValid` _array_element
      (:`Is Valid`
        (`PrimitiveComponent.SetOnlyOwnerSee` _array_element false))))
  (for _array_element_2 (`self.K2_GetComponentsByClass` _returnvalue "/Script/FSD.FirstPersonStaticMeshComponent")
    (`/Engine/EditorBlueprintResources/StandardMacros.IsValid` _array_element_2
      (:`Is Valid`
        (`PrimitiveComponent.SetOnlyOwnerSee` _array_element_2 false)))))

(fn `UserConstructionScript`
  (`TimelineComponent.SetPlayRate` (`self.TL_BackToNormalRotation`) 5.0))