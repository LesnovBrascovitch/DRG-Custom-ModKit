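; Billboard actor that plays flipbook animations from a list of materials in sequence for the custom victory pose framework, with optional 2D or positional music.
; It can first spawn a prop and wait for its finished event.
; Each material becomes a dynamic instance on one billboard component, and a replayed timeline drives its animation phase while opacity toggles between them.
; The last frame can be clamped, then optionally faded and destroyed.
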(event `self.ReceiveBeginPlay`
  (`MaterialBillboardComponent.SetElements` (`self.MaterialBillboard`) (`|MakeArray` (make `MaterialSpriteElement` null) :!type "MaterialSpriteElement Structure"))
  (if (`self.UseProp`)
    (bind _returnvalue (`|SpawnActorFromClass` (`self.PropClass`) (`KismetMathLibrary.MakeTransform` (`self.K2_GetActorLocation`)) "AlwaysSpawn" "OverrideRootScale" null null))
    (bind _output_get (set `self.InstancedProp` _returnvalue))
    (add `/Game/_DRGModding/_LesnovMods/Consmetics/CustomVictoryPose/_Framework/BP_BillboardFlipbook_Prop.OnPropFinished` _output_get (delegate `OnPropFinished_Event_0`))
    (else
      (`self.StartAnimation`))))

(event `OnPropFinished_Event_0`
  (`self.StartAnimation`))

(event `StartAnimation`
  (`|ExecutionSequence`
    (:`then_0`
      (`/Engine/EditorBlueprintResources/StandardMacros.IsValid` (`self.StartMusic`)
        (:`Is Valid`
          (`KismetSystemLibrary.Delay` (`self.StartMusicDelay`))
          (if (`self.Is2DSound`)
            (bind _returnvalue (`GameplayStatics.SpawnSound2D` (`self.StartMusic`) 1.0 1.0 0.0 null))
            (set `self.SpawnedSound` _returnvalue)
            (else
              (bind _returnvalue_2 (`GameplayStatics.SpawnSoundAtLocation` (`self.StartMusic`) (`self.K2_GetActorLocation`) (struct) 1.0 1.0 0.0 null null))
              (set `self.SpawnedSound` _returnvalue_2))))))
    (:`then_1`
      (bind _dmis (`self.PrepareFlipbook`))
      (`self.AddToBillboardMaterial` _dmis)
      (`TimelineComponent.SetPlayRate` (`self.Timeline_0`) (`self.Playrate`))
      (if (<= (`self.Index`) (`KismetArrayLibrary.Array_LastIndex` (`MaterialBillboardComponent.Elements` (`self.MaterialBillboard`)))) :!label _label
        (`self.StatePreCheck`)
        (bind (_direction _newtrack_0) (`Timeline|Timeline_0` :!via `PlayFromStart`)
          (:`Update`
            (if (`self.IsLast`)
              (`MaterialInstanceDynamic.SetScalarParameterValue` (`self.SelectedDMI`) "Animation  Phase (0-1) (S)" (`KismetMathLibrary.FClamp` _newtrack_0 0.0 (`self.LastFrameClamp`)))
              (else
                (`MaterialInstanceDynamic.SetScalarParameterValue` (`self.SelectedDMI`) "Animation  Phase (0-1) (S)" _newtrack_0))))
          (:`Finished`
            (if (`self.IsLast`)
              (`self.OnAnimationFinished`)
              (else
                (`MaterialInstanceDynamic.SetScalarParameterValue` (`|GetArrayItem` (`self.DMIs`) (`self.Index`)) "OpacityOffset" 0.0)
                (`/Engine/EditorBlueprintResources/StandardMacros.IncrementInt` (`self.Index`)
                  (:`  `
                    (goto _label)))))))))))

(event `OnAnimationFinished`
  (if (`self.DestroyOnFinish`)
    (`KismetSystemLibrary.Delay` (`self.DelayDestroy`))
    (if (`self.FadeOnDestroy`)
      (`TimelineComponent.SetPlayRate` (`self.Timeline_1`) 3.0)
      (bind (_direction _newtrack_0) (`Timeline|Timeline_1` :!via `PlayFromStart`)
        (:`Update`
          (`MaterialInstanceDynamic.SetScalarParameterValue` (`|GetArrayItem` (`self.DMIs`) (`KismetArrayLibrary.Array_LastIndex` (`self.DMIs`))) "OpacityOffset" (`KismetMathLibrary.Lerp` 1.0 0.0 _newtrack_0)))
        (:`Finished`
          (`self.K2_DestroyActor`)))
      (else
        (`self.K2_DestroyActor`)))))

(event `self.ReceiveDestroyed`
  (bind _instancedprop (`self.InstancedProp`))
  (bind _spawnedsound (`self.SpawnedSound`))
  (`/Engine/EditorBlueprintResources/StandardMacros.IsValid` _spawnedsound
    (:`Is Valid`
      (`AudioComponent.FadeOut` _spawnedsound 0.1 0.1 "Linear"))
    (:`Is Not Valid`
      _))
  (`/Engine/EditorBlueprintResources/StandardMacros.IsValid` _instancedprop
    (:`Is Valid`
      (`/Game/_DRGModding/_LesnovMods/Consmetics/CustomVictoryPose/_Framework/BP_BillboardFlipbook_Prop.OnParentDestroyed` _instancedprop))))

(fn `AddToBillboardMaterial`
  (params (DMIs :type "Array of MaterialInstanceDynamic Object Reference"))
  (locals (NewLocalVar_0 :type "Array of MaterialSpriteElement Structure"))
  (bind _size (`self.Size`))
  (for _array_element DMIs
    (`KismetArrayLibrary.Array_AddUnique` (`local.NewLocalVar_0`) (make `MaterialSpriteElement` _array_element null false _size _size)))
  (`MaterialBillboardComponent.SetElements` (`self.MaterialBillboard`) (`local.NewLocalVar_0`)))

(fn `PrepareFlipbook`
  (returns (DMIs :type "Array of MaterialInstanceDynamic Object Reference"))
  (for _array_element (`self.Materials`)
    (bind _returnvalue (`KismetMaterialLibrary.CreateDynamicMaterialInstance` _array_element))
    (`MaterialInstanceDynamic.SetScalarParameterValue` _returnvalue "Contrast (S)" (`self.Contrast`))
    (`MaterialInstanceDynamic.SetScalarParameterValue` _returnvalue "FlipbookRows" (`KismetMathLibrary.Conv_IntToDouble` (`self.FlipbookRow`)))
    (`MaterialInstanceDynamic.SetScalarParameterValue` _returnvalue "OpacityOffset" 0.0)
    (`MaterialInstanceDynamic.SetScalarParameterValue` _returnvalue "EmissiveOffset" (`self.EmissiveOffset`))
    (`KismetArrayLibrary.Array_AddUnique` (`self.DMIs`) _returnvalue))
  (return (`self.DMIs`)))

(fn `PrepareFlipbook(Preview)`
  (returns (OutputPin :type "MaterialInstanceDynamic Object Reference"))
  (bind _returnvalue (`KismetMaterialLibrary.CreateDynamicMaterialInstance` (`|GetArrayItem` (`self.Materials`))))
  (`MaterialInstanceDynamic.SetScalarParameterValue` _returnvalue "Contrast (S)" (`self.Contrast`))
  (`MaterialInstanceDynamic.SetScalarParameterValue` _returnvalue "FlipbookRows" (`KismetMathLibrary.Conv_IntToDouble` (`self.FlipbookRow`)))
  (`MaterialInstanceDynamic.SetScalarParameterValue` _returnvalue "OpacityOffset" 1.0)
  (`MaterialInstanceDynamic.SetScalarParameterValue` _returnvalue "EmissiveOffset" (`self.EmissiveOffset`))
  (return _returnvalue))

(fn `StatePreCheck`
  (`MaterialInstanceDynamic.SetScalarParameterValue` (`|GetArrayItem` (`self.DMIs`) (`self.Index`)) "OpacityOffset" 1.0)
  (set `self.IsLast` (== (`self.Index`) (`KismetArrayLibrary.Array_LastIndex` (`MaterialBillboardComponent.Elements` (`self.MaterialBillboard`)))))
  (set `self.SelectedDMI` (`|GetArrayItem` (`self.DMIs`) (`self.Index`))))

(fn `UserConstructionScript`
  (bind _size (`self.Size`))
  (bind _outputpin (`self.PrepareFlipbook(Preview)`))
  (`MaterialBillboardComponent.SetElements` (`self.MaterialBillboard`) (`|MakeArray` (make `MaterialSpriteElement` _outputpin null false _size _size) :!type "MaterialSpriteElement Structure")))