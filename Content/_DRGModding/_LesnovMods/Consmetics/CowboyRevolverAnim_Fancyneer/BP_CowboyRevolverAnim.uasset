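; Cosmetic mod actor that gives the local player's revolver cowboy-stance animations when a specific clip-size overclock is equipped.
; It binds to inventory equip and unequip events, rebinding whenever the player character is possessed.
; On equip it swaps the animation set and equip, fire, reload and gunsling montages, disables inspection, then plays a stance montage after a short delay.
; Reload completion replays the stance-enter montage; unequipping unbinds that handler.
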(event `self.ReceiveBeginPlay`
  (bind _fsdplayercontroller (`/Game/_DRGModding/_Frameworks/BML_Framework.GetLocalPlayerController(Macro)` true)
    (:`Completed`
      (set `self.FSDPlayer Controller` _fsdplayercontroller)
      (add `FSDPlayerController.OnPlayerCharacterPossesed` (`self.FSDPlayer Controller`) (delegate `OnPlayerCharacterPossesed_Event_0`))
      (bind _playercharacter (`/Game/_DRGModding/_Frameworks/BML_Framework.GetLocalPlayerCharacter(Macro)` true :!label _label)
        (:`Exec`
          (set `self.Player Character` _playercharacter)
          (bind _inventorycomponent (`PlayerCharacter.InventoryComponent` _playercharacter))
          (add `InventoryComponent.OnItemEquipped` _inventorycomponent (delegate `OnItemEquipped_Event_0`))
          (add `InventoryComponent.OnItemUnequipped` _inventorycomponent (delegate `OnItemUnequipped_Event_0`)))))))

(event `OnPlayerCharacterPossesed_Event_0`
  (params (Pawn :type "Pawn Object Reference"))
  (goto _label))

(event `OnItemEquipped_Event_0`
  (params (Item :type "Item Object Reference"))
  (if (== (`GameplayStatics.GetObjectClass` Item) "/Game/WeaponsNTools/Revolver/WPN_Revolver.WPN_Revolver_C")
    (bind _aswpn_revolver (cast `/Game/WeaponsNTools/Revolver/WPN_Revolver` Item))
    (if (== (`UpgradableGearComponent.GetEquippedOverclock` (`Item.UpgradableItem` _aswpn_revolver) "/Game/WeaponsNTools/Revolver/WPN_Revolver.WPN_Revolver_C") "/Game/WeaponsNTools/Revolver/Overclocks/OC_Revolver_ClipSize_B.OC_Revolver_ClipSize_B")
      (`/Game/_DRGModding/_Frameworks/BML_Framework.UpdateAnims(AnimatedItem)` _aswpn_revolver "/Game/_DRGModding/_LesnovMods/Consmetics/CowboyRevolverAnim_Fancyneer/IAS_Pistol_CowboyRevolver.IAS_Pistol_CowboyRevolver" "/Game/_DRGModding/_LesnovMods/GameplayMods/_WeaponStanceChanger/Mod_CowboyStance/Animations/Cowboy_Equip_Montage.Cowboy_Equip_Montage" false)
      (`/Game/_DRGModding/_Frameworks/BML_Framework.UpdateAnims(AmmoDrivenWeapon)` _aswpn_revolver "/Game/_DRGModding/_LesnovMods/GameplayMods/_WeaponStanceChanger/Mod_CowboyStance/Animations/CowboyStance_Fire_Montage.CowboyStance_Fire_Montage" "/Game/_DRGModding/_LesnovMods/Consmetics/CowboyRevolverAnim_Fancyneer/Fixed_CowboyStance_ExitReload_Montage.Fixed_CowboyStance_ExitReload_Montage" "/Game/_DRGModding/_LesnovMods/Consmetics/CowboyRevolverAnim_Fancyneer/Fixed_CowboyStance_RevolverReload_Montage.Fixed_CowboyStance_RevolverReload_Montage" (`|MakeArray` (make `ItemAnimationItem` "/Game/_DRGModding/_LesnovMods/GameplayMods/_WeaponStanceChanger/Mod_CowboyStance/Animations/FP_CowboyStance_Gunsling_Montage.FP_CowboyStance_Gunsling_Montage" null "/Game/_DRGModding/_LesnovMods/GameplayMods/_WeaponStanceChanger/Mod_CowboyStance/Animations/WPN_CowboyStance_RevolverGunsling_Montage.WPN_CowboyStance_RevolverGunsling_Montage") :!type "ItemAnimationItem Structure"))
      (add `ClipBasedItemAggregator.OnReloadComplete` (`AmmoDrivenWeapon.Aggregator` _aswpn_revolver) (`|CreateDelegate` :!event `OnReloadComplete_Event_0`))
      (`KismetSystemLibrary.Delay` 0.1)
      (`/Game/_DRGModding/_Frameworks/BML_Framework.PlayMontage(FPMesh)` (`self.Player Character`) "/Game/_DRGModding/_LesnovMods/GameplayMods/_WeaponStanceChanger/Mod_CowboyStance/Animations/CowboyStance_ExitReload_Montage.CowboyStance_ExitReload_Montage"))))

(event `OnItemUnequipped_Event_0`
  (params (Item :type "Item Object Reference"))
  (if (== (`GameplayStatics.GetObjectClass` Item) "/Game/WeaponsNTools/Revolver/WPN_Revolver.WPN_Revolver_C")
    (bind _aswpn_revolver (cast `/Game/WeaponsNTools/Revolver/WPN_Revolver` Item))
    (remove `ClipBasedItemAggregator.OnReloadComplete` (`AmmoDrivenWeapon.Aggregator` _aswpn_revolver) (`|CreateDelegate` :!event `OnReloadComplete_Event_0`))))

(event `OnReloadComplete_Event_0`
  (`/Game/_DRGModding/_Frameworks/BML_Framework.PlayMontage(FPMesh)` (`self.Player Character`) "/Game/_DRGModding/_LesnovMods/GameplayMods/_WeaponStanceChanger/Mod_CowboyStance/Animations/CowboyStance_Enter_Montage.CowboyStance_Enter_Montage"))

(fn `UserConstructionScript`)