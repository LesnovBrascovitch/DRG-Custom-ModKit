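; BP_Terminal_TakidashiComic is an interactive terminal that displays random Takidashi comic images on a widget.
; It enables local input, and Use line-traces from the first-person camera to detect hits on itself.
; A hit plays a slap montage and button sound, shows another image and rocks Bosco with a randomised timeline roll.
; Images are drawn without repeats from a cached array that refills when empty.
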(event `self.ReceiveBeginPlay`
  (bind _asmenu_takidashi_comic (cast `/Game/_DRGModding/_LesnovMods/Consmetics/TakidashiComics/Menu_TakidashiComic` (`WidgetComponent.GetWidget` (`self.MangaWidget`))))
  (set `self.As Menu Takidashi Comic` _asmenu_takidashi_comic)
  (`self.EnableInput` (`/Game/_DRGModding/_LesnovMods/_SharedAssets/BML_Actor.GetLocalPlayerController(Comp)`))
  (set `self.ImageSetsCache` (`self.ImageSets`))
  (`self.NewFunction_0`))

(event `InputAction|Use` :consume false
  (params (Key :type "Key Structure"))
  (bind _firstpersoncamera (`PlayerCharacter.FirstPersonCamera` (`GameFunctionLibrary.GetLocalPlayerCharacter`)))
  (bind _returnvalue (`SceneComponent.K2_GetComponentLocation` _firstpersoncamera))
  (:`Pressed`
    (bind (_outhit _returnvalue_2) (`KismetSystemLibrary.LineTraceSingle` _returnvalue (+ _returnvalue (* (`KismetMathLibrary.GetForwardVector` (`SceneComponent.K2_GetComponentRotation` _firstpersoncamera)) 300)) "TraceTypeQuery7" true (`|MakeArray` (`GameFunctionLibrary.GetLocalPlayerCharacter`) :!type "Actor Object Reference") "ForDuration" false))
    (if _returnvalue_2
      (if (== (`.HitActor` (`GameplayStatics.BreakHitResult` _outhit)) self)
        (`|PlayMontage` (`PlayerCharacter.FPMesh` (`GameFunctionLibrary.GetLocalPlayerCharacter`)) "/Game/CharacterStructure/Gear_Unarmed/FP/1P_Unarmed_Slap_A_Montage.1P_Unarmed_Slap_A_Montage"
          (:`then`
            (`self.NewFunction_0`)
            (`GameplayStatics.SpawnSoundAtLocation` "/Game/Audio/SFX/Characters/Arcade/ArcadeButtonPush_Cue.ArcadeButtonPush_Cue" (`SceneComponent.K2_GetComponentLocation` (`self.MonitorMain`)) (struct) 1.0 1.0 0.0 null null)
            (`self.OnTerminalInteract`)))))))

(event `OnTerminalInteract`
  (if (not (`TimelineComponent.IsPlaying` (`self.Timeline_0`)))
    (set `self.RotationOffset` (`KismetMathLibrary.RandomFloatInRange` 9.0 11.0))
    (bind (_direction _newtrack_0) (`Timeline|Timeline_0` :!via `PlayFromStart`)
      (:`Update`
        (`SceneComponent.K2_SetRelativeRotation` (`self.Bosco`) (`KismetMathLibrary.MakeRotator` (`KismetMathLibrary.Lerp` 8.0 (`self.RotationOffset`) _newtrack_0) 0.0 -180.0) false false)))))

(fn `NewFunction_0`
  (locals (NewLocalVar_0 :type "Texture2D Object Reference"))
  (bind (_outitem _outindex) (`KismetArrayLibrary.Array_Random` (`self.ImageSetsCache`)))
  (if (== _outindex -1)
    (set `self.ImageSetsCache` (`self.ImageSets`)))
  (bind _output_get (set `local.NewLocalVar_0` _outitem))
  (`/Game/_DRGModding/_LesnovMods/Consmetics/TakidashiComics/Menu_TakidashiComic.SetImage` (`self.As Menu Takidashi Comic`) _output_get)
  (`KismetArrayLibrary.Array_RemoveItem` (`self.ImageSetsCache`) (`local.NewLocalVar_0`)))

(fn `UserConstructionScript`)