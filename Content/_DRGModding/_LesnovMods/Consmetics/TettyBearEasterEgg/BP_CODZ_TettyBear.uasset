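; BP_CODZ_TettyBear is a usable teddy bear for a Call of Duty Zombies-style music easter egg.
; On first use, guarded by a DoOnce, it marks itself used, plays an activation sound and checks every bear of its class in the level.
; If any bear remains unused it prints a notice; otherwise it plays a boss music cue in 2D and prints that the song played.
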(event `self.InstantUsable.OnUsedBy`
  (params (User :type "PlayerCharacter Object Reference") (Key :type "EInputKeys Enum" :default "Use"))
  (`/Engine/EditorBlueprintResources/StandardMacros.DoOnce` false
    (:`Completed`
      (set `self.IsUsed` true)
      (`/Game/_DRGModding/_LesnovMods/_SharedAssets/BML_Actor.PlaySoundAtSelf` "/Game/_DRGModding/_LesnovMods/Consmetics/TettyBearEasterEgg/TeddyBearActivate_Cue.TeddyBearActivate_Cue")
      (bind _outactors (`GameplayStatics.GetAllActorsOfClass` "BP_CODZ_TettyBear_C"))
      (for _array_element _outactors
        (if (not (`/Game/_DRGModding/_LesnovMods/Consmetics/TettyBearEasterEgg/BP_CODZ_TettyBear.IsUsed` _array_element))
          (set `self.IsUsed_0` true)))
      (if (`self.IsUsed_0`)
        (`KismetSystemLibrary.PrintString` "Not All Teddy Bear Activated")
        (else
          (`GameplayStatics.PlaySound2D` "/Game/_DRGModding/_LesnovMods/Consmetics/TettyBearEasterEgg/St_Boss_Music_Cue.St_Boss_Music_Cue" 1.0 1.0 0.0 null null)
          (`KismetSystemLibrary.PrintString` "Teddy Bear Song Played"))))))

(fn `UserConstructionScript`)