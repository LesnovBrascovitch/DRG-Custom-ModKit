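; Free-fly camera actor that moves with WASD, speeds up on Left Shift, and returns view to the player on Space or DisableCamera.
; Tick offsets the actor by GetTargetOffset, whose forward/right movement math is not connected to any output.
; The activation chain, which positions the camera behind the player, takes over view and input and clears camera feedbacks, is unreachable, as OnControl is empty.
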(event `self.ReceiveBeginPlay`)

(event `/Game/_DRGModding/_LesnovMods/_SharedAssets/BPI_Controllable.OnControl`)

(event `Key|LeftShift`
  (params (Key :type "Key Structure"))
  (:`Pressed`
    (set `self.MoveSpeed` 15.0))
  (:`Released`
    (set `self.MoveSpeed` 8.0)))

(event `Key|SpaceBar`
  (params (Key :type "Key Structure"))
  (bind _player_controller (`self.Player Controller`))
  (:`Pressed`
    (`self.DisableInput` _player_controller :!label _label)
    (`PlayerController.SetViewTargetWithBlend` _player_controller (`GameplayStatics.GetPlayerCharacter` 0) 0.0 "VTBlend_Linear" 0.0 false)
    (`self.OnEmoteStoppedKeyPressed`)
    (set `self.A` false)
    (set `self.S` false)
    (set `self.W` false)
    (set `self.D` false)
    (`self.SetActorTickEnabled` false)))

(event `DisableCamera`
  (goto _label))

(event `self.ReceiveTick`
  (params (DeltaSeconds :type "Float (single-precision)"))
  (`self.K2_AddActorWorldOffset` (+ (* (`self.GetActorForwardVector`) (* (+ (`KismetMathLibrary.SelectFloat` 1.0 0.0 (`self.W`)) (`KismetMathLibrary.SelectFloat` -1.0 0.0 (`self.S`))) (`self.MoveSpeed`))) (* (`self.GetActorRightVector`) (* (+ (`KismetMathLibrary.SelectFloat` 1.0 0.0 (`self.D`)) (`KismetMathLibrary.SelectFloat` -1.0 0.0 (`self.A`))) (`self.MoveSpeed`))))))

(event `Key|W` :consume false
  (params (Key :type "Key Structure"))
  (:`Pressed`
    (set `self.W` true))
  (:`Released`
    (set `self.W` false)))

(event `Key|S` :consume false
  (params (Key :type "Key Structure"))
  (:`Pressed`
    (set `self.S` true))
  (:`Released`
    (set `self.S` false)))

(event `Key|D` :consume false
  (params (Key :type "Key Structure"))
  (:`Pressed`
    (set `self.D` true))
  (:`Released`
    (set `self.D` false)))

(event `Key|A` :consume false
  (params (Key :type "Key Structure"))
  (:`Pressed`
    (set `self.A` true))
  (:`Released`
    (set `self.A` false)))

(fn `UserConstructionScript`)