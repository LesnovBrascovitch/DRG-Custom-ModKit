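; BP_TPRig_PoseTattoo is a third-person rig preview actor that mirrors a vanity armor material from the local player's character, apparently for tattoos.
; On BeginPlay and on a looping five-second timer, it searches the character mesh's child components for names containing "SK_Vanity_Armor".
; It prints each match to chat and copies that skeletal mesh's second material slot onto the same slot of its BodyMesh.
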(event `CustomEvent_0`
  (bind _playercharacter (`/Game/_DRGModding/_Frameworks/BML_Framework.GetLocalPlayerCharacter(Macro)` true :!label _label)
    (:`Exec`
      (for _array_element (`SceneComponent.GetChildrenComponents` (`Character.Mesh` _playercharacter) true)
        (bind _returnvalue (`KismetSystemLibrary.GetDisplayName` _array_element))
        (if (`KismetStringLibrary.Contains` _returnvalue "SK_Vanity_Armor" false true)
          (`/Game/_DRGModding/_Frameworks/BML_Framework.PrintViaChat` false "" _returnvalue)
          (bind _asskeletal_mesh_component (cast `SkeletalMeshComponent` _array_element))
          (`PrimitiveComponent.SetMaterial` (`self.BodyMesh`) 1 (`PrimitiveComponent.GetMaterial` _asskeletal_mesh_component 1)))))))

(event `self.ReceiveBeginPlay`
  (`parent.ReceiveBeginPlay`)
  (`KismetSystemLibrary.K2_SetTimerDelegate` (delegate `CustomEvent_0`) 5.0 true)
  (goto _label))

(fn `UserConstructionScript`
  (`parent.UserConstructionScript`))