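; Test AI character using the dwarf third-person AnimBP, with randomized walk speed and a DisableAI flag that destroys it on spawn.
; A one-second timer feeds movement state to the AnimBP.
; Hits or Used knock it down after a random delay, setting a Blackboard bool until a timer stands it up.
; Attack plays a kick that launches and damages the local player; the SimpleMoveToActor follow loop is disconnected.
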(event `CustomEvent_0`
  (`/Game/_DRGModding/_Frameworks/BML_Framework.IsInDRG`
    (:`In DRG`
      (if (not (`PlayerAnimInstance.IsLyingDown` (`self.As ABP TP Dwarf`)))
        (`AIBlueprintHelperLibrary.SimpleMoveToActor` (`self.GetController`) (`self.Player Character`) :!label _label)))
    (:`In Editor`
      (goto _label))))

(event `self.ReceiveBeginPlay`
  (if (`self.DisableAI`)
    (`self.K2_DestroyActor`)
    (else
      (bind _asabp_tp_dwarf (cast `/Game/Character/ABP_TP_Dwarf` (`SkeletalMeshComponent.GetAnimInstance` (`self.Mesh`)))
        (:`then`
          (set `self.As ABP TP Dwarf` _asabp_tp_dwarf))
        (:`CastFailed`
          _))
      (bind _playercharacter (`/Game/_DRGModding/_Frameworks/BML_Framework.GetLocalPlayerCharacter(Macro)` true)
        (:`Exec`
          (set `self.Player Character` _playercharacter)
          (`KismetSystemLibrary.K2_SetTimerDelegate` (delegate `CustomEvent_1`) 1.0 true))))))

(event `CustomEvent_1`
  (bind _as_abp_tp_dwarf (`self.As ABP TP Dwarf`))
  (bind _velocity (`MovementComponent.Velocity` (`self.CharacterMovement`)))
  (set `PlayerAnimInstance.IsMoving` (!= _velocity (0.0 0.0 0.0)) _as_abp_tp_dwarf)
  (set `PlayerAnimInstance.Speed` (`KismetMathLibrary.VSize` _velocity) _as_abp_tp_dwarf))

(event `self.SimpleHealth.OnHit`
  (params (Damage :type "Float (single-precision)") (DamageData :type "DamageData Structure (by ref)") (anyHealthLost :type Boolean))
  (`KismetSystemLibrary.Delay` (`KismetMathLibrary.RandomFloatInRange` 0.0 0.7) :!label _label_2)
  (bind _output_get (set `PlayerAnimInstance.IsLyingDown` true (`self.As ABP TP Dwarf`)))
  (`BlackboardComponent.SetValueAsBool` (`AIController.Blackboard` (`AIBlueprintHelperLibrary.GetAIController` self)) (`self.Key Name`) _output_get)
  (`GameplayStatics.SpawnSoundAttached` "/Game/_DRGModding/_SharedAssets/_Lesnov/AI/AIDown.AIDown" (`self.Mesh`) "None" (0.0 0.0 0.0) (struct) "KeepRelativeOffset" false 1.0 1.0 0.0 null null)
  (bind _asaicontroller (cast `AIController` (`self.GetController`))
    (:`then`
      (`Controller.StopMovement` _asaicontroller))
    (:`CastFailed`
      _))
  (`KismetSystemLibrary.K2_SetTimerDelegate` (delegate `CustomEvent_2`) 10.0))

(event `Attack`
  (bind _player_character (`self.Player Character`))
  (`|PlayMontage` (`self.Mesh`) "/Game/CharacterStructure/Gear_Unarmed/TP/3P_Unarmed_Kick_A_Montage.3P_Unarmed_Kick_A_Montage"
    (:`then`
      (`self.LaunchCharacter` _player_character (+ (* (`self.GetActorForwardVector`) 3000) (0.0 0.0 30.0)) false false)
      (`HealthComponentBase.TakeDamageSimple` (`PlayerCharacter.HealthComponent` _player_character) 5.0 _player_character "/Game/GameElements/Damage/DMG_Physical.DMG_Physical"))))

(event `CustomEvent_2`
  (bind _output_get (set `PlayerAnimInstance.IsLyingDown` false (`self.As ABP TP Dwarf`)))
  (`BlackboardComponent.SetValueAsBool` (`AIController.Blackboard` (`AIBlueprintHelperLibrary.GetAIController` self)) (`self.Key Name`) _output_get))

(event `Used`
  (goto _label_2))

(fn `UserConstructionScript`
  (set `CharacterMovementComponent.MaxWalkSpeed` (`KismetMathLibrary.RandomFloatInRange` 400.0 600.0) (`self.CharacterMovement`)))