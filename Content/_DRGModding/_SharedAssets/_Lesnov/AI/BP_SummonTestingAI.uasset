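; BP_SummonTestingAI is a usable test actor that toggles repeated spawning of BP_TestingAI.
; Each use drives a FlipFlop: the first starts a looping timer that spawns AI at a reference object's location with randomized uniform scale.
; The next use clears the timer, destroys all BP_TestingAI actors and forces garbage collection.
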(event `CustomEvent_0`
  (`|SpawnActorFromClass` "/Game/_DRGModding/_SharedAssets/_Lesnov/AI/BP_TestingAI.BP_TestingAI_C" (`KismetMathLibrary.MakeTransform` (`self.K2_GetActorLocation` (`self.NewVar_0`)) (struct) (`KismetMathLibrary.Conv_DoubleToVector` (`KismetMathLibrary.RandomFloatInRange` 0.8 1.1))) "Undefined" "OverrideRootScale" null null))

(event `self.InstantUsable.OnUsedBy`
  (params (User :type "PlayerCharacter Object Reference") (Key :type "EInputKeys Enum" :default "Use"))
  (`/Engine/EditorBlueprintResources/StandardMacros.FlipFlop` :!label _label
    (:`A`
      (bind _returnvalue (`KismetSystemLibrary.K2_SetTimerDelegate` (delegate `CustomEvent_0`) 1.0 true)))
    (:`B`
      (`KismetSystemLibrary.K2_ClearAndInvalidateTimerHandle` _returnvalue)
      (bind _outactors (`GameplayStatics.GetAllActorsOfClass` "/Game/_DRGModding/_SharedAssets/_Lesnov/AI/BP_TestingAI.BP_TestingAI_C"))
      (`self.K2_DestroyActor` _outactors)
      (`KismetSystemLibrary.CollectGarbage`))))

(event `/Game/_DRGModding/_Tools/DummyPlayerCharacter/BPI_DummyCharacter.OnUsedBy(Dummy)`
  (goto _label))

(fn `UserConstructionScript`)