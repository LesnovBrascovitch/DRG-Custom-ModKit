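; Box-shaped damage testing prop, a variant of a parent damage testing class whose own event graph is inactive.
; It overrides the parent's target getters to supply the Cube as target mesh and the Box component as target collision.
; After the parent construction script runs, it raises the Box in world space by its scaled Z half-extent, so a box centred on the actor's origin rests on it.
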(fn `GetTargetCollision(Override)`
  (returns (Collision :type "PrimitiveComponent Object Reference"))
  (return (`self.Box`)))

(fn `GetTargetMesh(Override)`
  (returns (StaticMesh :type "StaticMeshComponent Object Reference"))
  (return (`self.Cube`)))

(fn `UserConstructionScript`
  (bind (_returnvalue_x _returnvalue_y _returnvalue_z) (`KismetMathLibrary.BreakVector` (`BoxComponent.GetScaledBoxExtent` (`self.Box`))))
  (bind (_returnvalue_x_2 _returnvalue_y_2 _returnvalue_z_2) (`KismetMathLibrary.BreakVector` (`SceneComponent.K2_GetComponentLocation` (`self.Box`))))
  (`parent.UserConstructionScript`)
  (`SceneComponent.K2_SetWorldLocation` (`self.Box`) (`KismetMathLibrary.MakeVector` _returnvalue_x_2 _returnvalue_y_2 (+ _returnvalue_z_2 _returnvalue_z)) false false))