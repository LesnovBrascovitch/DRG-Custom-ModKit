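; Movable damage-testing prop that travels along a chain of linked waypoint actors.
; Each Tick it moves its TargetCollisionOverride component toward the current waypoint at constant InterpSpeed, without sweeping, and switches to that waypoint's Target on arrival.
; BeginPlay also starts a timeline after a short random delay, though nothing in the graph consumes its output.
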(event `CustomEvent_1`
  (`Timeline|Timeline_1`))

(event `self.ReceiveBeginPlay`
  (`parent.ReceiveBeginPlay`)
  (`KismetSystemLibrary.K2_SetTimerDelegate` (delegate `CustomEvent_1`) (`KismetMathLibrary.RandomFloatInRange` 0.0 2.0)))

(event `self.ReceiveTick`
  (params (DeltaSeconds :type "Float (single-precision)"))
  (bind _newvar_0 (`self.NewVar_0`))
  (bind _returnvalue (`SceneComponent.K2_GetComponentLocation` (`self.GetTargetCollision(Override)`)))
  (bind _returnvalue_2 (`self.K2_GetActorLocation` _newvar_0))
  (`parent.ReceiveTick` DeltaSeconds)
  (`/Engine/EditorBlueprintResources/StandardMacros.IsValid` _newvar_0
    (:`Is Valid`
      (if (== _returnvalue _returnvalue_2 :`ErrorTolerance` 1.0)
        (set `self.NewVar_0` (`/Game/_DRGModding/_SharedAssets/_Lesnov/DamageTestingProp/BP_DamageTesting_Movable_Location.Target` (`self.NewVar_0`))))
      (`SceneComponent.K2_SetWorldLocation` (`self.GetTargetCollision(Override)`) (`KismetMathLibrary.VInterpTo_Constant` _returnvalue _returnvalue_2 DeltaSeconds (`self.Interp Speed`)) false false))))

(fn `UserConstructionScript`
  (`parent.UserConstructionScript`))