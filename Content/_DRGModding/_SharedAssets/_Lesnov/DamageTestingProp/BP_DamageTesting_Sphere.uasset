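; Sphere-shaped damage testing prop, a child Blueprint that supplies its shape components to the parent class.
; Overrides GetTargetMesh and GetTargetCollision to return the Sphere1 mesh and the Sphere collision component.
; After the parent construction script runs, it raises the collision sphere in world Z by its scaled radius.
; The event graph holds only disabled stub events.
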(fn `GetTargetCollision(Override)`
  (returns (Collision :type "PrimitiveComponent Object Reference"))
  (return (`self.Sphere`)))

(fn `GetTargetMesh(Override)`
  (returns (StaticMesh :type "StaticMeshComponent Object Reference"))
  (return (`self.Sphere1`)))

(fn `UserConstructionScript`
  (bind _sphere (`self.Sphere`))
  (bind (_returnvalue_x _returnvalue_y _returnvalue_z) (`KismetMathLibrary.BreakVector` (`SceneComponent.K2_GetComponentLocation` _sphere)))
  (`parent.UserConstructionScript`)
  (`SceneComponent.K2_SetWorldLocation` (`self.Sphere`) (`KismetMathLibrary.MakeVector` _returnvalue_x _returnvalue_y (+ _returnvalue_z (`SphereComponent.GetScaledSphereRadius` _sphere))) false false))