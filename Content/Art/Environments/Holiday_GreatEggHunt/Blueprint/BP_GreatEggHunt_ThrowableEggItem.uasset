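; Throwable egg item for the Great Egg Hunt holiday event, built as a child of a throwable item Blueprint.
; Its throw, spawn, equip and inventory-removal events only forward to the parent implementations, so it adds no event logic of its own.
; GetThrowLocation returns a zero vector, while the construction script and the UsedMaterial replication callback are empty.
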(event `self.ReceiveItemThrown`
  (params (thrownActor :type "ThrowableActor Object Reference"))
  (`parent.ReceiveItemThrown` thrownActor))

(event `self.RemovedFromInventory`
  (params (oldCharacter :type "Character Object Reference"))
  (`parent.RemovedFromInventory` oldCharacter))

(event `self.OnReceiveEquippedFinished`
  (`parent.OnReceiveEquippedFinished`))

(event `self.RecieveEquipped`
  (`parent.RecieveEquipped`))

(event `self.ReceiveItemSpawned`
  (params (thrownActor :type "ThrowableActor Object Reference"))
  (`parent.ReceiveItemSpawned` thrownActor))

(fn `GetThrowLocation`
  (returns (ReturnValue :type "Vector Structure"))
  (return (0.0 0.0 0.0)))

(fn `OnRep_UsedMaterial`)

(fn `UserConstructionScript`)