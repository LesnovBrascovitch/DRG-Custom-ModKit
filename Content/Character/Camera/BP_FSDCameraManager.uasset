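; BP_FSDCameraManager is a player camera manager Blueprint that currently adds no behavior of its own.
; BeginPlay, Tick, Destroyed, photography session events and PhotographyCameraModify only forward to the parent class.
; Photography toggle, camera return, loader sequence and distance and speed events and functions are empty stubs.
; Helpers for smoothed return velocity, sphere direction to player and third-person camera return zero values.
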(event `self.ReceiveBeginPlay`
  (`parent.ReceiveBeginPlay`))

(event `self.ReceiveTick`
  (params (DeltaSeconds :type "Float (single-precision)"))
  (`parent.ReceiveTick` DeltaSeconds))

(event `self.ReceiveDestroyed`
  (`parent.ReceiveDestroyed`))

(event `self.OnPhotographySessionEnd`
  (`parent.OnPhotographySessionEnd`))

(event `self.OnPhotographySessionStart`
  (`parent.OnPhotographySessionStart`))

(event `TogglePhotographyMode`
  (params (Active :type Boolean)))

(event `Return Camera`)

(event `LoaderStart`
  (params (LoaderLevelSequence :type "LevelSequence Object Reference")))

(event `LoaderStop`)

(fn `ChangeMaxDistance`
  (params (MaxDistance :type "Float (double-precision)")))

(fn `ChangeSpeed`
  (params (MaxSpeed :type "Float (double-precision)")))

(fn `PhotographyCameraModify`
  (params (NewCameraLocation :type "Vector Structure") (PreviousCameraLocation :type "Vector Structure") (OriginalCameraLocation :type "Vector Structure"))
  (returns (ResultCameraLocation :type "Vector Structure"))
  (bind _resultcameralocation (`parent.PhotographyCameraModify` NewCameraLocation PreviousCameraLocation OriginalCameraLocation))
  (return _resultcameralocation))

(fn `ReturnCameraMode`
  (params (Target :type "PlayerCharacter Object Reference") (newCameraMode :type "ECharacterCameraMode Enum" :default "FirstPerson")))

(fn `SetToThirdPersonCamera`
  (returns (`New Camera Position` :type "Vector Structure"))
  (return (0.0 0.0 0.0)))

(fn `SmoothReturnVelocity`
  (params (`New Camera Location` :type "Vector Structure"))
  (returns (ReturnValue :type "Float (double-precision)"))
  (return 0.0))

(fn `SphereDirectionToPlayer`
  (returns (Direction :type "Vector Structure"))
  (return (0.0 0.0 0.0)))

(fn `UserConstructionScript`)